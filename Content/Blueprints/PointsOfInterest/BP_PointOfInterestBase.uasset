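; Base Blueprint for points of interest that detect the player's boat entering an Area trigger.
; On entry it calls the empty ShipEnter hook and, if StopOnEnter is set, zeroes boat and speed station targets and physics velocity.
; It finds the boat through TopDownGameMode.
; ShipInDockArea guards re-entry, but other overlaps also flip it: non-qualifying begins clear it and non-qualifying ends set it.
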(event `self.ReceiveBeginPlay`
  (bind _returnvalue (`GameplayStatics.GetActorOfClass` "/Game/Blueprints/GameMode/TopDownGameMode.TopDownGameMode_C"))
  (set `self.GameManager` _returnvalue))

(event `self.Area.OnComponentBeginOverlap`
  (params (OverlappedComponent :type "PrimitiveComponent Object Reference") (OtherActor :type "Actor Object Reference") (OtherComp :type "PrimitiveComponent Object Reference") (OtherBodyIndex :type Integer) (bFromSweep :type Boolean) (SweepResult :type "HitResult Structure (by ref)"))
  ;[1 1 1] entered area
  (if (and (== OtherActor (`/Game/Blueprints/GameMode/TopDownGameMode.Boat` (`self.GameManager`))) (not (`self.ShipInDockArea`)))
    (set `self.ShipInDockArea` true)
    (`self.ShipEnter`)
    (if (`self.StopOnEnter`)
      ;[1 1 1] stop ship
      (`/Game/Blueprints/Boat/BP_Boat.SetTargetSpeed` (`/Game/Blueprints/GameMode/TopDownGameMode.Boat` (`self.GameManager`)) 0.0)
      (`/Game/Blueprints/Stations/BP_Speed.Set Target Speed` (`/Game/Blueprints/GameMode/TopDownGameMode.SpeedStation` (`self.GameManager`)) 0.0)
      (`PrimitiveComponent.SetPhysicsLinearVelocity` (`/Game/Blueprints/Boat/BP_Boat.PhysicsActors` (`/Game/Blueprints/GameMode/TopDownGameMode.Boat` (`self.GameManager`))) (0.0 0.0 0.0) false "None"))
    (else
      (set `self.ShipInDockArea` false))))

(event `self.Area.OnComponentEndOverlap`
  (params (OverlappedComponent :type "PrimitiveComponent Object Reference") (OtherActor :type "Actor Object Reference") (OtherComp :type "PrimitiveComponent Object Reference") (OtherBodyIndex :type Integer))
  ;[1 1 1] Set Variable when ship is out of range
  (if (and (== OtherActor (`/Game/Blueprints/GameMode/TopDownGameMode.Boat` (`self.GameManager`))) (<= (`KismetArrayLibrary.Array_Length` (`PrimitiveComponent.GetOverlappingActors` OverlappedComponent "/Game/Blueprints/Boat/BP_Boat.BP_Boat_C")) 0))
    (set `self.ShipInDockArea` false)
    (else
      (set `self.ShipInDockArea` true))))

(fn `ShipEnter`)

(fn `UserConstructionScript`)