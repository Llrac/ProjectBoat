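; Delivery zone actor that converts the boat's cargo into score while a BP_Boat overlaps it.
; Tick runs a countdown that, on each interval, calls ConvertCargoToScore for crystals, barrels and peanuts, each with its own point value.
; Cargo and score counts live on the game mode's MainHUD, which the function updates one unit at a time.
; When nothing converts, a DoOnce shows the converted total and plays a ping, resetting when the boat leaves.
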(event `self.ReceiveBeginPlay`
  (bind _returnvalue (`GameplayStatics.GetActorOfClass` "/Game/Blueprints/GameMode/TopDownGameMode.TopDownGameMode_C"))
  (set `self.GameManager` _returnvalue))

(event `self.ReceiveTick`
  (params (DeltaSeconds :type "Float (single-precision)"))
  (bind _main_hud (`/Game/Blueprints/GameMode/TopDownGameMode.Main_HUD` (`self.GameManager`)))
  (bind _output_get (set `self.CurrentConvertTime` (- (`self.CurrentConvertTime`) DeltaSeconds)))
  (if (and (<= _output_get 0.0) (`self.HasOverlap`))
    (set `self.CurrentConvertTime` (`self.ConvertRate`))
    (`|ExecutionSequence`
      (:`then_0`
        (bind _didconvert (`self.Convert Cargo to Score` "NewEnumerator0" 10)))
      (:`then_1`
        (bind _didconvert_2 (`self.Convert Cargo to Score` "NewEnumerator2" 20)))
      (:`then_2`
        (bind _didconvert_3 (`self.Convert Cargo to Score` "NewEnumerator3" 5)))
      (:`then_3`
        (if (not (or _didconvert _didconvert_2 _didconvert_3))
          (`/Engine/EditorBlueprintResources/StandardMacros.DoOnce` false :!label _label
            (:`Completed`
              (`TextBlock.SetText` (`/Game/Blueprints/Widgets/WBP_Main_HUD.DeliverFeedback` _main_hud) (`KismetTextLibrary.Conv_StringToText` (`KismetStringLibrary.Concat_StrStr` "You converted " (`KismetStringLibrary.Conv_IntToString` (`self.ConvertedCargoCount`)) " cargo resources!")))
              (`UserWidget.PlayAnimation` _main_hud (`/Game/Blueprints/Widgets/WBP_Main_HUD.AppearThenFade` _main_hud) 0.0 1 "Forward" 1.0 false)
              (set `self.ConvertedCargoCount` 0)
              (`GameplayStatics.PlaySoundAtLocation` "/Game/Audio/SFX/SFX/ping01.ping01" (`self.K2_GetActorLocation`) (struct) 1.0 1.0 0.0 null null null null))))))))

(event `self.ReceiveActorBeginOverlap`
  (params (OtherActor :type "Actor Object Reference"))
  (cast `/Game/Blueprints/Boat/BP_Boat` OtherActor)
  (set `self.HasOverlap` true))

(event `self.ReceiveActorEndOverlap`
  (params (OtherActor :type "Actor Object Reference"))
  (cast `/Game/Blueprints/Boat/BP_Boat` OtherActor)
  (set `self.HasOverlap` false)
  (goto _label :!via `Reset`))

(fn `Convert Cargo to Score`
  (params (CargoType :type "/Game/Blueprints/Enums/E_MainHUDVariables Enum" :default "NewEnumerator4") (ScorePerCargo :type Integer))
  (returns (DidConvert :type Boolean))
  (locals (HasConvertedAny :type Boolean :default false))
  (bind _main_hud (`/Game/Blueprints/GameMode/TopDownGameMode.Main_HUD` (`self.GameManager`)))
  (bind _main_hud_2 (`/Game/Blueprints/GameMode/TopDownGameMode.Main_HUD` (`self.GameManager`)))
  (bind _main_hud_3 (`/Game/Blueprints/GameMode/TopDownGameMode.Main_HUD` (`self.GameManager`)))
  (bind _barrelcount (`/Game/Blueprints/Widgets/WBP_Main_HUD.BarrelCount` (`/Game/Blueprints/GameMode/TopDownGameMode.Main_HUD` (`self.GameManager`))))
  (bind _peanutcount (`/Game/Blueprints/Widgets/WBP_Main_HUD.PeanutCount` (`/Game/Blueprints/GameMode/TopDownGameMode.Main_HUD` (`self.GameManager`))))
  (bind _crystalcount (`/Game/Blueprints/Widgets/WBP_Main_HUD.CrystalCount` (`/Game/Blueprints/GameMode/TopDownGameMode.Main_HUD` (`self.GameManager`))))
  (`|ExecutionSequence`
    (:`then_0`
      (switch `/Game/Blueprints/Enums/E_MainHUDVariables` CargoType
        (:`NewEnumerator4`
          (`KismetSystemLibrary.PrintString` "unacceptable cargo type" true true (struct :`R` 1.0 :`A` 1.0) 2.0 "ConvertError" :!label _label))
        (:`NewEnumerator0`
          (if (>= (- _crystalcount 1) 0)
            (`/Engine/EditorBlueprintResources/StandardMacros.DecrementInt` _crystalcount
              (:`  `
                (set `/Game/Blueprints/Widgets/WBP_Main_HUD.ScoreCount` (+ (`/Game/Blueprints/Widgets/WBP_Main_HUD.ScoreCount` _main_hud_3) ScorePerCargo) _main_hud_3)
                (`/Game/Blueprints/Widgets/WBP_Main_HUD.UpdateHUDVariable` _main_hud_3 CargoType)
                (`/Game/Blueprints/Widgets/WBP_Main_HUD.UpdateHUDVariable` _main_hud_3 "NewEnumerator4")
                (`/Engine/EditorBlueprintResources/StandardMacros.IncrementInt` (`self.ConvertedCargoCount`)
                  (:`  `
                    (set `local.HasConvertedAny` true)))))))
        (:`NewEnumerator2`
          (if (>= (- _barrelcount 1) 0)
            (`/Engine/EditorBlueprintResources/StandardMacros.DecrementInt` _barrelcount
              (:`  `
                (set `/Game/Blueprints/Widgets/WBP_Main_HUD.ScoreCount` (+ (`/Game/Blueprints/Widgets/WBP_Main_HUD.ScoreCount` _main_hud) ScorePerCargo) _main_hud)
                (`/Game/Blueprints/Widgets/WBP_Main_HUD.UpdateHUDVariable` _main_hud CargoType)
                (`/Game/Blueprints/Widgets/WBP_Main_HUD.UpdateHUDVariable` _main_hud "NewEnumerator4")
                (`/Engine/EditorBlueprintResources/StandardMacros.IncrementInt` (`self.ConvertedCargoCount`)
                  (:`  `
                    (set `local.HasConvertedAny` true)))))))
        (:`NewEnumerator3`
          (if (>= (- _peanutcount 1) 0)
            (`/Engine/EditorBlueprintResources/StandardMacros.DecrementInt` _peanutcount
              (:`  `
                (set `/Game/Blueprints/Widgets/WBP_Main_HUD.ScoreCount` (+ (`/Game/Blueprints/Widgets/WBP_Main_HUD.ScoreCount` _main_hud_2) ScorePerCargo) _main_hud_2)
                (`/Game/Blueprints/Widgets/WBP_Main_HUD.UpdateHUDVariable` _main_hud_2 CargoType)
                (`/Game/Blueprints/Widgets/WBP_Main_HUD.UpdateHUDVariable` _main_hud_2 "NewEnumerator4")
                (`/Engine/EditorBlueprintResources/StandardMacros.IncrementInt` (`self.ConvertedCargoCount`)
                  (:`  `
                    (set `local.HasConvertedAny` true)))))))
        (:`NewEnumerator1`
          (goto _label))))
    (:`then_1`
      (return (`local.HasConvertedAny`)))))

(fn `UserConstructionScript`)