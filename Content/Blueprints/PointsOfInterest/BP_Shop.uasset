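; BP_Shop is a point-of-interest shop that opens when the ship enters it, letting cargo boxes be bought and sold for money.
; Entering pauses the game and shows an animated WBP_Shop widget linked back to the actor; exiting unpauses, plays the close animation and removes it after a delay.
; While open, Buy and Sell check funds or cargo, then adjust HUD money and GameManager cargo boxes.
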(event `self.ReceiveActorBeginOverlap`
  (params (OtherActor :type "Actor Object Reference"))
  (`parent.ReceiveActorBeginOverlap` OtherActor))

(event `Enter`
  ;[1 1 1] spawn widget, pause game
  (bind _returnvalue (`|CreateWidget` "/Game/Blueprints/Widgets/WBP_Shop.WBP_Shop_C"))
  (`UserWidget.AddToViewport` _returnvalue 0)
  (bind _output_get (set `self.ShopWidget` _returnvalue))
  (set `/Game/Blueprints/Widgets/WBP_Shop.ShopActor` self _output_get)
  (`UserWidget.PlayAnimation` _output_get (`/Game/Blueprints/Widgets/WBP_Shop.Open` _output_get) 0.0 1 "Forward" 1.0 false)
  (`GameplayStatics.SetGamePaused` true)
  (set `self.Shop is Open` true))

(event `self.ReceiveActorEndOverlap`
  (params (OtherActor :type "Actor Object Reference"))
  (`parent.ReceiveActorEndOverlap` OtherActor))

(event `Exit`
  (bind _shopwidget (`self.ShopWidget`))
  ;[1 1 1] unpause game, remove widget
  (`GameplayStatics.SetGamePaused` false)
  (`UserWidget.PlayAnimation` _shopwidget (`/Game/Blueprints/Widgets/WBP_Shop.Close` _shopwidget) 0.0 1 "Forward" 1.0 false)
  (`KismetSystemLibrary.Delay` 1.0)
  (`Widget.RemoveFromParent` (`self.ShopWidget`))
  (set `self.Shop is Open` false))

(event `Sell`
  (if (`self.Shop is Open`)
    (if (> (`KismetArrayLibrary.Array_Length` (`/Game/Blueprints/GameMode/TopDownGameMode.CargoBoxes` (`self.GameManager`))) 0)
      ;[1 1 1] Add money
      (set `/Game/Blueprints/Widgets/WBP_HUD.Money` (+ (`/Game/Blueprints/Widgets/WBP_HUD.Money` (`/Game/Blueprints/GameMode/TopDownGameMode.Main_HUD` (`self.GameManager`))) (`self.SellPrice`)) (`/Game/Blueprints/GameMode/TopDownGameMode.Main_HUD` (`self.GameManager`)))
      (`/Game/Blueprints/GameMode/TopDownGameMode.RemoveCargoBox` (`self.GameManager`) 1))))

(event `Buy`
  (bind _returnvalue (- (`/Game/Blueprints/Widgets/WBP_HUD.Money` (`/Game/Blueprints/GameMode/TopDownGameMode.Main_HUD` (`self.GameManager`))) (`self.BuyPrice`)))
  (if (`self.Shop is Open`)
    (if (>= _returnvalue 0)
      ;[1 1 1] -money
      (set `/Game/Blueprints/Widgets/WBP_HUD.Money` _returnvalue (`/Game/Blueprints/GameMode/TopDownGameMode.Main_HUD` (`self.GameManager`)))
      (`/Game/Blueprints/GameMode/TopDownGameMode.AddCargoBox` (`self.GameManager`) 1))))

(fn `ShipEnter`
  (`parent.ShipEnter`)
  (`self.Enter`))

(fn `UserConstructionScript`
  (`parent.UserConstructionScript`))