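; Point-of-interest area that spawns and hosts a sandserpent enemy.
; On BeginPlay it clears StopOnEnter, line-traces down to find the ground, spawns BP_Sandserpent just above it, and assigns itself as the serpent's Zone.
; ShipEnter, gated on the Triggered flag, forces a new track on the TopDownGameMode's MusicManager.
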(event `self.ShipEnter`
  (if (`self.Triggered`)
    (bind _returnvalue (`GameplayStatics.GetActorOfClass` "/Game/Blueprints/GameMode/TopDownGameMode.TopDownGameMode_C"))
    (`/Game/Audio/BP_MusicManager.ForceQueueNew` (`/Game/Blueprints/GameMode/TopDownGameMode.MusicManager` _returnvalue) 1)
    (set `self.Triggered` true)))

(event `self.ReceiveBeginPlay`
  (bind _returnvalue (`self.GetTransform`))
  (bind (_returnvalue_x _returnvalue_y) (`KismetMathLibrary.BreakVector` (`self.K2_GetActorLocation`)))
  (set `self.StopOnEnter` false)
  (`parent.ReceiveBeginPlay`)
  (bind _outhit (`KismetSystemLibrary.LineTraceSingle` (`KismetMathLibrary.MakeVector` _returnvalue_x _returnvalue_y 100000.0) (`KismetMathLibrary.MakeVector` _returnvalue_x _returnvalue_y -10000.0) "TraceTypeQuery1"))
  (bind _returnvalue_2 (`|SpawnActorFromClass` "/Game/Blueprints/Serpent/BP_Sandserpent.BP_Sandserpent_C" (`KismetMathLibrary.MakeTransform` (`KismetMathLibrary.MakeVector` (.x (.location _returnvalue)) (.y (.location _returnvalue)) (+ (.z (`.Location` (`GameplayStatics.BreakHitResult` _outhit))) 50.0)) (.rotation _returnvalue) (.scale _returnvalue)) "AdjustIfPossibleButAlwaysSpawn" "OverrideRootScale" null null)) ; spawn location 50 units over ground location
  (bind _output_get (set `self.Serpent` _returnvalue_2))
  (set `/Game/Blueprints/Serpent/BP_Sandserpent.Zone` self _output_get)
  (set `/Game/Blueprints/Serpent/BP_Sandserpent.Debug?` false _output_get))

(fn `UserConstructionScript`
  (`parent.UserConstructionScript`))