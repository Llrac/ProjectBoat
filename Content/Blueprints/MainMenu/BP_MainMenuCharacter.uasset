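; Main menu character Blueprint that AI-moves to a Starting actor on BeginPlay and clears IsMoving two seconds after play begins.
; Its MoveTo event sends it to a given target actor, setting IsMoving at the start and clearing it two seconds after success or failure.
; A random wander branch gated on IsMoving is present but disconnected, so it never runs.
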(event `self.ReceiveBeginPlay`
  (`|ExecutionSequence`
    (:`then_0`
      (`|AIMoveTo` self (0.0 0.0 0.0) (`self.Starting`)))
    (:`then_1`
      (`KismetSystemLibrary.Delay` 2.0)
      (set `self.IsMoving` false))))

(event `self.ReceiveTick`
  (params (DeltaSeconds :type "Float (single-precision)")))

(event `MoveTo`
  (params (TargetActor :type "Actor Object Reference"))
  (`|AIMoveTo` self (0.0 0.0 0.0) TargetActor
    (:`then`
      (set `self.IsMoving` true))
    (:`OnSuccess`
      (`KismetSystemLibrary.Delay` 2.0 :!label _label)
      (set `self.IsMoving` false))
    (:`OnFail`
      (goto _label))))

(fn `UserConstructionScript`)