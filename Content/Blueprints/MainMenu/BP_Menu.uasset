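; BP_Menu is a main menu actor that hosts a menu widget and links to other menus through camera transitions.
; At start it disables its own collision to block interaction and binds to the widget's transition event, which picks a target from LinkedMenus by index.
; A transition blends the view target to that menu, then after the blend enables its collision and focuses its widget's button.
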(event `self.ReceiveBeginPlay`
  (bind _aswbp_menu_parent_class (cast `/Game/Blueprints/MainMenu/MenuWidgets/WBP_MenuParentClass` (`WidgetComponent.GetUserWidgetObject` (`self.Widget`))))
  (`self.SetActorEnableCollision` false) ; Disable Interaction with menu at start
  (add `/Game/Blueprints/MainMenu/MenuWidgets/WBP_MenuParentClass.TransitionToLinkedMenu` _aswbp_menu_parent_class (delegate `TransitionToLinkedMenu_Event`)))

(event `TransitionToLinkedMenu_Event`
  (params (MenuIndex :type Integer))
  (bind _linkedmenus (`self.LinkedMenus`))
  (if (`KismetArrayLibrary.Array_IsValidIndex` _linkedmenus MenuIndex)
    (`self.TransitionTo` (`|GetArrayItem` _linkedmenus MenuIndex) 2.0) ; Transition to menu at index
  ))

(event `TransitionTo`
  (params (`New Menu` :type "/Game/Blueprints/MainMenu/BP_Menu Object Reference") (TransitionTime :type "Float (double-precision)"))
  ;[1 1 1] TransitionTo
  (`self.SetActorEnableCollision` false)
  (`PlayerController.SetViewTargetWithBlend` (`GameplayStatics.GetPlayerController` 0) `New Menu` TransitionTime "VTBlend_EaseInOut" 2.0 false) ; Transitions between Cameras
  (`KismetSystemLibrary.Delay` TransitionTime)
  (`self.SetActorEnableCollision` `New Menu` true)
  (bind _aswbp_menu_parent_class (cast `/Game/Blueprints/MainMenu/MenuWidgets/WBP_MenuParentClass` (`WidgetComponent.GetUserWidgetObject` (`/Game/Blueprints/MainMenu/BP_Menu.Widget` `New Menu`))))
  (`/Game/Blueprints/MainMenu/MenuWidgets/WBP_MenuParentClass.SetFocusButton` _aswbp_menu_parent_class))

(fn `UserConstructionScript`)