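; BP_Ham is a ham pickup that the boat collects by touching its sphere trigger.
; On overlap with the game manager's Boat, it disables collision, hides itself and raises the ham count stored on the main HUD, capped at the maximum.
; It then refreshes the HUD, plays a randomly pitched ping and a particle burst, and destroys itself after a short delay.
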(event `self.ReceiveBeginPlay`
  (bind _returnvalue (`GameplayStatics.GetActorOfClass` "/Game/Blueprints/GameMode/TopDownGameMode.TopDownGameMode_C"))
  (set `self.GameManager` _returnvalue))

(event `self.Sphere.OnComponentBeginOverlap`
  (params (OverlappedComponent :type "PrimitiveComponent Object Reference") (OtherActor :type "Actor Object Reference") (OtherComp :type "PrimitiveComponent Object Reference") (OtherBodyIndex :type Integer) (bFromSweep :type Boolean) (SweepResult :type "HitResult Structure (by ref)"))
  (bind _returnvalue (`SceneComponent.K2_GetComponentLocation` (`self.Cylinder`)))
  (bind _main_hud (`/Game/Blueprints/GameMode/TopDownGameMode.Main_HUD` (`self.GameManager`)))
  (if (== OtherActor (`/Game/Blueprints/GameMode/TopDownGameMode.Boat` (`self.GameManager`)))
    (`PrimitiveComponent.SetCollisionResponseToAllChannels` (`self.Sphere`) "ECR_Ignore")
    (`self.SetActorHiddenInGame` true)
    (set `/Game/Blueprints/Widgets/WBP_Main_HUD.HamCount` (`KismetMathLibrary.Clamp` (+ (`/Game/Blueprints/Widgets/WBP_Main_HUD.HamCount` _main_hud) 1) 0 (`/Game/Blueprints/Widgets/WBP_Main_HUD.MaxHamCount` _main_hud)) _main_hud)
    (`/Game/Blueprints/Widgets/WBP_Main_HUD.UpdateHUDVariable` _main_hud "NewEnumerator3")
    (`GameplayStatics.PlaySoundAtLocation` "/Game/Audio/SFX/SFX/ping01.ping01" _returnvalue (struct) 0.5 (`KismetMathLibrary.RandomFloatInRange` 0.7 1.3) 0.0 null null null null)
    (`GameplayStatics.SpawnEmitterAtLocation` "/Game/StarterContent/Particles/P_ExplosionReverse.P_ExplosionReverse" _returnvalue)
    (`KismetSystemLibrary.Delay` 2.0)
    (`self.K2_DestroyActor`)))

(fn `UserConstructionScript`)