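; BP_DestructableCrystal is a destructible crystal prop that loses one hit point each time its Hit event fires.
; It caches an ImagePrompt widget from its ButtonPrompt component and uses that widget's slider to show remaining health as a fraction of max HP.
; At zero HP it hides the slider and spawns a short-lived, scaled-down FS_MasterField with radial force, triggering it at the crystal's transform to break it apart.
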(event `self.ReceiveBeginPlay`
  (bind _asimage_prompt (cast `/Game/Blueprints/Widgets/ImagePrompt` (`WidgetComponent.GetWidget` (`self.ButtonPrompt`))))
  (set `self.As Image Prompt` _asimage_prompt))

(event `/Game/Blueprints/Interfaces/BPI_HitByCannon.Hit`
  (params (HitDirection :type "Vector Structure"))
  (bind _as_image_prompt (`self.As Image Prompt`))
  (`/Engine/EditorBlueprintResources/StandardMacros.DecrementInt` (`self.Hp`)
    (:`  `
      (`/Game/Blueprints/Widgets/ImagePrompt.SetSlider` _as_image_prompt true (/ (`self.Hp`) (`self.MaxHp`)))
      (if (<= (`self.Hp`) 0)
        (`/Game/Blueprints/Widgets/ImagePrompt.SetSlider` _as_image_prompt false 0.0)
        (bind _returnvalue (`|SpawnActorFromClass` "/Engine/EditorResources/FieldNodes/FS_MasterField.FS_MasterField_C" (`KismetMathLibrary.MakeTransform` (`self.K2_GetActorLocation`) (`self.K2_GetActorRotation`) (0.7 0.7 0.7)) "Undefined" "OverrideRootScale" null null))
        (bind _output_get (set `self.Master Field` _returnvalue))
        (set `/Engine/EditorResources/FieldNodes/FS_MasterField.ActivationType` "NewEnumerator4" _output_get)
        (set `/Engine/EditorResources/FieldNodes/FS_MasterField.FieldLifespan` 0.01 _output_get)
        (set `/Engine/EditorResources/FieldNodes/FS_MasterField.Radial Magnitude` 150.0 _output_get)
        (`/Engine/EditorResources/FieldNodes/FS_MasterField.CE_Trigger` _output_get)))))

(fn `UserConstructionScript`)