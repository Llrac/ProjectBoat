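; Cargo box prop that the TopDownGameMode tracks in its CargoBoxes list and that shows a button prompt.
; Overlapping a Killbox-tagged actor turns off collision, removes the box from that list and destroys it after a short delay.
; When the box stops overlapping other cargo boxes, it restores blocking on a custom collision channel.
; ShowPrompt toggles a controller or keyboard icon, with the prompt holder's world rotation zeroed every tick.
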(event `self.ReceiveBeginPlay`
  (bind _returnvalue (`GameplayStatics.GetActorOfClass` "/Game/Blueprints/GameMode/TopDownGameMode.TopDownGameMode_C"))
  (set `self.GameManager` _returnvalue)
  (bind _asimage_prompt (cast `/Game/Blueprints/Widgets/ImagePrompt` (`WidgetComponent.GetWidget` (`self.ButtonPrompt`))))
  (set `self.As Image Prompt` _asimage_prompt))

(event `self.Cube.OnComponentBeginOverlap`
  (params (OverlappedComponent :type "PrimitiveComponent Object Reference") (OtherActor :type "Actor Object Reference") (OtherComp :type "PrimitiveComponent Object Reference") (OtherBodyIndex :type Integer) (bFromSweep :type Boolean) (SweepResult :type "HitResult Structure (by ref)"))
  (if (`self.ActorHasTag` OtherActor "Killbox")
    ;[1 1 1] change physics
    (`PrimitiveComponent.SetCollisionResponseToAllChannels` (`self.Cube`) "ECR_Ignore")
    (if (`KismetArrayLibrary.Array_Contains` (`/Game/Blueprints/GameMode/TopDownGameMode.CargoBoxes` (`self.GameManager`)) self)
      ;[1 1 1] remove from cargolist
      (`KismetArrayLibrary.Array_RemoveItem` (`/Game/Blueprints/GameMode/TopDownGameMode.CargoBoxes` (`self.GameManager`))))
    (`KismetSystemLibrary.Delay` 2.0)
    (`self.K2_DestroyActor`)))

(event `self.Cube.OnComponentEndOverlap`
  (params (OverlappedComponent :type "PrimitiveComponent Object Reference") (OtherActor :type "Actor Object Reference") (OtherComp :type "PrimitiveComponent Object Reference") (OtherBodyIndex :type Integer))
  (switch `ECollisionChannel` (`PrimitiveComponent.GetCollisionObjectType` OtherComp)
    (:`ECC_GameTraceChannel6`
      (if (< (`KismetArrayLibrary.Array_Length` (`self.GetOverlappingActors` "BP_CargoBox_C")) 1)
        (`PrimitiveComponent.SetCollisionResponseToChannel` (`self.Cube`) "ECC_GameTraceChannel6" "ECR_Block")))))

(event `self.ReceiveTick`
  (params (DeltaSeconds :type "Float (single-precision)"))
  (`SceneComponent.K2_SetWorldRotation` :`self` (`self.prompt holder`)))

(event `/Game/Blueprints/Interfaces/BPI_Highlightable.ShowPrompt`
  (params (Enable :type Boolean) (`Controller Input` :type Boolean))
  (bind _as_image_prompt (`self.As Image Prompt`))
  (bind _as_image_prompt_2 (`self.As Image Prompt`))
  ;[1 1 1] toggle button prompt
  (if Enable
    (if `Controller Input`
      (`/Game/Blueprints/Widgets/ImagePrompt.SetImage` _as_image_prompt "/Game/Blueprints/Widgets/ButtonPrompts/Xbox_Series/XboxSeriesX_A.XboxSeriesX_A" true false)
      (else
        (`/Game/Blueprints/Widgets/ImagePrompt.SetImage` _as_image_prompt "/Game/Blueprints/Widgets/ButtonPrompts/Keyboard___Mouse/Light/Space_Key_Light.Space_Key_Light" true false)))
    (elif `Controller Input`
      (`/Game/Blueprints/Widgets/ImagePrompt.SetImage` _as_image_prompt_2 "/Game/Blueprints/Widgets/ButtonPrompts/Xbox_Series/XboxSeriesX_A.XboxSeriesX_A" false false)
      (else
        (`/Game/Blueprints/Widgets/ImagePrompt.SetImage` _as_image_prompt_2 "/Game/Blueprints/Widgets/ButtonPrompts/Keyboard___Mouse/Light/Space_Key_Light.Space_Key_Light" false false)))))

(fn `UserConstructionScript`)