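; Boat component that keeps the hovering boat's physics body oriented and weighted while it leaves the ground.
; Each tick it traces along a speed-scaled forward ray, falling back to straight down, for a ground normal.
; Airborne hovers get PlaneStabilizer targets on a plane blending that normal with world up by distance, plus steering roll and flip-recovery bias.
; A height trace drives quadratic lift in flying mode, otherwise downforce when high.
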(event `self.ReceiveBeginPlay`
  ;[1 1 1] Set Physics reference
  (bind _asprimitive_component (cast `PrimitiveComponent` (`Actor.RootComponent` (`self.GetOwner`))))
  (set `self.Ref To Body` _asprimitive_component)
  ;[1 1 1] Get Movement Component reference
  (set `self.MovementComponent` (`Actor.GetComponentByClass` (`self.GetOwner`) "/Game/Blueprints/Boat/BP_MovementComponent.BP_MovementComponent_C"))
  (bind _asbp_boat (cast `/Game/Blueprints/Boat/BP_Boat` (`self.GetOwner`)))
  (set `self.Trimaran` (`/Game/Blueprints/Boat/BP_Boat.trimaran` _asbp_boat)))

(event `self.ReceiveTick`
  (params (DeltaSeconds :type "Float (single-precision)"))
  (bind _returnvalue (`self.GetOwner`))
  (bind _returnvalue_2 (`self.GetOwner`))
  (bind _returnvalue_3 (`self.GetOwner`))
  (bind _heighttoactivateairmode (`self.HeightToActivateAirMode`))
  (bind _ref_to_body (`self.Ref To Body`))
  (bind _hover (`self.Hover`))
  (bind _debug (`self.Debug`))
  (bind _hover_2 (`self.Hover`))
  (bind _debug_2 (`self.Debug`))
  (bind _debug_3 (`self.Debug`))
  (bind (_returnvalue_roll _returnvalue_pitch _returnvalue_yaw) (`KismetMathLibrary.BreakRotator` (`Actor.K2_GetActorRotation` (`self.GetOwner`))))
  (bind _returnvalue_4 (`Actor.K2_GetActorLocation` (`self.GetOwner`)))
  (bind _returnvalue_roll_2 (`KismetMathLibrary.BreakRotator` (`SceneComponent.K2_GetComponentRotation` _hover)))
  (bind _returnvalue_5 (`Actor.K2_GetActorLocation` _returnvalue_3))
  (bind _returnvalue_6 (select `bool` (`self.DebugRay`) :`true` "ForOneFrame" :!type "EDrawDebugTrace Enum"))
  (bind (_relativelocation_x _relativelocation_y _relativelocation_z) (`KismetMathLibrary.BreakVector` (`SceneComponent.RelativeLocation` _hover_2)))
  (bind _returnvalue_7 (`KismetMathLibrary.Abs` _returnvalue_roll_2))
  (bind _returnvalue_8 (+ (* (`SceneComponent.GetUpVector` _hover_2) _relativelocation_z -1.0) (`SceneComponent.K2_GetComponentLocation` (`self.Hover`))))
  (bind _returnvalue_9 (+ (* (`self.StartHeight`) (`Actor.GetActorForwardVector` _returnvalue_2)) (`Actor.K2_GetActorLocation` _returnvalue_2)))
  (bind _returnvalue_10 (`KismetMathLibrary.FClamp` (`KismetMathLibrary.SafeDivide` (select `bool` (`self.HitInFront?`) :`false` (`self.HitDistance`) :`true` (* (`self.HitDistance`) 0.5)) (`self.LineTraceDistance`))))
  (bind _returnvalue_11 (`KismetMathLibrary.MakePlaneFromPointAndNormal` (`SceneComponent.K2_GetComponentLocation` (`self.Ref To Body`)) (+ (* (+ (`self.Impact Normal`) (* (+ (`Actor.GetActorForwardVector` _returnvalue) (`Actor.GetActorUpVector` _returnvalue)) (`self.TiltForwardOffset`))) (- 1.0 _returnvalue_10)) (* (+ (`KismetMathLibrary.Vector_Up`) (* (`KismetMathLibrary.GreaterGreater_VectorRotator` (`KismetMathLibrary.Vector_Right`) (`KismetMathLibrary.MakeRotator` 0.0 0.0 _returnvalue_yaw)) (/ (`/Game/Blueprints/Boat/BP_MovementComponent.TargetAngularSpeed` (`self.MovementComponent`)) (`self.TurningRollDivisor`)))) _returnvalue_10) (* (+ (* (`SceneComponent.GetUpVector` _hover) (/ _returnvalue_7 90.0)) (* (`SceneComponent.GetRightVector` _hover) (/ _returnvalue_7 180.0))) (select `bool` (> (`KismetMathLibrary.Abs` _returnvalue_roll_2) 70.0) :`true` 2.0 :!type "Float (single-precision)")))))
  (bind _returnvalue_12 (`KismetMathLibrary.Vector_MirrorByPlane` _returnvalue_8 _returnvalue_11))
  (`|ExecutionSequence`
    (:`then_0`
      ;[1 1 1] Set is Airborne?
      (set `self.Airborne?` true)
      (for _array_element (`self.Hovers`)
        (bind _output_get (set `self.Airborne?` (not (`/Game/Blueprints/Boat/BP_HoverComponent.TouchingGround?` _array_element))))
        (if (not _output_get)
          (break))))
    (:`then_1`
      (if (`self.IsActive?`)
        (`|ExecutionSequence`
          (:`then_0`
            ;[0.2344 0.2344 0.2344] Line Trace to ground to correct the boats rotation
            ;;[1 1 1] Line trace forward to get the normal of the ground
            (set `self.LineTraceDistance` (+ (* (`KismetMathLibrary.FClamp` (`/Game/Blueprints/Boat/BP_MovementComponent.CurrentSpeed` (`self.MovementComponent`)) 0.0 1500.0) (`self.SpeedFactor`)) (`self.BaseDistance`)))
            (bind (_outhit _returnvalue_13) (`KismetSystemLibrary.LineTraceSingle` :`Start` _returnvalue_9 :`End` (- _returnvalue_9 (* (`KismetMathLibrary.Normal` (+ (* (`Actor.GetActorForwardVector` _returnvalue_2) (* 1.0 (`self.TiltForwardFactor`) -1.0)) (`KismetMathLibrary.Vector_Up`))) (`self.LineTraceDistance`))) :`TraceChannel` "TraceTypeQuery3" :`DrawDebugType` _returnvalue_6 :`TraceColor` (struct :`G` 0.977268 :`B` 1.0 :`A` 1.0)))
            (bind _output_get_2 (set `self.HitInFront?` _returnvalue_13))
            ;;[1 1 1] Line Trace straight down if we found no trace forward
            (if _output_get_2
              (bind (_bblockinghit _binitialoverlap _time _distance _location _impactpoint _normal _impactnormal) (`GameplayStatics.BreakHitResult` _outhit))
              (set `self.Impact Normal` _impactnormal)
              (set `self.HitDistance` _distance)
              (else
                (set `self.LineTraceDistance` 5000.0)
                (bind (_outhit_2 _returnvalue_14) (`KismetSystemLibrary.LineTraceSingle` :`Start` _returnvalue_5 :`End` (- _returnvalue_5 (* (+ (`Actor.GetActorUpVector` _returnvalue_3) (`KismetMathLibrary.Vector_Up`)) (`self.LineTraceDistance`))) :`TraceChannel` "TraceTypeQuery3" :`DrawDebugType` _returnvalue_6 :`TraceColor` (struct :`R` 1.0 :`B` 0.915568 :`A` 1.0)))
                (bind (_bblockinghit_2 _binitialoverlap_2 _time_2 _distance_2 _location_2 _impactpoint_2 _normal_2 _impactnormal_2) (`GameplayStatics.BreakHitResult` _outhit_2))
                (set `self.HitDistance` _distance_2)
                (set `self.Impact Normal` (select `bool` _returnvalue_14 :`false` (`KismetMathLibrary.Vector_Up`) :`true` _impactnormal_2)))))
          (:`then_1`
            ;[0.2344 0.2344 0.2344] PlaneStabilizer
            (if (> (`KismetMathLibrary.Dot_VectorVector` (`self.Impact Normal`) (`KismetMathLibrary.Vector_Up`)) 0.5)
              ;;[1 1 1] Activate Plane Stabilizer when a hover is airborne, try to match the boat rotation to ground plane
              (for _array_element_2 (`self.Hovers`)
                (bind _output_get_3 (set `self.Hover` _array_element_2))
                (if (not (`/Game/Blueprints/Boat/BP_HoverComponent.TouchingGround?` _output_get_3))
                  (`|ExecutionSequence`
                    (:`then_0`
                      (`/Game/Blueprints/Boat/BP_HoverComponent.PlaneStabilizer` (`self.Hover`) (- _returnvalue_8 (+ (* (- _returnvalue_8 _returnvalue_12) (select `bool` (`self.Airborne?`) :`false` (`self.AirborneAmplitude`) :`true` (`self.NearGroundAmplitude`))) _returnvalue_12))))
                    (:`then_1`
                      (if (`self.DebugRay`)
                        ;;;[1 1 1] Debug
                        (`KismetSystemLibrary.DrawDebugPlane` _returnvalue_11 (`SceneComponent.K2_GetComponentLocation` (`self.Ref To Body`)) 250.0 (struct :`R` 1.0 :`G` 1.0 :`B` 1.0 :`A` 1.0) 0.05))))))
              (else
                ;;[1 1 1] Discard plane adjustment if Impact normal is too steep
                (`KismetSystemLibrary.PrintString` "BP_AS: Skipped Plane Stabilizer" _debug_3 _debug_3 (struct :`R` 1.0 :`G` 0.959391 :`A` 1.0)))))
          (:`then_2`
            ;[0.2344 0.2344 0.2344] Lower mass if we´re in the air, increasing flight time
            (bind (_outhit_3 _returnvalue_15) (`KismetSystemLibrary.LineTraceSingle` :`Start` _returnvalue_4 :`End` (- _returnvalue_4 (* (`KismetMathLibrary.Vector_Up`) (`self.HeightToActivateAirMode`))) :`TraceChannel` "TraceTypeQuery3" :`DrawDebugType` (select `bool` (`self.DebugRay`) :`true` "ForOneFrame" :!type "EDrawDebugTrace Enum"))) ; Line Trace straight down to get how high in the air we are
            (if (`self.FlyingMode`)
              (bind (_bblockinghit_3 _binitialoverlap_3 _time_3 _distance_3) (`GameplayStatics.BreakHitResult` _outhit_3))
              (bind _returnvalue_16 (/ (`KismetMathLibrary.MultiplyMultiply_FloatFloat` (select `bool` _returnvalue_15 :`false` _heighttoactivateairmode :`true` _distance_3) 2.0) (`KismetMathLibrary.MultiplyMultiply_FloatFloat` _heighttoactivateairmode 2.0)))
              (`PrimitiveComponent.AddForce` _ref_to_body (* (`SceneComponent.GetUpVector` _ref_to_body) 1000000.0 200.0 (`GameplayStatics.GetWorldDeltaSeconds`) _returnvalue_16) "None" false)
              (`KismetSystemLibrary.PrintString` (`KismetStringLibrary.Concat_StrStr` "BP_AS - Flying up force: " (`KismetStringLibrary.Conv_IntToString` (`KismetMathLibrary.FTrunc` (* _returnvalue_16 100.0))) "% added") _debug_2 _debug_2 (struct :`G` 0.66 :`B` 1.0 :`A` 1.0) 2.0 "effawesf")
              (else
                ;[1 1 1] Apply downforce if we're not airborne
                (if (> (select `bool` _bblockinghit_3 :`false` (`self.HeightToActivateAirMode`) :`true` _distance_3 :!type "Float (double-precision)") 350.0)
                  (bind _returnvalue_17 (`PrimitiveComponent.GetPhysicsLinearVelocity` (`self.Ref To Body`) "None"))
                  (bind _returnvalue_18 (`KismetMathLibrary.Dot_VectorVector` _returnvalue_17 (`SceneComponent.GetUpVector` (`self.Ref To Body`))))
                  (bind _returnvalue_19 (* (* (`KismetMathLibrary.Vector_Up`) -1.0) 1000000.0 (`KismetMathLibrary.FClamp` (- 1000.0 (* _returnvalue_18 -1.0)) 0.0 500.0) (`GameplayStatics.GetWorldDeltaSeconds`)))
                  (`PrimitiveComponent.AddForce` (`self.Ref To Body`) _returnvalue_19 "None" false)
                  (`KismetSystemLibrary.PrintString` (`KismetStringLibrary.Concat_StrStr` "BP_AS - Applying downforce: current " (`KismetStringLibrary.Conv_IntToString` (`KismetMathLibrary.FTrunc` _returnvalue_18)) " Added force: " (`KismetStringLibrary.Conv_IntToString` (`KismetMathLibrary.FTrunc` (`KismetMathLibrary.VSize` _returnvalue_19)))) _debug _debug (struct :`G` 0.66 :`B` 1.0 :`A` 1.0) 2.0 "AdditionalGravity"))))))))))

(event `EnableFlyingMode`
  (params (Enabled :type Boolean))
  (bind _output_get (set `self.FlyingMode` Enabled))
  (if _output_get
    _))