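; Boat component that damps sideways drift by pushing the owner's physics root against its lateral velocity.
; On BeginPlay it caches the owner's root primitive; while active, each tick projects linear velocity onto the body's right vector.
; It applies an opposing acceleration scaled by SpeedForceFactor, fading with pitch and, at half the weight, roll.
; A Debug flag prints the applied force.
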(event `self.ReceiveBeginPlay`
  ;[1 1 1] Set Physics reference
  (bind _asprimitive_component (cast `PrimitiveComponent` (`Actor.RootComponent` (`self.GetOwner`))))
  (set `self.Ref to Body` _asprimitive_component))

(event `self.ReceiveTick`
  (params (DeltaSeconds :type "Float (single-precision)"))
  (bind _ref_to_body (`self.Ref to Body`))
  (bind _debug (`self.Debug`))
  (bind (_returnvalue_roll _returnvalue_pitch) (`KismetMathLibrary.BreakRotator` (`Actor.K2_GetActorRotation` (`self.GetOwner`))))
  (bind _ref_to_body_2 (`self.Ref to Body`)
    (:`then`
      (if (`self.isActive?`)
        ;[1 1 1] Calculate current Lateral movement (Y axis)
        (bind _returnvalue (`PrimitiveComponent.GetPhysicsLinearVelocity` _ref_to_body_2 "None"))
        (bind _returnvalue_2 (* (`KismetMathLibrary.Dot_VectorVector` _returnvalue (`SceneComponent.GetRightVector` _ref_to_body_2)) -1.0 (`self.SpeedForceFactor`) (`KismetMathLibrary.FClamp` (- 1.0 (/ (`KismetMathLibrary.FClamp` (`KismetMathLibrary.Abs` _returnvalue_pitch) 0.0 45.0) 45.0) (/ (`KismetMathLibrary.FClamp` (`KismetMathLibrary.Abs` _returnvalue_roll) 0.0 45.0) 90.0)))))
        (`PrimitiveComponent.AddForce` _ref_to_body (* _returnvalue_2 (`SceneComponent.GetRightVector` _ref_to_body)) "None" true)
        (`KismetSystemLibrary.PrintString` (`KismetStringLibrary.Concat_StrStr` "BP_LS - Sideways force added: " (`KismetStringLibrary.Conv_DoubleToString` _returnvalue_2)) _debug _debug (struct :`G` 0.66 :`B` 1.0 :`A` 1.0) 2.0 "SideForce")))
    (:`else`)))