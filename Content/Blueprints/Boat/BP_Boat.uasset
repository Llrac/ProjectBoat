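; BP_Boat is a hover-based boat pawn or actor that skims over sand, forwarding target speed and turn requests to its movement component.
; Each tick it checks its hover points for ground contact; when airborne it blocks forward input and switches from yaw and lateral stabilizers to the air stabilizer.
; A sand friction sound plays while grounded, pitched by current speed.
; It also hands a front-ship focus viewer to the game mode's main camera.
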(event `self.ReceiveBeginPlay`
  (bind _debug (`self.Debug`))
  (`|ExecutionSequence`
    (:`then_1`
      ;[1 1 1] set debug messages
      (set `/Game/Blueprints/Boat/BP_MovementComponent.Debug` _debug (`self.BP_MovementComponent`))
      (set `/Game/Blueprints/Boat/BP_YawStabilizer.Debug` _debug (`self.BP_YawStabilizer`))
      (set `/Game/Blueprints/Boat/BP_AirStabilizer.Debug` _debug (`self.BP_AirStabilizer`))
      (set `/Game/Blueprints/Boat/BP_LateralStabilizer.Debug` _debug (`self.BP_LateralStabilizer`)))))

(event `self.ReceiveTick`
  (params (DeltaSeconds :type "Float (single-precision)"))
  (bind _bp_movementcomponent (`self.BP_MovementComponent`))
  (bind _airborne_ (`self.Airborne?`))
  (bind _returnvalue (not _airborne_))
  (`|ExecutionSequence`
    (:`then_0`
      ;[1 1 1] Check every Hover if they are in contact with ground
      (set `self.Airborne?` true)
      (for _array_element (`SceneComponent.GetChildrenComponents` (`self.HoverPoints`) false)
        (bind _asbp_hover_component (cast `/Game/Blueprints/Boat/BP_HoverComponent` _array_element))
        (bind _output_get (set `self.Airborne?` (not (`/Game/Blueprints/Boat/BP_HoverComponent.TouchingGround?` _asbp_hover_component))))
        (if (not _output_get)
          (break))))
    (:`then_1`
      ;[1 1 1] Disable movement inputs if we're airborne
      (bind _output_get_2 (set `/Game/Blueprints/Boat/BP_MovementComponent.CanGoForward?` (not (`self.Airborne?`)) (`self.BP_MovementComponent`))))
    (:`then_2`
      ;[1 1 1] Enable air stabilizer if airborne
      (set `/Game/Blueprints/Boat/BP_AirStabilizer.IsActive?` _airborne_ (`self.BP_AirStabilizer`))
      (set `/Game/Blueprints/Boat/BP_LateralStabilizer.isActive?` _returnvalue (`self.BP_LateralStabilizer`))
      (set `/Game/Blueprints/Boat/BP_YawStabilizer.IsActive?` _returnvalue (`self.BP_YawStabilizer`)))
    (:`then_3`
      ;[1 1 1] Audio
      ;;[1 1 1] toggle friction sound when grounded
      (`|ExecutionSequence`
        (:`then_0`
          (if (not (`self.Airborne?`))
            (if (not (`AudioComponent.IsPlaying` (`self.SandFriction_Cue`)))
              (`AudioComponent.Play` (`self.SandFriction_Cue`) 0.0))
            (else
              (`AudioComponent.Stop` (`self.SandFriction_Cue`)))))
        (:`then_1`
          (`AudioComponent.SetPitchMultiplier` (`self.SandFriction_Cue`) (- (* (/ (`/Game/Blueprints/Boat/BP_MovementComponent.CurrentSpeed` _bp_movementcomponent) (`/Game/Blueprints/Boat/BP_MovementComponent.MaxSpeed` _bp_movementcomponent)) 2.2) 0.2)) ; pitch wont go over 2 because reasons
        )))
    (:`then_4`
      (if (`self.Debug`)
        (`KismetSystemLibrary.PrintString` (`KismetStringLibrary.Concat_StrStr` "Is Airborne? " (`KismetStringLibrary.Conv_BoolToString` (`self.Airborne?`))) true true (struct :`G` 0.66 :`B` 1.0 :`A` 1.0) 2.0 "Airborne?")))))

(event `SetTargetSpeed`
  (params (TargetSpeed :type "Float (double-precision)"))
  (set `/Game/Blueprints/Boat/BP_MovementComponent.TargetSpeed` TargetSpeed (`self.BP_MovementComponent`)))

(event `SetTargetAngularSpeed`
  (params (AngularSpeed :type "Float (double-precision)"))
  (bind _output_get (set `/Game/Blueprints/Boat/BP_MovementComponent.TargetAngularSpeed` AngularSpeed (`self.BP_MovementComponent`))))

(event `GetFocusView`
  (bind _astop_down_game_mode (cast `/Game/Blueprints/GameMode/TopDownGameMode` (`GameplayStatics.GetGameMode`)))
  (`/Game/Blueprints/Camera/BP_MainCamera.Set Default Focus Viewer` (`/Game/Blueprints/GameMode/TopDownGameMode.MainCamera` _astop_down_game_mode) (`self.SC_FocusViewer(FrontShip)`)))

(fn `UserConstructionScript`)