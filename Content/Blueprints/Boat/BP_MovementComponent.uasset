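; Boat movement component that drives the owner's physics root body toward target forward speed and turning rate.
; Each tick it measures forward speed and applies clamped, mass-scaled force along the forward vector, with a separate brake factor, plus up-axis torque for turning.
; Events add boost time, which raises speed and acceleration limits, latch braking until speed drops below target, or apply upward force, logged as volcano lift.
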(event `self.ReceiveBeginPlay`
  ;[1 1 1] Get boat physics reference
  (bind _asprimitive_component (cast `PrimitiveComponent` (`Actor.RootComponent` (`self.GetOwner`))))
  (set `self.Ref to Body` _asprimitive_component))

(event `self.ReceiveTick`
  (params (DeltaSeconds :type "Float (single-precision)"))
  (bind _debug (`self.Debug`))
  (bind _debug_2 (`self.Debug`))
  (bind _maxaccelerationspeed (`self.MaxAccelerationSpeed`))
  (bind _debug_3 (`self.Debug`))
  (bind _ref_to_body (`self.Ref to Body`))
  (bind _ref_to_body_2 (`self.Ref to Body`))
  (bind _ref_to_body_3 (`self.Ref to Body`))
  (bind _ref_to_body_4 (`self.Ref to Body`))
  (bind _returnvalue (* (`self.TargetAngularSpeed`) (`self.AngularSpeedToTorqueFactor`)))
  (bind _returnvalue_2 (- (+ (`self.Boost`) (`self.TargetSpeed`)) (`self.CurrentSpeed`)))
  (bind _returnvalue_3 (`KismetMathLibrary.FClamp` _returnvalue_2 (select `bool` (`self.DoBrake`) :`true` (* _maxaccelerationspeed -20.0)) _maxaccelerationspeed))
  (bind _returnvalue_4 (* _returnvalue_3 (* (* (`PrimitiveComponent.GetMass` _ref_to_body_3) (`PrimitiveComponent.GetMassScale` _ref_to_body_3 "None")) (`KismetMathLibrary.SelectFloat` (`self.MoveForwardFactor`) (`self.BrakeFactor`) (> _returnvalue_3 0.0))) 1.0))
  (`|ExecutionSequence`
    (:`then_0`
      (bind _ref_to_body_5 (`self.Ref to Body`)
        (:`then`
          ;[1 1 1] Calculate current speed
          (bind _returnvalue_5 (`PrimitiveComponent.GetPhysicsLinearVelocity` _ref_to_body_5 "None"))
          (set `self.CurrentSpeed` (`KismetMathLibrary.Dot_VectorVector` _returnvalue_5 (`SceneComponent.GetForwardVector` _ref_to_body_5)))
          (`|ExecutionSequence`
            (:`then_0`
              (`self.Calculate Decceleration` (`self.CurrentSpeed`)))
            (:`then_1`
              (set `self.CurrentAngularSpeed` (`KismetMathLibrary.Dot_VectorVector` (`PrimitiveComponent.GetPhysicsAngularVelocityInDegrees` _ref_to_body "None") (`SceneComponent.GetUpVector` _ref_to_body)))
              ;[1 1 1] Add force forward multiplied by delta target speed
              (if (`self.CanGoForward?`)
                (`PrimitiveComponent.AddForce` _ref_to_body_2 (* (* (`SceneComponent.GetForwardVector` _ref_to_body_2) _returnvalue_4) (`GameplayStatics.GetWorldDeltaSeconds`) 60.0) "None" false)
                ;[1 1 1] Add torque around the up vector (think mast of ship)
                (if (`self.CanTurn?`)
                  (`PrimitiveComponent.AddTorqueInDegrees` _ref_to_body_4 (* (* (`SceneComponent.GetUpVector` _ref_to_body_4) _returnvalue) (`GameplayStatics.GetWorldDeltaSeconds`) 60.0) "None" true)
                  (`|ExecutionSequence`
                    (:`then_0`
                      ;[1 1 1] Debug
                      (`KismetSystemLibrary.PrintString` (`KismetStringLibrary.Concat_StrStr` "BP_MC - Current Speed: " (`KismetStringLibrary.Conv_IntToString` (`KismetMathLibrary.FTrunc` (`self.CurrentSpeed`)))) _debug _debug (struct :`G` 0.66 :`B` 1.0 :`A` 1.0) 2.0 "CurrentSpeed"))
                    (:`then_1`
                      (`KismetSystemLibrary.PrintString` (`KismetStringLibrary.Concat_StrStr` "BP_MC - Forward force added: " (`KismetStringLibrary.Conv_IntToString` (`KismetMathLibrary.FTrunc` _returnvalue_4))) _debug_2 _debug_2 (struct :`G` 0.66 :`B` 1.0 :`A` 1.0) 2.0 "ForwardForce"))
                    (:`then_2`
                      (`KismetSystemLibrary.PrintString` (`KismetStringLibrary.Concat_StrStr` "BP_MC - Turning torque added: " (`KismetStringLibrary.Conv_IntToString` (`KismetMathLibrary.FTrunc` _returnvalue))) _debug_3 _debug_3 (struct :`G` 0.66 :`B` 1.0 :`A` 1.0) 2.0 "TurningTorque"))
                    (:`then_3`
                      (if (> (`self.BoostDuration`) 0.0)
                        (set `self.DoDecceleration` false)
                        (set `self.MaxAccelerationSpeed` 2000.0)
                        (set `self.Boost` 2500.0)
                        (else
                          (set `self.DoDecceleration` true)
                          (set `self.MaxAccelerationSpeed` 1000.0)
                          (set `self.Boost` 0.0))))))))))
        (:`else`)))
    (:`then_1`
      ;[1 1 1] Handbreak
      (if (> _returnvalue_2 0.0)
        (set `self.DoBrake` false) ; Gets set from Handbreak
      ))))

(event `AddBoost`
  (params (Duration :type "Float (double-precision)"))
  (bind _debug (`self.Debug`))
  (`|ExecutionSequence`
    (:`then_0`
      (`KismetSystemLibrary.PrintString` (`KismetStringLibrary.Concat_StrStr` "BP_MC: Boost " (`KismetStringLibrary.Conv_IntToString` (`KismetMathLibrary.FTrunc` 0.0)) " Speed for " (`KismetStringLibrary.Conv_IntToString` (`KismetMathLibrary.FTrunc` Duration)) " seconds") _debug _debug (struct :`G` 0.66 :`B` 1.0 :`A` 1.0) Duration))
    (:`then_1`
      (if (<= (`self.BoostDuration`) 0.0)
        _
        (else
          _))
      (set `self.BoostDuration` (+ Duration (`self.BoostDuration`))))))

(event `Brake`
  ;[1 1 1] Brake
  (set `self.DoBrake` true))

(event `AddUpForce`
  (params (UpForce :type "Float (single-precision)"))
  (bind _debug (`self.Debug`))
  (`PrimitiveComponent.AddForce` (`self.Ref to Body`) (* (`KismetMathLibrary.Vector_Up`) (`GameplayStatics.GetWorldDeltaSeconds`) UpForce) "None" false)
  (`KismetSystemLibrary.PrintString` (`KismetStringLibrary.Concat_StrStr` "BP_MC - Volcano Applying  " (`KismetStringLibrary.Conv_IntToString` (`KismetMathLibrary.FTrunc` UpForce)) " Up Force") _debug _debug (struct :`G` 1.0 :`B` 0.024869 :`A` 1.0) 2.0 "Volcano"))

(fn `Calculate Decceleration`
  (params (LastFrameSpeed :type "Float (double-precision)"))
  (`|ExecutionSequence`
    (:`then_0`
      (if (and (< (`self.CurrentSpeed`) (`self.LastFrameSpeed`)) (`self.DoDecceleration`))
        (bind _output_get (set `self.TargetSpeed` (- (`self.TargetSpeed`) (/ (`KismetMathLibrary.Abs` (- (`self.CurrentSpeed`) (`self.LastFrameSpeed`))) 5.0))))
        ;[1 1 1] Slider variables and refs
        (bind _returnvalue (`GameplayStatics.GetActorOfClass` "/Game/Blueprints/GameMode/TopDownGameMode.TopDownGameMode_C"))))
    (:`then_1`
      (set `self.LastFrameSpeed` LastFrameSpeed) ; new last frame speed
    )))