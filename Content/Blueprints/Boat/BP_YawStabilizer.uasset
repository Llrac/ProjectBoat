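; Boat component that damps yaw spin by applying counter-torque to the owner's physics body.
; BeginPlay caches the owner's root as a PrimitiveComponent.
; While active, each Tick projects angular velocity onto the body's up vector, negates it, scales it by SpeedForceFactor and delta time, and applies it along that axis as mass-independent torque.
; An optional debug print reports the torque added.
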(event `self.ReceiveBeginPlay`
  ;[1 1 1] Set Physics reference
  (bind _asprimitive_component (cast `PrimitiveComponent` (`Actor.RootComponent` (`self.GetOwner`))))
  (set `self.Ref to Body` _asprimitive_component))

(event `self.ReceiveTick`
  (params (DeltaSeconds :type "Float (single-precision)"))
  (bind _ref_to_body (`self.Ref to Body`))
  (bind _debug (`self.Debug`))
  (bind _ref_to_body_2 (`self.Ref to Body`)
    (:`then`
      (if (`self.IsActive?`)
        (bind _returnvalue (* (`KismetMathLibrary.Dot_VectorVector` (`PrimitiveComponent.GetPhysicsAngularVelocityInDegrees` _ref_to_body_2 "None") (`SceneComponent.GetUpVector` _ref_to_body_2)) -1.0 (`self.SpeedForceFactor`) (`GameplayStatics.GetWorldDeltaSeconds`)))
        ;[1 1 1] Add counter torque on Z axis
        (`PrimitiveComponent.AddTorqueInDegrees` _ref_to_body (* (`SceneComponent.GetUpVector` _ref_to_body) _returnvalue) "None" true)
        (`KismetSystemLibrary.PrintString` (`KismetStringLibrary.Concat_StrStr` "BP_YS - Sideways torque added: " (`KismetStringLibrary.Conv_DoubleToString` _returnvalue)) _debug _debug (struct :`G` 0.66 :`B` 1.0 :`A` 1.0) 2.0 "YawStab")))
    (:`else`)))