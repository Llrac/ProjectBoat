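; Hover suspension component for the boat, pushing the owner's physics-simulated root body away from the ground at the component's location.
; Each tick it traces down along its up vector and applies a mass-scaled spring-damper force from compression and its rate of change.
; PlaneStabilizer applies a PID correction force from a supplied error vector, with the integral clamped against wind-up and reset on ground contact.
; AirStabilizer is an older scalar version of that stabilizer.
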(event `self.ReceiveBeginPlay`
  ;[1 1 1] Get reference to physics body
  (bind _asprimitive_component (cast `PrimitiveComponent` (`Actor.RootComponent` (`self.GetOwner`)))
    (:`then`
      (bind _output_get (set `self.RefToBody` _asprimitive_component))
      (if (not (`self.IsSimulatingPhysics` _output_get "None"))
        (set `self.RefToBody` null)))
    (:`CastFailed`
      (`KismetSystemLibrary.PrintText` "Cast failed to primitive"))))

(event `self.ReceiveTick`
  (params (DeltaSeconds :type "Float (single-precision)"))
  (bind _returnvalue (`self.K2_GetComponentLocation`))
  (bind _returnvalue_2 (`KismetSystemLibrary.GetDisplayName` self))
  (bind _returnvalue_3 (* (`PrimitiveComponent.GetMass` (`self.RefToBody`)) 2.0))
  (bind _returnvalue_4 (`KismetStringLibrary.GetSubstring` _returnvalue_2 (- (`KismetStringLibrary.Len` _returnvalue_2) 2) 2))
  ;[1 1 1] LineTrace down to determine how close to the ground we are
  (`self.RefToBody`
    (:`then`
      (`KismetArrayLibrary.Array_Add` (`self.ActorsToIgnore`) (`self.GetOwner`))
      (bind (_outhit _returnvalue_5) (`KismetSystemLibrary.LineTraceSingle` _returnvalue (- _returnvalue (* (`self.GetUpVector`) (`self.HoverDistance`))) "TraceTypeQuery3" false (`self.ActorsToIgnore`) (select `bool` (`self.DebugRay`) :`true` "ForOneFrame" :!type "EDrawDebugTrace Enum")))
      (bind _output_get (set `self.TouchingGround?` _returnvalue_5))
      (`|ExecutionSequence`
        (:`then_0`
          (if (`self.DebugRay`)
            ;[1 1 1] Debug
            (`KismetSystemLibrary.PrintString` (`KismetStringLibrary.Concat_StrStr` (`KismetStringLibrary.Concat_StrStr` _returnvalue_4 " is touching ground: ") (`KismetStringLibrary.Conv_BoolToString` (`self.TouchingGround?`))) true true (struct :`G` 0.66 :`B` 1.0 :`A` 1.0) 2.0 (`KismetStringLibrary.Conv_StringToName` _returnvalue_4))))
        (:`then_1`
          (if _output_get
            (set `self.VIntegralError` (0.0 0.0 0.0)) ; Reset Integral Error if we hit ground
            (bind _returnvalue_6 (/ (- (`self.HoverDistance`) (`.Distance` (`GameplayStatics.BreakHitResult` _outhit))) (`self.HoverDistance`)))
            ;[1 1 1] Add Force relative to up
            (set `self.HoverForce` (+ (* (/ (- _returnvalue_6 (`self.PrevConpression`)) (`GameplayStatics.GetWorldDeltaSeconds`)) (* (`self.Damping`) _returnvalue_3)) (* _returnvalue_6 (* (`self.Stiffness`) _returnvalue_3))))
            (set `self.PrevConpression` _returnvalue_6)
            (`PrimitiveComponent.AddForceAtLocation` (`self.RefToBody`) (* (`self.GetUpVector`) (`self.HoverForce`)) (`self.K2_GetComponentLocation`) "None")))))
    (:`else`)))

(event `AirStabilizer`
  (params (CurrentError :type "Float (double-precision)") (`Airborne?` :type Boolean))
  (bind _returnvalue (`KismetSystemLibrary.GetDisplayName` self))
  (bind _returnvalue_2 (* (+ (`self.Current Error`) (`self.LastError`) (`self.IntegralError`)) (select `bool` `Airborne?` :`true` 500.0)))
  ;[1 1 1] Old
  (bind _output_get (set `self.Counter` (- (`self.Counter`) (`GameplayStatics.GetWorldDeltaSeconds`))))
  (if (< _output_get 0.0)
    (set `self.Current Error` CurrentError)
    (set `self.IntegralError` (+ (`self.IntegralError`) (* (select `bool` `Airborne?` :`false` (/ (`self.IntegralGain`) 100.0) :`true` (`self.IntegralGain`)) (`GameplayStatics.GetWorldDeltaSeconds`) CurrentError)))
    (set `self.LastError` (/ (- (`self.Current Error`) (`self.LastError`)) (`GameplayStatics.GetWorldDeltaSeconds`)))
    (`PrimitiveComponent.AddForceAtLocation` (`self.RefToBody`) (* (`self.GetUpVector`) _returnvalue_2 -1) (`self.K2_GetComponentLocation`) "None")
    (set `self.LastError` (`self.Current Error`))
    (if (`self.Debug`)
      (`KismetSystemLibrary.PrintString` (`KismetStringLibrary.Concat_StrStr` _returnvalue " : Added force down: " (`KismetStringLibrary.Conv_DoubleToString` _returnvalue_2)) true true (struct :`G` 0.66 :`B` 1.0 :`A` 1.0) 2.0 (`KismetStringLibrary.Conv_StringToName` _returnvalue)))))

(event `PlaneStabilizer`
  (params (Error :type "Vector Structure"))
  (bind _maxvintegralerror (`self.MaxVIntegralError`))
  (bind _returnvalue (`KismetSystemLibrary.GetDisplayName` self))
  (bind _returnvalue_2 (* (+ (`self.VIntegralError`) (`self.VCurrentError`) (`self.VLastError`)) (`self.VForce`)))
  ;[1 1 1] PlaneStablilizer, uses a PID Regulator to correct the error
  (bind _output_get (set `self.VCurrentError` Error))
  (set `self.VIntegralError` (`KismetMathLibrary.ClampVectorSize` (+ (`self.VIntegralError`) (* (`self.IntegralGain`) (`GameplayStatics.GetWorldDeltaSeconds`) _output_get)) (* _maxvintegralerror -1.0) _maxvintegralerror))
  (set `self.VLastError` (* (/ (- (`self.VCurrentError`) (`self.VLastError`)) (`GameplayStatics.GetWorldDeltaSeconds`)) (`self.DerivativeGain`)))
  (`PrimitiveComponent.AddForceAtLocation` (`self.RefToBody`) _returnvalue_2 (`self.K2_GetComponentLocation`) "None")
  (set `self.VLastError` (`self.VCurrentError`))
  ;;[1 1 1] Debug
  (if (`self.Debug`)
    (`KismetSystemLibrary.PrintString` (`KismetStringLibrary.Concat_StrStr` _returnvalue " - Added force: " (`KismetStringLibrary.Conv_IntToString` (`KismetMathLibrary.FTrunc` (`KismetMathLibrary.VSize` _returnvalue_2))) " - IError: " (`KismetStringLibrary.Conv_IntToString` (`KismetMathLibrary.FTrunc` (`KismetMathLibrary.VSize` (`self.VIntegralError`))))) true true (struct :`G` 0.66 :`B` 1.0 :`A` 1.0) 2.0 (`KismetStringLibrary.Conv_StringToName` _returnvalue))))