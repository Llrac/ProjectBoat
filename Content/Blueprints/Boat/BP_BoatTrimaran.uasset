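; BP_BoatTrimaran is a physics-driven trimaran boat that steers through a movement component and stabilizes itself in the air.
; Each tick it treats the boat as airborne when no hover component touches ground, which disables forward and turn input.
; While airborne, PD-style torques combining angle error and angular velocity correct roll and pitch toward a target rotation.
; Setter events forward target speeds to movement, enabling the yaw stabilizer only at zero turn speed.
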(event `self.ReceiveBeginPlay`)

(event `self.ReceiveTick`
  (params (DeltaSeconds :type "Float (single-precision)"))
  (bind (_targetrotation_x _targetrotation_y) (`KismetMathLibrary.BreakVector` (`self.TargetRotation`)))
  (bind _bp_movementcomponent (`self.BP_MovementComponent`))
  (bind (_returnvalue_roll _returnvalue_pitch) (`KismetMathLibrary.BreakRotator` (`SceneComponent.K2_GetComponentRotation` (`self.PhysicsActor`))))
  (bind (_returnvalue_x _returnvalue_y) (`KismetMathLibrary.BreakVector` (* (`PrimitiveComponent.GetPhysicsAngularVelocityInDegrees` (`self.PhysicsActor`) "None") (`self.CurrentRotationToSpeedRatio`))))
  (`|ExecutionSequence`
    (:`then_0`
      ;[1 1 1] Check every Hover if they are in contact with ground
      (set `self.Airborne?` true)
      (for _array_element (`SceneComponent.GetChildrenComponents` (`self.PhysicsActor`) false)
        (bind _asbp_hover_component (cast `/Game/Blueprints/Boat/BP_HoverComponent` _array_element))
        (bind _output_get (set `self.Airborne?` (not (`/Game/Blueprints/Boat/BP_HoverComponent.TouchingGround?` _asbp_hover_component))))
        (if (not _output_get)
          (break))))
    (:`then_1`
      ;[1 1 1] Disable movement inputs if we're airborne
      (bind _output_get_2 (set `/Game/Blueprints/Boat/BP_MovementComponent.CanGoForward?` (not (`self.Airborne?`)) _bp_movementcomponent))
      (set `/Game/Blueprints/Boat/BP_MovementComponent.CanTurn?` _output_get_2 _bp_movementcomponent))
    (:`then_2`
      (if (`self.Airborne?`)
        (`|ExecutionSequence`
          (:`then_0`
            ;[1 1 1] Stabilize around X axis (Roll)
            (`PrimitiveComponent.AddTorqueInDegrees` (`self.PhysicsActor`) (* (* (`self.TorqueFactor`) (- (- _returnvalue_roll _targetrotation_x) _returnvalue_x)) (`SceneComponent.GetForwardVector` (`self.PhysicsActor`))) "None" true))
          (:`then_1`
            ;[1 1 1] Stabilize around Y axis (Pitch)
            (`PrimitiveComponent.AddTorqueInDegrees` (`self.PhysicsActor`) (* (* (`self.TorqueFactor`) (- (- _returnvalue_pitch _targetrotation_y) _returnvalue_y)) (`SceneComponent.GetRightVector` (`self.PhysicsActor`))) "None" true)))))
    (:`then_3`
      (if (`self.Debug`)
        (`KismetSystemLibrary.PrintString` (`KismetStringLibrary.Concat_StrStr` "Is Airborne? " (`KismetStringLibrary.Conv_BoolToString` (`self.Airborne?`))) true true (struct :`G` 0.66 :`B` 1.0 :`A` 1.0) 2.0 "Airborne?")))))

(event `SetTargetSpeed`
  (params (TargetSpeed :type "Float (double-precision)"))
  (set `/Game/Blueprints/Boat/BP_MovementComponent.TargetSpeed` TargetSpeed (`self.BP_MovementComponent`)))

(event `SetTargetAngularSpeed`
  (params (AngularSpeed :type "Float (double-precision)"))
  (bind _output_get (set `/Game/Blueprints/Boat/BP_MovementComponent.TargetAngularSpeed` AngularSpeed (`self.BP_MovementComponent`)))
  (set `/Game/Blueprints/Boat/BP_YawStabilizer.IsActive?` (== _output_get 0.0) (`self.BP_YawStabilizer`)))

(fn `UserConstructionScript`)