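; Environment spawner actor that scatters mountains and sabertooth skulls over the ground inside bounds set by its min/max marker components.
; On BeginPlay it repeatedly line-traces from random points at the top of the bounds to independently random points at the bottom.
; Each trace's location and surface normal feed SpawnRandomMountain, which uses a random MultiGate to pick one of five Blueprints and spawns it tilted to the slope.
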(event `self.ReceiveBeginPlay`
  (bind (_returnvalue_x _returnvalue_y) (`KismetMathLibrary.BreakVector` (`SceneComponent.K2_GetComponentLocation` (`self.MinY`))))
  (bind (_returnvalue_x_2 _returnvalue_y_2 _returnvalue_z) (`KismetMathLibrary.BreakVector` (`SceneComponent.K2_GetComponentLocation` (`self.MinZ`))))
  (bind (_returnvalue_x_3 _returnvalue_y_3 _returnvalue_z_2) (`KismetMathLibrary.BreakVector` (`SceneComponent.K2_GetComponentLocation` (`self.MaxZ`))))
  (bind _returnvalue_x_4 (`KismetMathLibrary.BreakVector` (`SceneComponent.K2_GetComponentLocation` (`self.MaxX`))))
  (bind (_returnvalue_x_5 _returnvalue_y_4) (`KismetMathLibrary.BreakVector` (`SceneComponent.K2_GetComponentLocation` (`self.MaxY`))))
  (bind _returnvalue_x_6 (`KismetMathLibrary.BreakVector` (`SceneComponent.K2_GetComponentLocation` (`self.MinX`))))
  (bind _returnvalue (`KismetMathLibrary.RandomFloatInRange` _returnvalue_x_6 _returnvalue_x_4))
  (bind _returnvalue_2 (`KismetMathLibrary.RandomFloatInRange` _returnvalue_y _returnvalue_y_4))
  (for _ (range 102)
    (bind _outhit (`KismetSystemLibrary.LineTraceSingle` (`KismetMathLibrary.MakeVector` _returnvalue _returnvalue_2 _returnvalue_z_2) (`KismetMathLibrary.MakeVector` _returnvalue _returnvalue_2 _returnvalue_z) "TraceTypeQuery1"))
    (bind (_outslopepitchdegreeangle _outsloperolldegreeangle) (`KismetMathLibrary.GetSlopeDegreeAngles` (0.0 1.0 0.0) (`.Normal` (`GameplayStatics.BreakHitResult` _outhit)) (0.0 0.0 1.0)))
    (bind (_returnvalue_x_7 _returnvalue_y_5) (`KismetMathLibrary.BreakVector` (`KismetMathLibrary.MakeVector` _outsloperolldegreeangle _outslopepitchdegreeangle)))
    (`self.SpawnRandomMountain` (`.Location` (`GameplayStatics.BreakHitResult` _outhit)) (* _returnvalue_x_7 -1.0) _returnvalue_y_5)))

(fn `SpawnRandomMountain`
  (params (SpawnTransform_Location :type "Vector Structure") (SpawnTransform_Rotation_Roll :type "Float (single-precision)") (SpawnTransform_Rotation_Pitch :type "Float (single-precision)"))
  (`|MultiGate` true
    (:`Out 0`
      (`|SpawnActorFromClass` "/Game/Blueprints/EnvironmentSpawner/BP_Mountain1.BP_Mountain1_C" (`KismetMathLibrary.MakeTransform` SpawnTransform_Location (`KismetMathLibrary.MakeRotator` SpawnTransform_Rotation_Roll SpawnTransform_Rotation_Pitch)) "Undefined" "OverrideRootScale" null null))
    (:`Out 1`
      (`|SpawnActorFromClass` "/Game/Blueprints/EnvironmentSpawner/BP_Mountain2.BP_Mountain2_C" (`KismetMathLibrary.MakeTransform` SpawnTransform_Location (`KismetMathLibrary.MakeRotator` SpawnTransform_Rotation_Roll SpawnTransform_Rotation_Pitch)) "Undefined" "OverrideRootScale" null null))
    (:`Out 2`
      (`|SpawnActorFromClass` "/Game/Blueprints/EnvironmentSpawner/BP_Mountain3.BP_Mountain3_C" (`KismetMathLibrary.MakeTransform` SpawnTransform_Location (`KismetMathLibrary.MakeRotator` SpawnTransform_Rotation_Roll SpawnTransform_Rotation_Pitch)) "Undefined" "OverrideRootScale" null null))
    (:`Out 3`
      (`|SpawnActorFromClass` "/Game/Blueprints/EnvironmentSpawner/BP_Mountain4.BP_Mountain4_C" (`KismetMathLibrary.MakeTransform` SpawnTransform_Location (`KismetMathLibrary.MakeRotator` SpawnTransform_Rotation_Roll SpawnTransform_Rotation_Pitch)) "Undefined" "OverrideRootScale" null null))
    (:`Out 4`
      (`|SpawnActorFromClass` "/Game/Blueprints/EnvironmentSpawner/BP_SabertoothSkull.BP_SabertoothSkull_C" (`KismetMathLibrary.MakeTransform` SpawnTransform_Location (`KismetMathLibrary.MakeRotator` SpawnTransform_Rotation_Roll SpawnTransform_Rotation_Pitch)) "Undefined" "OverrideRootScale" null null))))

(fn `UserConstructionScript`)