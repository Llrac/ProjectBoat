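; Boat steering station that a controller or keyboard player can take over to turn the boat.
; Tick builds a clamped angular velocity from steer input, eases it back toward zero when unmanned, and sends it to the boat by station Id.
; That velocity also rotates the wheel mesh and, with player input, drives the turning sound's playback and pitch.
; Highlight and switch events toggle each player's button prompts and steering UI, and switching notifies the music manager.
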(event `/Game/Blueprints/Interfaces/BPI_Station.Highlight`
  (params (Enable :type Boolean) (ControllerInput :type Boolean))
  (bind _players_input (`/Game/Blueprints/GameMode/TopDownGameMode.Players Input` (`self.GameManager`)))
  (if ControllerInput
    (`/Game/Blueprints/Players/BP_ThirdPersonCharacter.SetButtonImage` (`/Game/Blueprints/Players/BP_PlayersCombo.Player1BP` _players_input) "/Game/Blueprints/Widgets/ButtonPrompts/Xbox_Series/XboxSeriesX_X.XboxSeriesX_X" Enable false)
    (else
      (`/Game/Blueprints/Players/BP_ThirdPersonCharacter.SetButtonImage` (`/Game/Blueprints/Players/BP_PlayersCombo.Player2BP` _players_input) "/Game/Blueprints/Widgets/ButtonPrompts/Keyboard___Mouse/Light/E_Key_Light.E_Key_Light" Enable false))))

(event `self.ReceiveBeginPlay`
  (bind _returnvalue (`GameplayStatics.GetActorOfClass` "/Game/Blueprints/GameMode/TopDownGameMode.TopDownGameMode_C"))
  (set `self.GameManager` _returnvalue)
  (bind _assteer_prompt (cast `/Game/Blueprints/Widgets/SteerPrompt` (`WidgetComponent.GetWidget` (`self.SteerPrompt`))))
  (set `self.As Steer Prompt` _assteer_prompt)
  (bind _astext_prompt (cast `/Game/Blueprints/Widgets/TextPrompt` (`WidgetComponent.GetWidget` (`self.TextPrompt`))))
  (bind _output_get (set `self.As Text Prompt` _astext_prompt))
  (`/Game/Blueprints/Widgets/TextPrompt.SetText` _output_get "Steer"))

(event `/Game/Blueprints/Interfaces/BPI_RecieveInput.OnSwitchedFrom`
  (params (UsingControllerInput :type Boolean))
  (bind _gamemanager (`self.GameManager`))
  (bind _players_input (`/Game/Blueprints/GameMode/TopDownGameMode.Players Input` (`self.GameManager`)))
  (bind _player2bp (`/Game/Blueprints/Players/BP_PlayersCombo.Player2BP` _players_input))
  (bind _player1bp (`/Game/Blueprints/Players/BP_PlayersCombo.Player1BP` _players_input))
  ;[1 1 1] Event On Switched From
  (`|ExecutionSequence`
    (:`then_0`
      (set `self.ControlledByPlayer` true)
      (if (`self.Use Image Prompts`)
        ;;[1 1 1] Show Image
        (`/Game/Blueprints/Widgets/SteerPrompt.SetSteeringUI` (`self.As Steer Prompt`) UsingControllerInput true)
        (if UsingControllerInput
          (`/Game/Blueprints/Players/BP_ThirdPersonCharacter.SetButtonImage` _player1bp null false false)
          (else
            (`/Game/Blueprints/Players/BP_ThirdPersonCharacter.SetButtonImage` _player2bp null false false)))
        (else
          ;;[1 1 1] Show Text (Old)
          (if UsingControllerInput
            (`/Game/Blueprints/Players/BP_ThirdPersonCharacter.Set Button Prompt` _player1bp (`/Game/Blueprints/GameMode/TopDownGameMode.Interact Btn2 Con` _gamemanager) true)
            (else
              (`/Game/Blueprints/Players/BP_ThirdPersonCharacter.Set Button Prompt` _player2bp (`/Game/Blueprints/GameMode/TopDownGameMode.Interact Btn2` _gamemanager) true))))))
    (:`then_1`
      (`/Game/Audio/BP_MusicManager.Update Adaption Variables` (`/Game/Blueprints/GameMode/TopDownGameMode.MusicManager` (`self.GameManager`)) false true))))

(event `self.ReceiveTick`
  (params (DeltaSeconds :type "Float (single-precision)"))
  (bind _returnvalue (`GameplayStatics.GetWorldDeltaSeconds`))
  (bind (_returnvalue_2 _gets_player_input) (`self.Wheel Is Turning`))
  (bind _maxturnangle (`self.MaxTurnAngle`))
  (bind _steerwheelturn_cue (`self.SteerwheelTurn_Cue`))
  (bind _debug (`self.Debug`))
  (bind _steerwheelturn_cue_2 (`self.SteerwheelTurn_Cue`))
  (bind _target_angularvel (`self.Target AngularVel`))
  (bind _maxturnangle_2 (`self.MaxTurnAngle`))
  (bind _target_angularvel_2 (`self.Target AngularVel`))
  (`|ExecutionSequence`
    (:`then_0`
      ;[1 1 1] Steering
      (if (and (not (`self.ControlledByPlayer`)) (== (`self.Steer X`) 0.0))
        (if (< _target_angularvel_2 0.0)
          (set `self.Target AngularVel` (`KismetMathLibrary.FInterpTo` _target_angularvel 0.0 _returnvalue (* (/ (/ (* _maxturnangle -1.0) _target_angularvel_2) (`self.TurnSpeedLag`)) 50.0)))
          (else
            (set `self.Target AngularVel` (`KismetMathLibrary.FInterpTo` _target_angularvel 0.0 _returnvalue (* (/ (/ _maxturnangle _target_angularvel_2) (`self.TurnSpeedLag`)) 50.0)))))
        (else
          (set `self.Target AngularVel` (`KismetMathLibrary.FClamp` (+ (* (`GameplayStatics.GetWorldDeltaSeconds`) (`self.Steer X`) (`self.TurnSpeedLag`)) (`self.Target AngularVel`)) (* _maxturnangle_2 -1.0) _maxturnangle_2))))
      (`/Game/Blueprints/Boat/BP_Boat.SetTargetAngularSpeed` (`/Game/Blueprints/GameMode/TopDownGameMode.Boat` (`self.GameManager`)) (`self.Target AngularVel`) (`self.Id`))
      ;[1 1 1] steeringwheel
      (`SceneComponent.K2_SetRelativeRotation` (`self.Steerwheel`) (`KismetMathLibrary.MakeRotator` 0.0 (* (`self.Target AngularVel`) 2.0) 90.0) false false)
      (`|ExecutionSequence`
        (:`then_0`
          (if _gets_player_input
            (`AudioComponent.SetPitchMultiplier` _steerwheelturn_cue_2 2.0) ; pitch wont go over 2 because reasons
            (else
              (`AudioComponent.SetPitchMultiplier` _steerwheelturn_cue_2 1.0) ; pitch wont go over 2 because reasons
            )))
        (:`then_1`
          (if (not (and (`AudioComponent.IsPlaying` _steerwheelturn_cue) _returnvalue_2))
            (`AudioComponent.Play` _steerwheelturn_cue 0.0)))
        (:`then_2`
          (`KismetSystemLibrary.PrintString` (`KismetStringLibrary.Concat_StrStr` "Steer" (`KismetStringLibrary.Conv_IntToString` (`self.Id`)) " - Turn: " (`KismetStringLibrary.Conv_IntToString` (`KismetMathLibrary.FTrunc` (`self.Target AngularVel`))) " Max turn:  " (`KismetStringLibrary.Conv_IntToString` (`KismetMathLibrary.FTrunc` (`self.MaxTurnAngle`)))) _debug _debug (struct :`G` 0.66 :`B` 1.0 :`A` 1.0) 2.0 (`KismetStringLibrary.Conv_StringToName` (`KismetStringLibrary.Concat_StrStr` (`KismetSystemLibrary.GetDisplayName` self) (`KismetStringLibrary.Conv_IntToString` (`self.Id`))))))))))

(event `/Game/Blueprints/Interfaces/BPI_RecieveInput.2Vector Input_1`
  (params (`Action Value X` :type "Float (double-precision)") (`Action Value Y` :type "Float (double-precision)"))
  (set `self.Steer X` (`KismetMathLibrary.FClamp` `Action Value X` -1.0)))

(event `/Game/Blueprints/Interfaces/BPI_RecieveInput.OnSwitchedTo`
  (params (UseControllerInput :type Boolean))
  (bind _gamemanager (`self.GameManager`))
  (bind _players_input (`/Game/Blueprints/GameMode/TopDownGameMode.Players Input` (`self.GameManager`)))
  (bind _player1bp (`/Game/Blueprints/Players/BP_PlayersCombo.Player1BP` _players_input))
  (bind _player2bp (`/Game/Blueprints/Players/BP_PlayersCombo.Player2BP` _players_input))
  ;[1 1 1] Event On Switched To
  (`|ExecutionSequence`
    (:`then_0`
      (set `self.ControlledByPlayer` false)
      (if true
        ;;[1 1 1] Hide Image
        (`/Game/Blueprints/Widgets/SteerPrompt.SetSteeringUI` (`self.As Steer Prompt`) UseControllerInput false)
        (if UseControllerInput
          (`/Game/Blueprints/Players/BP_ThirdPersonCharacter.SetButtonImage` _player1bp "/Game/Blueprints/Widgets/ButtonPrompts/Xbox_Series/XboxSeriesX_X.XboxSeriesX_X" true false)
          (else
            (`/Game/Blueprints/Players/BP_ThirdPersonCharacter.SetButtonImage` _player2bp "/Game/Blueprints/Widgets/ButtonPrompts/Keyboard___Mouse/Light/E_Key_Light.E_Key_Light" true false)))
        (else
          ;;[1 1 1] Hide Text (Old)
          (if UseControllerInput
            (`/Game/Blueprints/Players/BP_ThirdPersonCharacter.Set Button Prompt` _player1bp (`/Game/Blueprints/GameMode/TopDownGameMode.Interact Btn Con` _gamemanager) false)
            (else
              (`/Game/Blueprints/Players/BP_ThirdPersonCharacter.Set Button Prompt` _player2bp (`/Game/Blueprints/GameMode/TopDownGameMode.interact btn` _gamemanager) false))))))
    (:`then_1`
      (`/Game/Audio/BP_MusicManager.Update Adaption Variables` (`/Game/Blueprints/GameMode/TopDownGameMode.MusicManager` (`self.GameManager`)) false true))))

(fn `UserConstructionScript`)

(fn `Wheel Is Turning`
  (returns (ReturnValue :type Boolean) (`Gets Player Input` :type Boolean))
  (bind _controlledbyplayer (`self.ControlledByPlayer`))
  (return (or (and (!= (`self.Target AngularVel`) 0.0) (not _controlledbyplayer)) (and (and _controlledbyplayer (!= (`self.Steer X`) 0.0)) (!= (`KismetMathLibrary.Abs` (`self.Target AngularVel`)) (`self.MaxTurnAngle`)))) (and (`self.ControlledByPlayer`) (!= (`self.Steer X`) 0.0))))