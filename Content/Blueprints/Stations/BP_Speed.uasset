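; Player-operated station that sets the boat's speed through repeated pump presses, with button prompts for controller or keyboard players.
; Each press adds speed, restarts the boat's Niagara speed effects and plays a timeline-driven lever pump with sound.
; Tick clamps the target speed, sends it to the boat and decays it in proportion to its fraction of max.
; The same fraction drives BP_Handbreak's lever rotation and both stations' prompt sliders.
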(event `self.ReceiveBeginPlay`
  (bind _returnvalue (`GameplayStatics.GetActorOfClass` "/Game/Blueprints/GameMode/TopDownGameMode.TopDownGameMode_C"))
  (set `self.GameManager` _returnvalue)
  (bind _returnvalue_2 (`GameplayStatics.GetActorOfClass` "/Game/Blueprints/Stations/BP_Handbreak.BP_Handbreak_C"))
  (set `self.Handbreak` _returnvalue_2)
  (`KismetSystemLibrary.DelayUntilNextTick`)
  (bind _asimage_prompt (cast `/Game/Blueprints/Widgets/ImagePrompt` (`WidgetComponent.GetWidget` (`self.ImagePrompt`))))
  (set `self.As Image Prompt` _asimage_prompt)
  ;[1 1 1] old
  (bind _astext_prompt (cast `/Game/Blueprints/Widgets/TextPrompt` (`WidgetComponent.GetWidget` (`self.TextPrompt1`))))
  (bind _output_get (set `self.TextPrompt` _astext_prompt))
  (`/Game/Blueprints/Widgets/TextPrompt.SetText` _output_get "Speed"))

(event `/Game/Blueprints/Interfaces/BPI_Station.Highlight`
  (params (Enable :type Boolean) (ControllerInput :type Boolean))
  (bind _players_input (`/Game/Blueprints/GameMode/TopDownGameMode.Players Input` (`self.GameManager`)))
  ;[1 1 1] Set Button Image
  (if ControllerInput
    (`/Game/Blueprints/Players/BP_ThirdPersonCharacter.SetButtonImage` (`/Game/Blueprints/Players/BP_PlayersCombo.Player1BP` _players_input) "/Game/Blueprints/Widgets/ButtonPrompts/Xbox_Series/XboxSeriesX_X.XboxSeriesX_X" Enable false)
    (else
      (`/Game/Blueprints/Players/BP_ThirdPersonCharacter.SetButtonImage` (`/Game/Blueprints/Players/BP_PlayersCombo.Player2BP` _players_input) "/Game/Blueprints/Widgets/ButtonPrompts/Keyboard___Mouse/Light/E_Key_Light.E_Key_Light" Enable false))))

(event `/Game/Blueprints/Interfaces/BPI_RecieveInput.OnSwitchedFrom`
  (params (UsingControllerInput :type Boolean))
  (bind _gamemanager (`self.GameManager`))
  (bind _as_image_prompt (`self.As Image Prompt`))
  (bind _players_input (`/Game/Blueprints/GameMode/TopDownGameMode.Players Input` (`self.GameManager`)))
  (bind _player2bp (`/Game/Blueprints/Players/BP_PlayersCombo.Player2BP` _players_input))
  (bind _player1bp (`/Game/Blueprints/Players/BP_PlayersCombo.Player1BP` _players_input))
  ;[1 1 1] Event On Switched From
  (set `self.ControlledByPlayer` true)
  (if (`self.UseImagePrompts`)
    ;;[1 1 1] Show Image
    (if UsingControllerInput
      (`/Game/Blueprints/Widgets/ImagePrompt.SetImage` _as_image_prompt "/Game/Blueprints/Widgets/ButtonPrompts/Xbox_Series/XboxSeriesX_A.XboxSeriesX_A" true true)
      (`/Game/Blueprints/Players/BP_ThirdPersonCharacter.SetButtonImage` _player1bp null false false)
      (else
        (`/Game/Blueprints/Widgets/ImagePrompt.SetImage` _as_image_prompt "/Game/Blueprints/Widgets/ButtonPrompts/Keyboard___Mouse/Light/Space_Key_Light.Space_Key_Light" true true)
        (`/Game/Blueprints/Players/BP_ThirdPersonCharacter.SetButtonImage` _player2bp null false false)))
    (`/Game/Blueprints/Widgets/ImagePrompt.SetSlider` _as_image_prompt false (/ (`self.Current Target Speed`) (`self.MaxSpeed`)))
    (else
      ;;[1 1 1] Show Text (Old)
      (if UsingControllerInput
        (`/Game/Blueprints/Players/BP_ThirdPersonCharacter.Set Button Prompt` _player1bp (`/Game/Blueprints/GameMode/TopDownGameMode.Interact Btn2 Con` _gamemanager) true)
        (else
          (`/Game/Blueprints/Players/BP_ThirdPersonCharacter.Set Button Prompt` _player2bp (`/Game/Blueprints/GameMode/TopDownGameMode.Interact Btn2` _gamemanager) true))))))

(event `self.ReceiveTick`
  (params (DeltaSeconds :type "Float (single-precision)"))
  (bind _handbreak (`self.Handbreak`))
  (`|ExecutionSequence`
    (:`then_0`
      ;[1 1 1] Speed
      (bind _output_get (set `self.Current Target Speed` (`KismetMathLibrary.FClamp` (+ (* (`GameplayStatics.GetWorldDeltaSeconds`) (* (`self.Drive Y`) 200.0)) (`self.Current Target Speed`)) 0.0 (`self.MaxSpeed`))))
      (`/Game/Blueprints/Boat/BP_Boat.SetTargetSpeed` (`/Game/Blueprints/GameMode/TopDownGameMode.Boat` (`self.GameManager`)) _output_get))
    (:`then_1`
      ;[1 1 1] Rotation for levers
      (`/Game/Blueprints/Stations/BP_Handbreak.Set Rotation` _handbreak (`KismetMathLibrary.MakeVector` (* (/ (`self.Current Target Speed`) (`self.MaxSpeed`)) 120.0)))
      (bind _as_image_prompt (`/Game/Blueprints/Stations/BP_Handbreak.As Image Prompt` _handbreak)
        (:`then`
          (`/Game/Blueprints/Widgets/ImagePrompt.SetSlider` _as_image_prompt false (/ (`self.Current Target Speed`) (`self.MaxSpeed`))))
        (:`else`)))
    (:`then_2`
      ;[1 1 1] lower over time, scaled by percentage of max
      (set `self.Current Target Speed` (- (`self.Current Target Speed`) (* (`GameplayStatics.GetWorldDeltaSeconds`) (`self.Decceleration Rate`) (/ (`self.Current Target Speed`) (`self.MaxSpeed`))))))
    (:`then_3`
      ;[1 1 1] update slider when controlled
      (bind _as_image_prompt_2 (`self.As Image Prompt`)
        (:`then`
          (`/Game/Blueprints/Widgets/ImagePrompt.SetSlider` _as_image_prompt_2 false (/ (`self.Current Target Speed`) (`self.MaxSpeed`))))
        (:`else`)))))

(event `/Game/Blueprints/Interfaces/BPI_RecieveInput.2Vector Input_1`
  (params (`Action Value X` :type "Float (double-precision)") (`Action Value Y` :type "Float (double-precision)")))

(event `Set Target Speed`
  (params (Speed :type "Float (double-precision)"))
  ;[1 1 1] Set Target Speed
  (set `self.Current Target Speed` Speed))

(event `/Game/Blueprints/Interfaces/BPI_RecieveInput.Interaction Key_1`
  (params (Start :type Boolean) (Cancel :type Boolean))
  ;[1 1 1] Event interaction Key 1
  (if Start
    (`/Game/Blueprints/Widgets/WBP_Main_HUD.UpdateHUDValue` (`/Game/Blueprints/GameMode/TopDownGameMode.Main_HUD` (`self.GameManager`)) "NewEnumerator1")
    (bind _output_get (set `self.Current Target Speed` (+ (`self.Current Target Speed`) (`self.Speed Per Press`))))
    (`/Game/Blueprints/Widgets/ImagePrompt.SetSlider` (`self.As Image Prompt`) false (/ _output_get (`self.MaxSpeed`)))
    (for _array_element (`/Game/Blueprints/Boat/BP_Boat.NiagaraSpeed` (`/Game/Blueprints/GameMode/TopDownGameMode.Boat` (`self.GameManager`)))
      (`ActorComponent.SetActive` _array_element true true)
      (`Timeline|Timeline` :!via `Reverse`
        (:`Update`
          _)
        (:`Finished`
          (`GameplayStatics.PlaySoundAtLocation` "/Game/Audio/SFX/Stations/pump.pump" (`self.K2_GetActorLocation`) (struct) 0.2 2.0 0.0 null null null null)
          (bind (_direction _rotation) (`Timeline|PumpRotation` :!via `PlayFromStart`)
            (:`Update`
              _))))
      (`SceneComponent.K2_SetRelativeRotation` (`self.leverholderRoot`) (`KismetMathLibrary.MakeRotator` 0.0 _rotation 90.0) false false))))

(event `/Game/Blueprints/Interfaces/BPI_RecieveInput.OnSwitchedTo`
  (params (UseControllerInput :type Boolean))
  (bind _gamemanager (`self.GameManager`))
  (bind _as_image_prompt (`self.As Image Prompt`))
  (bind _players_input (`/Game/Blueprints/GameMode/TopDownGameMode.Players Input` (`self.GameManager`)))
  (bind _player2bp (`/Game/Blueprints/Players/BP_PlayersCombo.Player2BP` _players_input))
  (bind _player1bp (`/Game/Blueprints/Players/BP_PlayersCombo.Player1BP` _players_input))
  ;[1 1 1] Event On Switched To
  (set `self.ControlledByPlayer` false)
  (if (`self.UseImagePrompts`)
    ;;[1 1 1] Hide Image
    (if UseControllerInput
      (`/Game/Blueprints/Widgets/ImagePrompt.SetImage` _as_image_prompt "/Game/Blueprints/Widgets/ButtonPrompts/Xbox_Series/XboxSeriesX_A.XboxSeriesX_A" false true)
      (`/Game/Blueprints/Players/BP_ThirdPersonCharacter.SetButtonImage` _player1bp "/Game/Blueprints/Widgets/ButtonPrompts/Xbox_Series/XboxSeriesX_X.XboxSeriesX_X" true false)
      (else
        (`/Game/Blueprints/Widgets/ImagePrompt.SetImage` _as_image_prompt "/Game/Blueprints/Widgets/ButtonPrompts/Keyboard___Mouse/Light/Space_Key_Light.Space_Key_Light" false true)
        (`/Game/Blueprints/Players/BP_ThirdPersonCharacter.SetButtonImage` _player2bp "/Game/Blueprints/Widgets/ButtonPrompts/Keyboard___Mouse/Light/E_Key_Light.E_Key_Light" true false)))
    (`/Game/Blueprints/Widgets/ImagePrompt.SetSlider` _as_image_prompt false (/ (`self.Current Target Speed`) (`self.MaxSpeed`)))
    (else
      ;;[1 1 1] Hide Text (Old)
      (if UseControllerInput
        (`/Game/Blueprints/Players/BP_ThirdPersonCharacter.Set Button Prompt` _player1bp (`/Game/Blueprints/GameMode/TopDownGameMode.Interact Btn Con` _gamemanager) false)
        (else
          (`/Game/Blueprints/Players/BP_ThirdPersonCharacter.Set Button Prompt` _player2bp (`/Game/Blueprints/GameMode/TopDownGameMode.interact btn` _gamemanager) false))))))

(fn `UserConstructionScript`)