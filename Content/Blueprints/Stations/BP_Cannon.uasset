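; Player-operated cannon station that either local player can take over to aim, charge and fire, offsetting the shared camera with the aim.
; While manned, a timer runs PredictHit, sphere-tracing along a predicted projectile arc with debug drawing.
; Holding charge slows turning and swells the barrel; that scale also sets trace and blast radius.
; Release spawns no projectile: it explodes instantly at the predicted hit and notifies BPI_HitByCannon actors in range.
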(event `SwitchFireMode`
  (set `self.Alt_Fire` (not (`self.Alt_Fire`)))
  (`GameplayStatics.PlaySoundAtLocation` "/Game/Audio/SFX/SFX/ping01.ping01" (`self.K2_GetActorLocation`) (struct) 0.5 0.2 0.0 null null null null))

(event `PredictHitEvent`
  (bind _outhit (`self.PredictHit`)))

(event `/Game/Blueprints/Interfaces/BPI_Station.Highlight`
  (params (Enable :type Boolean) (ControllerInput :type Boolean))
  (bind _pointlight (`self.PointLight`))
  (bind _players_input (`/Game/Blueprints/GameMode/TopDownGameMode.Players Input` (`self.GameManager`)))
  ;[1 1 1] highlight toggles
  (`SceneComponent.SetVisibility` _pointlight Enable false)
  (if ControllerInput
    (`/Game/Blueprints/Players/BP_ThirdPersonCharacter.SetButtonImage` (`/Game/Blueprints/Players/BP_PlayersCombo.Player1BP` _players_input) "/Game/Blueprints/Widgets/ButtonPrompts/Xbox_Series/XboxSeriesX_X.XboxSeriesX_X" Enable false)
    (`LightComponent.SetLightColor` _pointlight (struct :`R` 1.0 :`G` 1.0 :`A` 1.0) true)
    (else
      (`/Game/Blueprints/Players/BP_ThirdPersonCharacter.SetButtonImage` (`/Game/Blueprints/Players/BP_PlayersCombo.Player2BP` _players_input) "/Game/Blueprints/Widgets/ButtonPrompts/Keyboard___Mouse/Light/E_Key_Light.E_Key_Light" Enable false))))

(event `self.ReceiveBeginPlay`
  (bind _gamemanager (`self.GameManager`))
  (bind _returnvalue (`GameplayStatics.GetActorOfClass` "/Game/Blueprints/GameMode/TopDownGameMode.TopDownGameMode_C"))
  (set `self.GameManager` _returnvalue)
  (bind _ascannon_prompt (cast `/Game/Blueprints/Widgets/CannonPrompt` (`WidgetComponent.GetWidget` (`self.ButtonPrompt`))))
  (set `self.As Cannon Prompt` _ascannon_prompt)
  (bind _astext_prompt (cast `/Game/Blueprints/Widgets/TextPrompt` (`WidgetComponent.GetWidget` (`self.TextPrompt`))))
  (bind _output_get (set `self.As Text Prompt` _astext_prompt))
  (`/Game/Blueprints/Widgets/TextPrompt.SetText` _output_get "Cannon")
  (`SceneComponent.SetVisibility` (`self.FXS_CannonBeam`) false false)
  (`|ExecutionSequence`
    (:`then_0`
      (set `self.StartCannonScale` (`SceneComponent.K2_GetComponentScale` (`self.Cannon`)))
      (`SceneComponent.SetVisibility` (`self.PointLight`) false false))
    (:`then_1`
      (`KismetSystemLibrary.DelayUntilNextTick`)
      (for _array_element (`/Game/Blueprints/GameMode/TopDownGameMode.CannonStations` _gamemanager)
        (`KismetArrayLibrary.Array_AddUnique` (`self.PredictActorsToIgnore`) _array_element))
      (`KismetArrayLibrary.Array_AddUnique` (`self.PredictActorsToIgnore`) (`/Game/Blueprints/GameMode/TopDownGameMode.Boat` _gamemanager)))))

(event `/Game/Blueprints/Interfaces/BPI_RecieveInput.OnSwitchedFrom`
  (params (UsingControllerInput :type Boolean))
  (bind _players_input (`/Game/Blueprints/GameMode/TopDownGameMode.Players Input` (`self.GameManager`)))
  (bind _maincamera (`/Game/Blueprints/GameMode/TopDownGameMode.MainCamera` (`self.GameManager`)))
  ;[1 1 1] playercontrol
  (bind _returnvalue (`KismetSystemLibrary.K2_SetTimerDelegate` (delegate `PredictHitEvent`) (/ (`GameplayStatics.GetWorldDeltaSeconds`) 2.0) true))
  (set `self.ControlledByPlayer` true)
  (`LightComponent.SetLightColor` (`self.PointLight`) (struct :`G` 1.0 :`A` 1.0) true)
  (`/Game/Blueprints/Widgets/CannonPrompt.SetCannonUI` (`self.As Cannon Prompt`) UsingControllerInput true)
  (if UsingControllerInput
    (`/Game/Blueprints/Players/BP_ThirdPersonCharacter.SetButtonImage` (`/Game/Blueprints/Players/BP_PlayersCombo.Player1BP` _players_input) null false false)
    (else
      (`/Game/Blueprints/Players/BP_ThirdPersonCharacter.SetButtonImage` (`/Game/Blueprints/Players/BP_PlayersCombo.Player2BP` _players_input) null false false)))
  (`SceneComponent.SetVisibility` (`self.FXS_CannonBeam`) true false)
  (set `/Game/Blueprints/Camera/BP_MainCamera.LookAtOffset` (`self.Mid Base Offset`) _maincamera)
  (set `/Game/Blueprints/Camera/BP_MainCamera.CamBaseOffset` (`self.Cam Base Offset`) _maincamera)
  (`GameplayStatics.PlaySoundAtLocation` "/Game/Audio/SFX/Stations/gun_load.gun_load" (`self.K2_GetActorLocation`) (struct) 0.2 1.0 0.0 null null null null))

(event `self.ReceiveTick`
  (params (DeltaSeconds :type "Float (single-precision)"))
  (bind _maxturnangle_x (`self.MaxTurnAngle X`))
  (bind _maxturnangle_y (`self.MaxTurnAngle Y`))
  (bind _maxturnangle_x_2 (`self.MaxTurnAngle X`))
  (bind _maxturnangle_y_2 (`self.MaxTurnAngle Y`))
  (bind (_cannonscaledelta_x _cannonscaledelta_y _cannonscaledelta_z) (`KismetMathLibrary.BreakVector` (`self.CannonScaleDelta`)))
  (bind _maincamera (`/Game/Blueprints/GameMode/TopDownGameMode.MainCamera` (`self.GameManager`)))
  (`|ExecutionSequence`
    (:`then_0`
      (set `self.CurrentFireCooldown` (- (`self.CurrentFireCooldown`) DeltaSeconds))
      (if (`self.ControlledByPlayer`)
        (`|ExecutionSequence`
          (:`then_1`
            (if (not (`self.IsCharging`))
              (set `self.Target Angle X` (`KismetMathLibrary.FClamp` (+ (* (`GameplayStatics.GetWorldDeltaSeconds`) (`self.Steer X`) (`self.Turn Lag`)) (`self.Target Angle X`)) (* _maxturnangle_x -1.0) _maxturnangle_x))
              (set `self.Target Angle Y` (`KismetMathLibrary.FClamp` (+ (* (`GameplayStatics.GetWorldDeltaSeconds`) (`self.Steer Y`) (`self.Turn Lag`)) (`self.Target Angle Y`)) (* _maxturnangle_y -1.0) _maxturnangle_y))
              (else
                (set `self.Target Angle X` (`KismetMathLibrary.FClamp` (+ (* (`GameplayStatics.GetWorldDeltaSeconds`) (`self.Steer X`) 15.0) (`self.Target Angle X`)) (* _maxturnangle_x_2 -1.0) _maxturnangle_x_2))
                (set `self.Target Angle Y` (`KismetMathLibrary.FClamp` (+ (* (`GameplayStatics.GetWorldDeltaSeconds`) (`self.Steer Y`) 15.0) (`self.Target Angle Y`)) (* _maxturnangle_y_2 -1.0) _maxturnangle_y_2)))))
          (:`then_2`
            ;[1 1 1] rotation
            (`SceneComponent.K2_SetRelativeRotation` (`self.Cannon`) (`KismetMathLibrary.MakeRotator` 0.0 (`self.Target Angle Y`) (`self.Target Angle X`)) false false)
            ;[1 1 1] Comment
            (set `/Game/Blueprints/Camera/BP_MainCamera.CamBaseOffset` (+ (`self.Cam Base Offset`) (`KismetMathLibrary.MakeVector` 0.0 (* (`self.Target Angle X`) 40.0) (* (`self.Target Angle Y`) -20.0))) _maincamera)
            (set `/Game/Blueprints/Camera/BP_MainCamera.LookAtOffset` (+ (`self.Mid Base Offset`) (`KismetMathLibrary.MakeVector` 0.0 (* (`self.Target Angle X`) 20.0) (* (`self.Target Angle Y`) 20.0))) _maincamera))
          (:`then_3`
            (`self.Increase Pitch`))
          (:`then_4`
            (if (`self.IsCharging`)
              (`self.Set Cannon Scale` "NewEnumerator1")
              (else
                (`self.Set Cannon Scale` "NewEnumerator2"))))
          (:`then_5`
            (if (>= _cannonscaledelta_z 0.5)
              (`/Game/Blueprints/Widgets/TextPrompt.DecreaseFontScale` (`self.As Text Prompt`)))))
        (else
          (`self.Set Cannon Scale` "NewEnumerator0"))))
    (:`then_1`
      (if (`self.IsCharging`)
        (set `self.ChargeTime` (+ (`self.ChargeTime`) (`GameplayStatics.GetWorldDeltaSeconds`)))))))

(event `/Game/Blueprints/Interfaces/BPI_RecieveInput.OnSwitchedTo`
  (params (UseControllerInput :type Boolean))
  (bind _players_input (`/Game/Blueprints/GameMode/TopDownGameMode.Players Input` (`self.GameManager`)))
  (bind _maincamera (`/Game/Blueprints/GameMode/TopDownGameMode.MainCamera` (`self.GameManager`)))
  ;[1 1 1] release control
  (`KismetSystemLibrary.K2_ClearAndInvalidateTimerHandle` (stale `/Game/Blueprints/Interfaces/BPI_RecieveInput.OnSwitchedFrom` _returnvalue))
  (set `self.ControlledByPlayer` false)
  (`LightComponent.SetLightColor` (`self.PointLight`) (struct :`R` 1.0 :`G` 1.0 :`A` 1.0) true)
  (`/Game/Blueprints/Widgets/CannonPrompt.SetCannonUI` (`self.As Cannon Prompt`) UseControllerInput false)
  (if UseControllerInput
    (`/Game/Blueprints/Players/BP_ThirdPersonCharacter.SetButtonImage` (`/Game/Blueprints/Players/BP_PlayersCombo.Player1BP` _players_input) "/Game/Blueprints/Widgets/ButtonPrompts/Xbox_Series/XboxSeriesX_X.XboxSeriesX_X" true false)
    (else
      (`/Game/Blueprints/Players/BP_ThirdPersonCharacter.SetButtonImage` (`/Game/Blueprints/Players/BP_PlayersCombo.Player2BP` _players_input) "/Game/Blueprints/Widgets/ButtonPrompts/Keyboard___Mouse/Light/E_Key_Light.E_Key_Light" true false)))
  (`SceneComponent.SetVisibility` (`self.FXS_CannonBeam`) false false)
  (set `/Game/Blueprints/Camera/BP_MainCamera.LookAtOffset` (0.0 0.0 0.0) _maincamera)
  (set `/Game/Blueprints/Camera/BP_MainCamera.CamBaseOffset` (0.0 0.0 0.0) _maincamera))

(event `/Game/Blueprints/Interfaces/BPI_RecieveInput.2Vector Input_1`
  (params (`Action Value X` :type "Float (double-precision)") (`Action Value Y` :type "Float (double-precision)"))
  (bind _controllersensitivity (`self.ControllerSensitivity`))
  (bind _keyboardsensitivity (`self.KeyboardSensitivity`))
  (bind _returnvalue (/ `Action Value Y` _controllersensitivity))
  (bind _returnvalue_2 (/ `Action Value X` _controllersensitivity))
  (bind _returnvalue_3 (/ `Action Value X` _keyboardsensitivity))
  (bind _returnvalue_4 (/ `Action Value Y` _keyboardsensitivity))
  (if (== self (`/Game/Blueprints/Players/BP_PlayersCombo.Player1` (`/Game/Blueprints/GameMode/TopDownGameMode.Players Input` (`self.GameManager`))))
    (`|ExecutionSequence`
      (:`then_0`
        (if (`self.IsInvertedX`)
          (set `self.Steer X` (* _returnvalue_2 -1.0))
          (else
            (set `self.Steer X` _returnvalue_2))))
      (:`then_1`
        (if (`self.IsInvertedY`)
          (set `self.Steer Y` (* _returnvalue -1.0))
          (else
            (set `self.Steer Y` _returnvalue)))))
    (else
      (`|ExecutionSequence`
        (:`then_0`
          (if (`self.IsInvertedX`)
            (set `self.Steer X` (* _returnvalue_3 -1.0))
            (else
              (set `self.Steer X` _returnvalue_3))))
        (:`then_1`
          (if (`self.IsInvertedY`)
            (set `self.Steer Y` (* _returnvalue_4 -1.0))
            (else
              (set `self.Steer Y` _returnvalue_4))))))))

(event `/Game/Blueprints/Interfaces/BPI_RecieveInput.Interaction Key_1`
  (params (Start :type Boolean) (Cancel :type Boolean))
  (bind _hitlocation (`self.HitLocation`))
  (bind (_cannonscaledelta_x _cannonscaledelta_y _cannonscaledelta_z) (`KismetMathLibrary.BreakVector` (`self.CannonScaleDelta`)))
  (bind _muzzle (`self.muzzle`))
  (bind _hitlocation_2 (`self.HitLocation`))
  (bind (_cannonscaledelta_x_2 _cannonscaledelta_y_2 _cannonscaledelta_z_2) (`KismetMathLibrary.BreakVector` (`self.CannonScaleDelta`)))
  (bind _cannonexplosionscalemultiplier (`self.CannonExplosionScaleMultiplier`))
  (bind _muzzle_2 (`self.muzzle`))
  (bind _sc_chargingcannon (`self.SC_ChargingCannon`))
  (bind _returnvalue (`SceneComponent.K2_GetComponentLocation` _muzzle_2))
  (bind _returnvalue_2 (+ (`self.VisualExplosionScale`) (* _cannonscaledelta_z_2 _cannonexplosionscalemultiplier)))
  (if Cancel
    (`|ExecutionSequence`
      (:`then_0`
        (set `self.IsCharging` false)
        (`AudioComponent.Stop` (`self.SC_ChargingCannon`))
        (`AudioComponent.SetPitchMultiplier` _sc_chargingcannon 0.0)
        (set `self.CurrentFireCooldown` (`self.FireCooldown`)))
      (:`then_1`
        ;[1 1 1] Vector References
        ;;[1 1 1] line
        (set `self.RayStartPoint` _returnvalue)
        (set `self.RayEndPoint` (+ _returnvalue (* (`SceneComponent.GetForwardVector` _muzzle_2) 50000)))
        ;;[1 1 1] Projectile spawn location
        (set `self.MuzzleRotation` (`SceneComponent.K2_GetComponentRotation` _muzzle))
        (set `self.ProjectileSpawnLocation` (+ (`SceneComponent.K2_GetComponentLocation` _muzzle) (* (`SceneComponent.GetForwardVector` _muzzle) 10))))
      (:`then_2`
        (if (> (`self.ChargeTime`) 0.2)
          ;[1 1 1] Predict Fire
          (bind (_outhit _returnedhit) (`self.PredictHit`))
          (if _returnedhit
            (set `self.HitLocation` (`.Location` (`GameplayStatics.BreakHitResult` _outhit)))
            (`|ExecutionSequence`
              (:`then_0`
                ;[1 1 1] Spawn Explosion
                (`GameplayStatics.SpawnEmitterAtLocation` "/Game/StarterContent/Particles/P_Explosion.P_Explosion" _hitlocation_2 (struct) (* _cannonscaledelta_z_2 _cannonexplosionscalemultiplier (`KismetMathLibrary.MakeVector` _returnvalue_2 _returnvalue_2 _returnvalue_2)))
                (`NiagaraFunctionLibrary.SpawnSystemAtLocation` "/Game/Niagara/Sand/FXS_SandExplosionCannon.FXS_SandExplosionCannon" _hitlocation_2)
                (`GameplayStatics.PlaySoundAtLocation` "/Game/Audio/SFX/Stations/CannonFire.CannonFire" (`self.RayStartPoint`) (struct) 0.4 (`KismetMathLibrary.RandomFloatInRange` 0.8 1.3) 0.0 null null null null)
                ;[1 1 1] Explosion Collision
                (bind (_outhits _returnvalue_3) (`KismetSystemLibrary.SphereTraceMulti` :`Start` _hitlocation :`End` _hitlocation :`Radius` (* _cannonscaledelta_z (`self.CannonExplosionScaleMultiplier`) 1000.0) :`TraceChannel` "TraceTypeQuery1" :`DrawTime` 1.0))
                (if _returnvalue_3
                  (for _array_element _outhits
                    (bind (_bblockinghit _binitialoverlap _time _distance _location _impactpoint _normal _impactnormal _physmat _hitactor) (`GameplayStatics.BreakHitResult` _array_element))
                    (if (`KismetSystemLibrary.DoesImplementInterface` _hitactor "/Game/Blueprints/Interfaces/BPI_HitByCannon.BPI_HitByCannon_C")
                      (bind _asbpi_hit_by_cannon (cast `/Game/Blueprints/Interfaces/BPI_HitByCannon` _hitactor))
                      (`/Game/Blueprints/Interfaces/BPI_HitByCannon.Hit` _asbpi_hit_by_cannon (`self.HitLocation`))))))
              (:`then_1`
                (set `self.CannonScaleDelta` (0.0 0.0 0.0))
                (set `self.VisualCannonScaleDelta` (+ (`self.VisualCannonScaleDelta`) (1.0 1.0 1.0)))
                (set `self.CannonXPosDelta` -100.0))))))
      (:`then_3`
        (set `self.ChargeTime` 0.0)))
    (else
      (set `self.IsCharging` true)
      (`AudioComponent.Play` _sc_chargingcannon 0.0)
      (`AudioComponent.SetPitchMultiplier` _sc_chargingcannon 0.0))))

(fn `CalculateNormal`
  (params (Normal :type "Vector Structure"))
  (returns (NewRoll :type "Float (double-precision)") (NewPitch :type "Float (double-precision)"))
  (bind (_outslopepitchdegreeangle _outsloperolldegreeangle) (`KismetMathLibrary.GetSlopeDegreeAngles` (0.0 1.0 0.0) Normal (0.0 0.0 1.0)))
  (bind (_returnvalue_x _returnvalue_y) (`KismetMathLibrary.BreakVector` (`KismetMathLibrary.MakeVector` _outsloperolldegreeangle _outslopepitchdegreeangle)))
  (return (* _returnvalue_x -1.0) _returnvalue_y))

(fn `Increase Pitch`
  (bind _sc_chargingcannon (`self.SC_ChargingCannon`))
  (`AudioComponent.SetPitchMultiplier` _sc_chargingcannon (`KismetMathLibrary.FInterpTo` (`KismetMathLibrary.FClamp` (`AudioComponent.PitchMultiplier` _sc_chargingcannon) 0.5 2.0) 2.0 (`GameplayStatics.GetWorldDeltaSeconds`) 8.0)))

(fn `PredictHit`
  (returns (OutHit :type "HitResult Structure") (ReturnedHit :type Boolean) (PredictArray :type "Array of PredictProjectilePathPointData Structure"))
  (bind _predictlength (`self.PredictLength`))
  (bind _muzzle (`self.muzzle`))
  (bind (_cannonscaledelta_x _cannonscaledelta_y _cannonscaledelta_z) (`KismetMathLibrary.BreakVector` (`self.CannonScaleDelta`)))
  (bind _predictresult (`GameplayStatics.Blueprint_PredictProjectilePath_Advanced` (make `PredictProjectilePathParams` (`SceneComponent.K2_GetComponentLocation` _muzzle) (* (`KismetMathLibrary.Conv_RotatorToVector` (`SceneComponent.K2_GetComponentRotation` _muzzle)) (`KismetMathLibrary.MakeVector` _predictlength _predictlength (`self.PredictHeight`))) true 15.0 10.0 true "ECC_WorldStatic" _ (`self.PredictActorsToIgnore`) 5.0 0.0 "None" (/ (`GameplayStatics.GetWorldDeltaSeconds`) 2.0) true)))
  (for (_array_element _array_index) (break `PredictProjectilePathResult` _predictresult)
    (if (< _array_index (- (`KismetArrayLibrary.Array_Length` (break `PredictProjectilePathResult` _predictresult)) 1))
      (bind _output_location (break `PredictProjectilePathPointData` (`|GetArrayItem` (break `PredictProjectilePathResult` _predictresult) (+ _array_index 1))))
      (bind (_outhit _returnvalue) (`KismetSystemLibrary.SphereTraceSingle` (break `PredictProjectilePathPointData` _array_element) _output_location (* _cannonscaledelta_z (`self.CannonExplosionScaleMultiplier`) 20.0) "TraceTypeQuery1" true (`self.PredictActorsToIgnore`) "ForDuration" true (make `LinearColor` 1.0 (- 1.0 (* 2.5 (- _cannonscaledelta_z 0.2)))) (struct :`R` 1.0 :`A` 1.0) (/ (`GameplayStatics.GetWorldDeltaSeconds`) 2.0)))
      (if _returnvalue
        (break))))
  (return _outhit _returnvalue (break `PredictProjectilePathResult` _predictresult)))

(fn `Set Cannon Scale`
  (params (CannonState :type "/Game/Blueprints/Enums/E_CannonStates Enum" :default "NewEnumerator0"))
  (`|ExecutionSequence`
    (:`then_0`
      (switch `/Game/Blueprints/Enums/E_CannonStates` CannonState
        (:`NewEnumerator0`
          (set `self.CannonScaleDelta` (`KismetMathLibrary.VInterpTo` (`self.CannonScaleDelta`) (0.0 0.0 0.0) (`GameplayStatics.GetWorldDeltaSeconds`) 2.0)))
        (:`NewEnumerator2`
          (set `self.CannonScaleDelta` (`KismetMathLibrary.VInterpTo` (`self.CannonScaleDelta`) (0.2 0.2 0.2) (`GameplayStatics.GetWorldDeltaSeconds`) 2.0)))
        (:`NewEnumerator1`
          (set `self.CannonScaleDelta` (`KismetMathLibrary.VInterpTo` (`self.CannonScaleDelta`) (0.4 0.6 0.6) (`GameplayStatics.GetWorldDeltaSeconds`) 2.0)))))
    (:`then_1`
      (set `self.VisualCannonScaleDelta` (`KismetMathLibrary.VInterpTo` (`self.VisualCannonScaleDelta`) (0.0 0.0 0.0) (`GameplayStatics.GetWorldDeltaSeconds`) 2.0))
      (`SceneComponent.SetWorldScale3D` (`self.Cannon`) (+ (`self.CannonScaleDelta`) (`self.StartCannonScale`) (`self.VisualCannonScaleDelta`))))))

(fn `UserConstructionScript`)