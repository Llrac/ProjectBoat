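; BP_ReverseCannonBall is a station projectile actor that flies in a straight line and removes itself after a fixed lifetime.
; Tick offsets it along its forward vector at a constant, frame-rate-independent speed without sweeping, so the movement does no collision checks.
; BeginPlay starts the delayed self-destruct.
; An impact sequence with a reverse explosion, debug print, hiding and delayed destroy is present but never runs.
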(event `self.ReceiveBeginPlay`
  (`KismetSystemLibrary.Delay` 10.0)
  (`self.K2_DestroyActor`))

(event `self.ReceiveTick`
  (params (DeltaSeconds :type "Float (single-precision)"))
  (`self.K2_AddActorWorldOffset` (* (`self.GetActorForwardVector` self) DeltaSeconds 10000.0)))

(fn `UserConstructionScript`)