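; BP_CannonToggle is an interactable station that switches the fire mode of every BP_Cannon in the level.
; BeginPlay caches the game mode, cannons and prompt widgets.
; Interaction key 1 calls SwitchFireMode on each cannon and plays a Timeline button animation.
; Highlight and switch events swap player and station prompts for controller (Player 1) or keyboard (Player 2), using images or legacy text.
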(event `self.ReceiveBeginPlay`
  (bind _returnvalue (`GameplayStatics.GetActorOfClass` "/Game/Blueprints/GameMode/TopDownGameMode.TopDownGameMode_C"))
  (set `self.GameManager` _returnvalue)
  (`GameplayStatics.GetActorOfClass` "/Game/Blueprints/Stations/BP_Handbreak.BP_Handbreak_C")
  (bind _outactors (`GameplayStatics.GetAllActorsOfClass` "/Game/Blueprints/Stations/BP_Cannon.BP_Cannon_C"))
  (set `self.cannons` _outactors)
  (bind _asimage_prompt (cast `/Game/Blueprints/Widgets/ImagePrompt` (`WidgetComponent.GetWidget` (`self.Prompt`))))
  (set `self.As Image Prompt` _asimage_prompt)
  ;[1 1 1] old
  (bind _astext_prompt (cast `/Game/Blueprints/Widgets/TextPrompt` (`WidgetComponent.GetWidget` (`self.ButtonPrompt`))))
  (set `self.TextPrompt` _astext_prompt))

(event `/Game/Blueprints/Interfaces/BPI_Station.Highlight`
  (params (Enable :type Boolean) (ControllerInput :type Boolean))
  (bind _gamemanager (`self.GameManager`))
  (bind _players_input (`/Game/Blueprints/GameMode/TopDownGameMode.Players Input` (`self.GameManager`)))
  (bind _player2bp (`/Game/Blueprints/Players/BP_PlayersCombo.Player2BP` _players_input))
  (bind _player1bp (`/Game/Blueprints/Players/BP_PlayersCombo.Player1BP` _players_input))
  (if (`self.UseImagePrompts`)
    ;[1 1 1] Set Button Image
    (if ControllerInput
      (`/Game/Blueprints/Players/BP_ThirdPersonCharacter.SetButtonImage` _player1bp "/Game/Blueprints/Widgets/ButtonPrompts/Xbox_Series/XboxSeriesX_X.XboxSeriesX_X" Enable false)
      (else
        (`/Game/Blueprints/Players/BP_ThirdPersonCharacter.SetButtonImage` _player2bp "/Game/Blueprints/Widgets/ButtonPrompts/Keyboard___Mouse/Light/E_Key_Light.E_Key_Light" Enable false)))
    (else
      ;[1 1 1] Set Button Text (Old)
      (if Enable
        (if ControllerInput
          (`/Game/Blueprints/Players/BP_ThirdPersonCharacter.Set Button Prompt` _player1bp (`/Game/Blueprints/GameMode/TopDownGameMode.Interact Btn Con` _gamemanager) false)
          (else
            (`/Game/Blueprints/Players/BP_ThirdPersonCharacter.Set Button Prompt` _player2bp (`/Game/Blueprints/GameMode/TopDownGameMode.interact btn` _gamemanager) false)))
        (elif ControllerInput
          (`/Game/Blueprints/Players/BP_ThirdPersonCharacter.Set Button Prompt` _player1bp "" false)
          (else
            (`/Game/Blueprints/Players/BP_ThirdPersonCharacter.Set Button Prompt` _player2bp "" false)))))))

(event `/Game/Blueprints/Interfaces/BPI_RecieveInput.OnSwitchedFrom`
  (params (UsingControllerInput :type Boolean))
  (bind _gamemanager (`self.GameManager`))
  (bind _as_image_prompt (`self.As Image Prompt`))
  (bind _players_input (`/Game/Blueprints/GameMode/TopDownGameMode.Players Input` (`self.GameManager`)))
  (bind _player2bp (`/Game/Blueprints/Players/BP_PlayersCombo.Player2BP` _players_input))
  (bind _player1bp (`/Game/Blueprints/Players/BP_PlayersCombo.Player1BP` _players_input))
  ;[1 1 1] Event On Switched From
  (set `self.ControlledByPlayer` true)
  (if (`self.UseImagePrompts`)
    ;;[1 1 1] Show Image
    (if UsingControllerInput
      (`/Game/Blueprints/Widgets/ImagePrompt.SetImage` _as_image_prompt "/Game/Blueprints/Widgets/ButtonPrompts/Xbox_Series/XboxSeriesX_A.XboxSeriesX_A" true false)
      (`/Game/Blueprints/Players/BP_ThirdPersonCharacter.SetButtonImage` _player1bp null false false)
      (else
        (`/Game/Blueprints/Widgets/ImagePrompt.SetImage` _as_image_prompt "/Game/Blueprints/Widgets/ButtonPrompts/Keyboard___Mouse/Light/Space_Key_Light.Space_Key_Light" true false)
        (`/Game/Blueprints/Players/BP_ThirdPersonCharacter.SetButtonImage` _player2bp null false false)))
    (else
      ;;[1 1 1] Show Text (Old)
      (if UsingControllerInput
        (`/Game/Blueprints/Players/BP_ThirdPersonCharacter.Set Button Prompt` _player1bp (`/Game/Blueprints/GameMode/TopDownGameMode.Interact Btn2 Con` _gamemanager) false)
        (else
          (`/Game/Blueprints/Players/BP_ThirdPersonCharacter.Set Button Prompt` _player2bp (`/Game/Blueprints/GameMode/TopDownGameMode.Interact Btn2` _gamemanager) false))))))

(event `/Game/Blueprints/Interfaces/BPI_RecieveInput.Interaction Key_1`
  (params (Start :type Boolean) (Cancel :type Boolean))
  (bind _staticmesh1 (`self.StaticMesh1`))
  (bind (_relativelocation_x _relativelocation_y) (`KismetMathLibrary.BreakVector` (`SceneComponent.RelativeLocation` _staticmesh1)))
  ;[1 1 1] Event interaction Key 1
  (if Start
    (for _array_element (`self.cannons`)
      (`/Game/Blueprints/Stations/BP_Cannon.SwitchFireMode` _array_element))
    ;;[1 1 1] button anim
    (bind (_direction _button) (`Timeline|Timeline` :!via `PlayFromStart`)
      (:`Update`
        (`SceneComponent.K2_SetRelativeLocation` _staticmesh1 (`KismetMathLibrary.MakeVector` _relativelocation_x _relativelocation_y _button) false false)))))

(event `/Game/Blueprints/Interfaces/BPI_RecieveInput.OnSwitchedTo`
  (params (UseControllerInput :type Boolean))
  (bind _gamemanager (`self.GameManager`))
  (bind _as_image_prompt (`self.As Image Prompt`))
  (bind _players_input (`/Game/Blueprints/GameMode/TopDownGameMode.Players Input` (`self.GameManager`)))
  (bind _player2bp (`/Game/Blueprints/Players/BP_PlayersCombo.Player2BP` _players_input))
  (bind _player1bp (`/Game/Blueprints/Players/BP_PlayersCombo.Player1BP` _players_input))
  ;[1 1 1] Event On Switched To
  (set `self.ControlledByPlayer` false)
  (if (`self.UseImagePrompts`)
    ;;[1 1 1] Hide Image
    (if UseControllerInput
      (`/Game/Blueprints/Widgets/ImagePrompt.SetImage` _as_image_prompt "/Game/Blueprints/Widgets/ButtonPrompts/Xbox_Series/XboxSeriesX_A.XboxSeriesX_A" false false)
      (`/Game/Blueprints/Players/BP_ThirdPersonCharacter.SetButtonImage` _player1bp "/Game/Blueprints/Widgets/ButtonPrompts/Xbox_Series/XboxSeriesX_X.XboxSeriesX_X" true false)
      (else
        (`/Game/Blueprints/Widgets/ImagePrompt.SetImage` _as_image_prompt "/Game/Blueprints/Widgets/ButtonPrompts/Keyboard___Mouse/Light/Space_Key_Light.Space_Key_Light" false false)
        (`/Game/Blueprints/Players/BP_ThirdPersonCharacter.SetButtonImage` _player2bp "/Game/Blueprints/Widgets/ButtonPrompts/Keyboard___Mouse/Light/E_Key_Light.E_Key_Light" true false)))
    (else
      ;;[1 1 1] Hide Text (Old)
      (if UseControllerInput
        (`/Game/Blueprints/Players/BP_ThirdPersonCharacter.Set Button Prompt` _player1bp (`/Game/Blueprints/GameMode/TopDownGameMode.Interact Btn Con` _gamemanager) false)
        (else
          (`/Game/Blueprints/Players/BP_ThirdPersonCharacter.Set Button Prompt` _player2bp (`/Game/Blueprints/GameMode/TopDownGameMode.interact btn` _gamemanager) false))))))

(fn `UserConstructionScript`)