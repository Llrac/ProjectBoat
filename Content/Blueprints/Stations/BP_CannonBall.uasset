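; BP_CannonBall is a cannonball projectile that explodes visually on impact and applies no damage itself.
; Tick pushes it along its forward vector at a constant speed using unswept world offsets, without a projectile movement component.
; A Collider hit spawns an explosion emitter, hides the cannon fire effect, stops physics simulation and destroys the actor after a short delay.
; A timed delay from BeginPlay also destroys it, capping its lifetime.
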(event `self.ReceiveBeginPlay`
  (`KismetSystemLibrary.Delay` 10.0)
  (`self.K2_DestroyActor`))

(event `self.ReceiveTick`
  (params (DeltaSeconds :type "Float (single-precision)"))
  (`self.K2_AddActorWorldOffset` (* (`self.GetActorForwardVector` self) DeltaSeconds 1000.0)))

(event `self.collider.OnComponentHit`
  (params (HitComponent :type "PrimitiveComponent Object Reference") (OtherActor :type "Actor Object Reference") (OtherComp :type "PrimitiveComponent Object Reference") (NormalImpulse :type "Vector Structure") (Hit :type "HitResult Structure (by ref)"))
  (`GameplayStatics.SpawnEmitterAtLocation` "/Game/StarterContent/Particles/P_Explosion.P_Explosion" (`.Location` (`GameplayStatics.BreakHitResult` Hit)))
  (`SceneComponent.SetVisibility` (`self.FXS_CannonFire`) false false)
  (`PrimitiveComponent.SetSimulatePhysics` (`self.collider`) false)
  (`KismetSystemLibrary.Delay` 1.0)
  (`self.K2_DestroyActor`))

(fn `UserConstructionScript`)