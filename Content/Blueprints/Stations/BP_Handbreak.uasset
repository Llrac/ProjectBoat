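; Handbrake station on the boat that a player takes over to slow it down, playing a brake sound on engage.
; While engaged, Tick zeroes boost duration and steadily lowers the target speed on both the boat and the BP_Speed station.
; Switch events toggle braking and swap controller or keyboard prompts, with a widget slider showing speed against maximum.
; The turn-rate boost on InteractionKey1 is disconnected.
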(event `/Game/Blueprints/Interfaces/BPI_Station.Highlight`
  (params (Enable :type Boolean) (ControllerInput :type Boolean))
  (bind _gamemanager (`self.GameManager`))
  (bind _players_input (`/Game/Blueprints/GameMode/TopDownGameMode.Players Input` (`self.GameManager`)))
  (bind _player2bp (`/Game/Blueprints/Players/BP_PlayersCombo.Player2BP` _players_input))
  (bind _player1bp (`/Game/Blueprints/Players/BP_PlayersCombo.Player1BP` _players_input))
  (if (`self.UseImagePrompts`)
    ;[1 1 1] Set Button Image
    (if ControllerInput
      (`/Game/Blueprints/Players/BP_ThirdPersonCharacter.SetButtonImage` _player1bp "/Game/Blueprints/Widgets/ButtonPrompts/Xbox_Series/XboxSeriesX_X.XboxSeriesX_X" Enable false)
      (else
        (`/Game/Blueprints/Players/BP_ThirdPersonCharacter.SetButtonImage` _player2bp "/Game/Blueprints/Widgets/ButtonPrompts/Keyboard___Mouse/Light/E_Key_Light.E_Key_Light" Enable false)))
    (elif Enable
      (if ControllerInput
        (`/Game/Blueprints/Players/BP_ThirdPersonCharacter.Set Button Prompt` _player1bp (`/Game/Blueprints/GameMode/TopDownGameMode.Interact Btn Con` _gamemanager) false)
        (else
          (`/Game/Blueprints/Players/BP_ThirdPersonCharacter.Set Button Prompt` _player2bp (`/Game/Blueprints/GameMode/TopDownGameMode.interact btn` _gamemanager) false)))
      (elif ControllerInput
        (`/Game/Blueprints/Players/BP_ThirdPersonCharacter.Set Button Prompt` _player1bp "" false)
        (else
          (`/Game/Blueprints/Players/BP_ThirdPersonCharacter.Set Button Prompt` _player2bp "" false))))))

(event `self.ReceiveBeginPlay`
  (bind _returnvalue (`GameplayStatics.GetActorOfClass` "/Game/Blueprints/GameMode/TopDownGameMode.TopDownGameMode_C"))
  (set `self.GameManager` _returnvalue)
  (bind _returnvalue_2 (`GameplayStatics.GetActorOfClass` "/Game/Blueprints/Stations/BP_Speed.BP_Speed_C"))
  (set `self.SpeedStation` _returnvalue_2)
  (bind _asimage_prompt (cast `/Game/Blueprints/Widgets/ImagePrompt` (`WidgetComponent.GetWidget` (`self.ButtonPrompt`))))
  (set `self.As Image Prompt` _asimage_prompt)
  (bind _astext_prompt (cast `/Game/Blueprints/Widgets/TextPrompt` (`WidgetComponent.GetWidget` (`self.TextPrompt`))))
  (bind _output_get (set `self.As Text Prompt` _astext_prompt))
  (`/Game/Blueprints/Widgets/TextPrompt.SetText` _output_get "Brake"))

(event `self.ReceiveTick`
  (params (DeltaSeconds :type "Float (single-precision)"))
  (bind _boat (`/Game/Blueprints/GameMode/TopDownGameMode.Boat` (`self.GameManager`)))
  (bind _bp_movementcomponent (`/Game/Blueprints/Boat/BP_Boat.BP_MovementComponent` _boat))
  (bind _returnvalue (- (`/Game/Blueprints/Boat/BP_MovementComponent.TargetSpeed` _bp_movementcomponent) (* DeltaSeconds (`self.BreakSpeed`))))
  (`|ExecutionSequence`
    (:`then_0`
      ;[1 1 1] break
      (if (`self.DoBreak`)
        (set `/Game/Blueprints/Boat/BP_MovementComponent.BoostDuration` 0.0 _bp_movementcomponent)
        (`/Game/Blueprints/Boat/BP_Boat.SetTargetSpeed` _boat _returnvalue)
        (`/Game/Blueprints/Stations/BP_Speed.Set Target Speed` (`self.SpeedStation`) _returnvalue)))
    (:`then_1`
      ;[1 1 1] update slider when controlled
      (bind _as_image_prompt (`self.As Image Prompt`)
        (:`then`
          (`/Game/Blueprints/Widgets/ImagePrompt.SetSlider` _as_image_prompt (`self.ControlledByPlayer`) (/ (`/Game/Blueprints/Boat/BP_MovementComponent.TargetSpeed` (`/Game/Blueprints/Boat/BP_Boat.BP_MovementComponent` (`/Game/Blueprints/GameMode/TopDownGameMode.Boat` (`self.GameManager`)))) (`self.MaxSpeed`)))
          (`/Game/Blueprints/Widgets/WBP_Main_HUD.UpdateHUDVariable` (`/Game/Blueprints/GameMode/TopDownGameMode.Main_HUD` (`self.GameManager`)) "NewEnumerator1"))
        (:`else`)))))

(event `/Game/Blueprints/Interfaces/BPI_RecieveInput.OnSwitchedFrom`
  (params (UsingControllerInput :type Boolean))
  (bind _gamemanager (`self.GameManager`))
  (bind _as_image_prompt (`self.As Image Prompt`))
  (bind _players_input (`/Game/Blueprints/GameMode/TopDownGameMode.Players Input` (`self.GameManager`)))
  (bind _player2bp (`/Game/Blueprints/Players/BP_PlayersCombo.Player2BP` _players_input))
  (bind _player1bp (`/Game/Blueprints/Players/BP_PlayersCombo.Player1BP` _players_input))
  ;[1 1 1] Event On Switched From
  (`GameplayStatics.PlaySoundAtLocation` "/Game/Audio/SFX/Stations/326469__miekyj__handbreak-owi.326469__miekyj__handbreak-owi" (`self.K2_GetActorLocation`) (struct) 1.0 1.0 0.0 null null null null)
  (set `self.DoBreak` true)
  (set `self.ControlledByPlayer` true)
  (if (`self.UseImagePrompts`)
    ;;[1 1 1] Show Image
    (if UsingControllerInput
      (`/Game/Blueprints/Widgets/ImagePrompt.SetImage` _as_image_prompt "/Game/Blueprints/Widgets/ButtonPrompts/Xbox_Series/XboxSeriesX_A.XboxSeriesX_A" false true)
      (`/Game/Blueprints/Players/BP_ThirdPersonCharacter.SetButtonImage` _player1bp null false false)
      (else
        (`/Game/Blueprints/Widgets/ImagePrompt.SetImage` _as_image_prompt "/Game/Blueprints/Widgets/ButtonPrompts/Keyboard___Mouse/Light/Space_Key_Light.Space_Key_Light" false true)
        (`/Game/Blueprints/Players/BP_ThirdPersonCharacter.SetButtonImage` _player2bp null false false)))
    (`/Game/Blueprints/Widgets/ImagePrompt.SetSlider` _as_image_prompt true (/ (`/Game/Blueprints/Boat/BP_MovementComponent.TargetSpeed` (`/Game/Blueprints/Boat/BP_Boat.BP_MovementComponent` (`/Game/Blueprints/GameMode/TopDownGameMode.Boat` (`self.GameManager`)))) (`self.MaxSpeed`)))
    (else
      ;;[1 1 1] Show Text (Old)
      (if UsingControllerInput
        (`/Game/Blueprints/Players/BP_ThirdPersonCharacter.Set Button Prompt` _player1bp (`/Game/Blueprints/GameMode/TopDownGameMode.Interact Btn2 Con` _gamemanager) true)
        (else
          (`/Game/Blueprints/Players/BP_ThirdPersonCharacter.Set Button Prompt` _player2bp (`/Game/Blueprints/GameMode/TopDownGameMode.Interact Btn2` _gamemanager) true))))))

(event `/Game/Blueprints/Interfaces/BPI_RecieveInput.Interaction Key_1`
  (params (Start :type Boolean) (Cancel :type Boolean))
  ;[1 1 1] Boost turnrate on break
)

(event `Set Rotation`
  (params (LeverRotation :type "Vector Structure"))
  ;[1 1 1] lever rot
  (`SceneComponent.K2_SetRelativeRotation` (`self.leverholderRoot`) (`KismetMathLibrary.MakeRotator` LeverRotation_X LeverRotation_Y LeverRotation_Z) false false))

(event `/Game/Blueprints/Interfaces/BPI_RecieveInput.OnSwitchedTo`
  (params (UseControllerInput :type Boolean))
  (bind _gamemanager (`self.GameManager`))
  (bind _as_image_prompt (`self.As Image Prompt`))
  (bind _players_input (`/Game/Blueprints/GameMode/TopDownGameMode.Players Input` (`self.GameManager`)))
  (bind _player2bp (`/Game/Blueprints/Players/BP_PlayersCombo.Player2BP` _players_input))
  (bind _player1bp (`/Game/Blueprints/Players/BP_PlayersCombo.Player1BP` _players_input))
  ;[1 1 1] Event On Switched To
  (set `self.DoBreak` false)
  (set `self.ControlledByPlayer` false)
  (if (`self.UseImagePrompts`)
    ;;[1 1 1] Hide Image
    (if UseControllerInput
      (`/Game/Blueprints/Widgets/ImagePrompt.SetImage` _as_image_prompt "/Game/Blueprints/Widgets/ButtonPrompts/Xbox_Series/XboxSeriesX_A.XboxSeriesX_A" false true)
      (`/Game/Blueprints/Players/BP_ThirdPersonCharacter.SetButtonImage` _player1bp "/Game/Blueprints/Widgets/ButtonPrompts/Xbox_Series/XboxSeriesX_X.XboxSeriesX_X" true false)
      (else
        (`/Game/Blueprints/Widgets/ImagePrompt.SetImage` _as_image_prompt "/Game/Blueprints/Widgets/ButtonPrompts/Keyboard___Mouse/Light/Space_Key_Light.Space_Key_Light" false true)
        (`/Game/Blueprints/Players/BP_ThirdPersonCharacter.SetButtonImage` _player2bp "/Game/Blueprints/Widgets/ButtonPrompts/Keyboard___Mouse/Light/E_Key_Light.E_Key_Light" true false)))
    (`/Game/Blueprints/Widgets/ImagePrompt.SetSlider` _as_image_prompt false (/ (`self.Current Target Speed`) (`self.MaxSpeed`)))
    (else
      ;;[1 1 1] Hide Text (Old)
      (if UseControllerInput
        (`/Game/Blueprints/Players/BP_ThirdPersonCharacter.Set Button Prompt` _player1bp (`/Game/Blueprints/GameMode/TopDownGameMode.Interact Btn Con` _gamemanager) false)
        (else
          (`/Game/Blueprints/Players/BP_ThirdPersonCharacter.Set Button Prompt` _player2bp (`/Game/Blueprints/GameMode/TopDownGameMode.interact btn` _gamemanager) false))))))

(fn `UserConstructionScript`)