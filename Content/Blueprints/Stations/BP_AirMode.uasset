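; BP_AirMode is a boat station that lets a player switch flying mode on and off.
; Highlight shows or hides the button prompt on Player 1 (Xbox) or Player 2 (keyboard), based on ControllerInput.
; OnSwitchedfrom flips the boat's air stabilizer mode through the game mode reference and calls ToggleWings.
; It also updates the Flying On/Off text, animates the button mesh with a reversible timeline and plays a sound.
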(event `self.ReceiveBeginPlay`
  ;[1 1 1] Set References
  (bind _returnvalue (`GameplayStatics.GetActorOfClass` "/Game/Blueprints/GameMode/TopDownGameMode.TopDownGameMode_C"))
  (set `self.GameManager` _returnvalue)
  (bind _asimage_prompt (cast `/Game/Blueprints/Widgets/ImagePrompt` (`WidgetComponent.GetWidget` (`self.Prompt`))))
  (set `self.As Image Prompt` _asimage_prompt)
  (bind _astext_prompt (cast `/Game/Blueprints/Widgets/TextPrompt` (`WidgetComponent.GetWidget` (`self.ButtonPrompt`))))
  (bind _output_get (set `self.As Text Prompt` _astext_prompt))
  (`/Game/Blueprints/Widgets/TextPrompt.SetText` _output_get "Flying Off"))

(event `/Game/Blueprints/Interfaces/BPI_Station.Highlight`
  (params (Enable :type Boolean) (ControllerInput :type Boolean))
  (bind _players_input (`/Game/Blueprints/GameMode/TopDownGameMode.Players Input` (`self.GameManager`)))
  ;[1 1 1] Highlight
  (bind _output_get (set `self.ControllerInput` ControllerInput))
  ;;[1 1 1] Set Button Image
  (if _output_get
    (`/Game/Blueprints/Players/BP_ThirdPersonCharacter.SetButtonImage` (`/Game/Blueprints/Players/BP_PlayersCombo.Player1BP` _players_input) "/Game/Blueprints/Widgets/ButtonPrompts/Xbox_Series/XboxSeriesX_X.XboxSeriesX_X" Enable false)
    (else
      (`/Game/Blueprints/Players/BP_ThirdPersonCharacter.SetButtonImage` (`/Game/Blueprints/Players/BP_PlayersCombo.Player2BP` _players_input) "/Game/Blueprints/Widgets/ButtonPrompts/Keyboard___Mouse/Light/E_Key_Light.E_Key_Light" Enable false))))

(event `/Game/Blueprints/Interfaces/BPI_RecieveInput.OnSwitchedFrom`
  (params (UsingControllerInput :type Boolean))
  (bind _staticmesh1 (`self.StaticMesh1`))
  (bind _boat (`/Game/Blueprints/GameMode/TopDownGameMode.Boat` (`self.GameManager`)))
  (bind (_relativelocation_x _relativelocation_y) (`KismetMathLibrary.BreakVector` (`SceneComponent.RelativeLocation` _staticmesh1)))
  (bind _bp_airstabilizer (`/Game/Blueprints/Boat/BP_Boat.BP_AirStabilizer` _boat))
  (bind _flyingmode (`/Game/Blueprints/Boat/BP_AirStabilizer.FlyingMode` _bp_airstabilizer))
  (bind _returnvalue (not _flyingmode))
  ;[1 1 1] Event interaction Key 1
  (if true
    (`|ExecutionSequence`
      (:`then_0`
        (`/Game/Blueprints/Boat/BP_AirStabilizer.EnableFlyingMode` _bp_airstabilizer _returnvalue)
        (`/Game/Blueprints/Boat/BP_Boat.ToggleWings` _boat _returnvalue)
        (`/Game/Blueprints/Widgets/TextPrompt.SetText` (`self.As Text Prompt`) (select `bool` _flyingmode :`false` "Flying Off" :`true` "Flying On" :!type "Text"))
        (if _flyingmode
          ;;[1 1 1] button anim
          (bind (_direction _button) (`Timeline|Timeline` :!via `PlayFromStart` :!label _label)
            (:`Update`
              _)
            (:`Finished`
              _))
          (`SceneComponent.K2_SetRelativeLocation` _staticmesh1 (`KismetMathLibrary.MakeVector` _relativelocation_x _relativelocation_y _button) false false)
          (else
            (goto _label :!via `ReverseFromEnd`))))
      (:`then_1`
        (`GameplayStatics.PlaySoundAtLocation` "/Game/Audio/SFX/Stations/SteerwheelTurn.SteerwheelTurn" (`self.K2_GetActorLocation`) (struct) 0.2 2.0 0.0 null null null null))
      (:`then_2`
        (`/Game/Blueprints/Widgets/TextPrompt.DecreaseFontScale` (`self.As Text Prompt`))))))

(fn `UserConstructionScript`)