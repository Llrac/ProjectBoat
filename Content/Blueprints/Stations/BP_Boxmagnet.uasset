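; Player-operated box magnet station that applies force to pushable physics objects inside its trigger box.
; Vertical input raises or lowers a clamped charge, which drives the magnetic field particles, beam sound volume and lever rotation.
; Box overlaps track components of BPI_Pushable actors, and Tick pushes the simulating ones along the plane's negative up vector, scaled by charge.
; Highlight and switch events swap button prompts for controller or keyboard players.
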(event `self.ReceiveBeginPlay`
  (bind _returnvalue (`GameplayStatics.GetActorOfClass` "/Game/Blueprints/GameMode/TopDownGameMode.TopDownGameMode_C"))
  (set `self.GameManager` _returnvalue)
  (`GameplayStatics.GetActorOfClass` "/Game/Blueprints/Stations/BP_Handbreak.BP_Handbreak_C")
  (bind _asimage_prompt (cast `/Game/Blueprints/Widgets/ImagePrompt` (`WidgetComponent.GetWidget` (`self.ButtonPrompt`))))
  (set `self.As Image Prompt` _asimage_prompt))

(event `/Game/Blueprints/Interfaces/BPI_Station.Highlight`
  (params (Enable :type Boolean) (ControllerInput :type Boolean))
  (bind _players_input (`/Game/Blueprints/GameMode/TopDownGameMode.Players Input` (`self.GameManager`)))
  (if ControllerInput
    (`/Game/Blueprints/Players/BP_ThirdPersonCharacter.SetButtonImage` (`/Game/Blueprints/Players/BP_PlayersCombo.Player1BP` _players_input) "/Game/Blueprints/Widgets/ButtonPrompts/Xbox_Series/XboxSeriesX_X.XboxSeriesX_X" Enable false)
    (else
      (`/Game/Blueprints/Players/BP_ThirdPersonCharacter.SetButtonImage` (`/Game/Blueprints/Players/BP_PlayersCombo.Player2BP` _players_input) "/Game/Blueprints/Widgets/ButtonPrompts/Keyboard___Mouse/Light/E_Key_Light.E_Key_Light" Enable false))))

(event `/Game/Blueprints/Interfaces/BPI_RecieveInput.OnSwitchedFrom`
  (params (UsingControllerInput :type Boolean))
  (bind _as_image_prompt (`self.As Image Prompt`))
  (bind _players_input (`/Game/Blueprints/GameMode/TopDownGameMode.Players Input` (`self.GameManager`)))
  (set `self.ControlledByPlayer` true)
  (if UsingControllerInput
    (`/Game/Blueprints/Widgets/ImagePrompt.SetImage` _as_image_prompt "/Game/Blueprints/Widgets/ButtonPrompts/Others/Xbox_One/XboxOne_Left_Stick.XboxOne_Left_Stick" true false)
    (`/Game/Blueprints/Players/BP_ThirdPersonCharacter.SetButtonImage` (`/Game/Blueprints/Players/BP_PlayersCombo.Player1BP` _players_input) null false false)
    (else
      (`/Game/Blueprints/Widgets/ImagePrompt.SetImage` _as_image_prompt "/Game/Blueprints/Widgets/ButtonPrompts/Keyboard___Mouse/Light/W_Key_Light.W_Key_Light" true false)
      (`/Game/Blueprints/Players/BP_ThirdPersonCharacter.SetButtonImage` (`/Game/Blueprints/Players/BP_PlayersCombo.Player2BP` _players_input) null false false))))

(event `/Game/Blueprints/Interfaces/BPI_RecieveInput.2Vector Input_1`
  (params (`Action Value X` :type "Float (double-precision)") (`Action Value Y` :type "Float (double-precision)"))
  (bind _fsx_magneticfield (`self.FSX_MagneticField`))
  (bind _returnvalue (/ (`self.Current Target Charge`) (`self.Max Charge`)))
  (`|ExecutionSequence`
    (:`then_0`
      (set `self.Input` (`KismetMathLibrary.FClamp` `Action Value Y` -1.0)))
    (:`then_1`
      ;[1 1 1] set new charge
      (set `self.Current Target Charge` (`KismetMathLibrary.FClamp` (+ (* (`GameplayStatics.GetWorldDeltaSeconds`) (* (`self.Input`) 2000.0)) (`self.Current Target Charge`)) 0.0 (`self.Max Charge`)))
      ;[1 1 1] Particle Variables
      ;;[1 1 1] Set Percentage
      (bind _output_get (set `self.ParticleAlpha` (* _returnvalue 0.9)))
      (bind _output_get_2 (set `self.DownForce` (* _returnvalue -1000.0)))
      (`|ExecutionSequence`
        (:`then_0`
          (`NiagaraComponent.SetVariableLinearColor` _fsx_magneticfield "Color" (make `LinearColor` 0.0 0.65 1.0 _output_get))
          (`NiagaraComponent.SetVariableVec3` _fsx_magneticfield "Force" (`KismetMathLibrary.MakeVector` 0.0 0.0 _output_get_2)))
        (:`then_1`
          (`AudioComponent.SetVolumeMultiplier` (`self.MagnetBeam_Cue`) (* _returnvalue 0.5)))))
    (:`then_2`
      ;[1 1 1] Rotation for levers
      (`SceneComponent.K2_SetRelativeRotation` (`self.leverholderRoot`) (`KismetMathLibrary.MakeRotator` (* (/ (`self.Current Target Charge`) (`self.Max Charge`)) 120.0)) false false))))

(event `self.ReceiveTick`
  (params (DeltaSeconds :type "Float (single-precision)"))
  ;[1 1 1] Force towards area down foreach item in range
  (for _array_element (`self.ActorsInRange`)
    (if (`SceneComponent.IsSimulatingPhysics` _array_element "None")
      (`PrimitiveComponent.AddForce` _array_element (* (* (`KismetMathLibrary.Normal` (`SceneComponent.GetUpVector` (`self.Plane`)) 0.01) -1) (`self.Current Target Charge`)) "None" false))))

(event `/Game/Blueprints/Interfaces/BPI_RecieveInput.OnSwitchedTo`
  (params (UseControllerInput :type Boolean))
  (bind _as_image_prompt (`self.As Image Prompt`))
  (bind _players_input (`/Game/Blueprints/GameMode/TopDownGameMode.Players Input` (`self.GameManager`)))
  (set `self.ControlledByPlayer` false)
  (if UseControllerInput
    (`/Game/Blueprints/Widgets/ImagePrompt.SetImage` _as_image_prompt "/Game/Blueprints/Widgets/ButtonPrompts/Xbox_Series/XboxSeriesX_A.XboxSeriesX_A" false true)
    (`/Game/Blueprints/Players/BP_ThirdPersonCharacter.SetButtonImage` (`/Game/Blueprints/Players/BP_PlayersCombo.Player1BP` _players_input) "/Game/Blueprints/Widgets/ButtonPrompts/Xbox_Series/XboxSeriesX_X.XboxSeriesX_X" true false)
    (else
      (`/Game/Blueprints/Widgets/ImagePrompt.SetImage` _as_image_prompt "/Game/Blueprints/Widgets/ButtonPrompts/Keyboard___Mouse/Light/Space_Key_Light.Space_Key_Light" false true)
      (`/Game/Blueprints/Players/BP_ThirdPersonCharacter.SetButtonImage` (`/Game/Blueprints/Players/BP_PlayersCombo.Player2BP` _players_input) "/Game/Blueprints/Widgets/ButtonPrompts/Keyboard___Mouse/Light/E_Key_Light.E_Key_Light" true false))))

(event `self.Box.OnComponentBeginOverlap`
  (params (OverlappedComponent :type "PrimitiveComponent Object Reference") (OtherActor :type "Actor Object Reference") (OtherComp :type "PrimitiveComponent Object Reference") (OtherBodyIndex :type Integer) (bFromSweep :type Boolean) (SweepResult :type "HitResult Structure (by ref)"))
  ;[1 1 1] add or remove pushable objects withing forcearea
  (if (`KismetSystemLibrary.DoesImplementInterface` OtherActor "/Game/Blueprints/Interfaces/BPI_Pushable.BPI_Pushable_C")
    (`KismetArrayLibrary.Array_AddUnique` (`self.ActorsInRange`) OtherComp)))

(event `self.Box.OnComponentEndOverlap`
  (params (OverlappedComponent :type "PrimitiveComponent Object Reference") (OtherActor :type "Actor Object Reference") (OtherComp :type "PrimitiveComponent Object Reference") (OtherBodyIndex :type Integer))
  (bind _actorsinrange (`self.ActorsInRange`))
  ;[1 1 1] add or remove pushable objects withing forcearea
  (if (`KismetArrayLibrary.Array_Contains` _actorsinrange OtherComp)
    (`KismetArrayLibrary.Array_RemoveItem` _actorsinrange OtherComp)))

(fn `UserConstructionScript`)