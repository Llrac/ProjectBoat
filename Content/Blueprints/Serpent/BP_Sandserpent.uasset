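; Sea serpent enemy that roams a radius around its spawn, chases the player's boat when in range, attacks it and flees.
; A Passive/Chase/Attack/Flee state machine on Tick sets a target point, with chase shadowing the nearer side ahead of the boat.
; An invisible-style lead Sphere is force-driven toward that target, and the serpent mesh is pushed and rotated to trail it.
; Box overlap lands attacks, currently only sound and debug print; repeated hits trigger fleeing.
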(event `Passive Behavior`
  (bind _startchaseque (`self.StartChaseQue`))
  ;[1 1 1] Move around area
  (if (< (`KismetMathLibrary.VSize` (- (`SceneComponent.K2_GetComponentLocation` (`self.Sphere`)) (`self.BoatLocation`))) (`self.Aggro Range`))
    (`self.SetBehavior` "NewEnumerator2") ; start chase
    (set `AudioComponent.PitchMultiplier` (`KismetMathLibrary.RandomFloatInRange` 0.8 1.2) _startchaseque)
    (`AudioComponent.Play` _startchaseque 0.0)
    (else
      ;;[1 1 1] new target in radius
      (if (`self.IsNearTargetLocation`)
        (bind _newpoint (`self.Get New Roam Point` (`self.RoamZone Radius`)))
        (set `self.TargetPoint` (`KismetMathLibrary.Conv_Vector2DToVector` _newpoint))))))

(event `Chase Behavior`
  (bind (_leftof _chasepointleft _chasepointright) (`self.GetBoatFollowSide`))
  ;[1 1 1] Move towards ship and follow side
  (if _leftof
    (set `self.TargetPoint` _chasepointleft)
    (else
      (set `self.TargetPoint` _chasepointright)))
  (if (<= (`self.Distance to Target`) (`self.Is Near Target Range`))
    (set `self.ChaseTimerToAttack` (- (`self.ChaseTimerToAttack`) (`GameplayStatics.GetWorldDeltaSeconds`)))
    (if (<= (`self.ChaseTimerToAttack`) 0.0)
      (set `self.ChaseTimerToAttack` (`self.MaxChaseTime`))
      (`self.SetBehavior` "NewEnumerator3")
      (`GameplayStatics.PlaySoundAtLocation` "/Game/Audio/SFX/Serpent/SerpentStartAttack.SerpentStartAttack" (`SceneComponent.K2_GetComponentLocation` (`self.SM_Sandserpent`)) (struct) 0.5 (`KismetMathLibrary.RandomFloatInRange` 0.8 1.2) 0.0 null null null null))
    (elif (> (`self.Distance to Target`) (`self.Aggro Range`))
      (`self.SetBehavior` "NewEnumerator4")
      (`GameplayStatics.PlaySoundAtLocation` "/Game/Audio/SFX/Serpent/SerpentFlee.SerpentFlee" (`SceneComponent.K2_GetComponentLocation` (`self.SM_Sandserpent`)) (struct) 1.0 (`KismetMathLibrary.RandomFloatInRange` 0.8 1.2) 0.0 null null null null))))

(event `self.ReceiveBeginPlay`
  (bind _returnvalue (`SceneComponent.K2_GetComponentLocation` (`self.DefaultSceneRoot`)))
  ;[1 1 1] Set Variables
  (bind _returnvalue_2 (`GameplayStatics.GetActorOfClass` "/Game/Blueprints/GameMode/TopDownGameMode.TopDownGameMode_C"))
  (bind _output_get (set `self.GameManager` _returnvalue_2))
  (bind _boat (`/Game/Blueprints/GameMode/TopDownGameMode.Boat` _output_get)
    (:`then`
      (set `self.Boat` _boat))
    (:`else`
      (bind _returnvalue_3 (`GameplayStatics.GetActorOfClass` "/Game/Blueprints/Boat/BP_Boat.BP_Boat_C"))
      (set `self.Boat` _returnvalue_3)))
  (set `self.BoatLocation` (`self.K2_GetActorLocation` (`self.Boat`)))
  (bind _dist (`self.Get Distance And Rot from ControlSphere`))
  (bind _output_get_2 (set `self.Distance to ControlSphere` _dist))
  (set `self.TargetDistance From ControlSphere` (`KismetMathLibrary.VSize` _output_get_2))
  (set `self.RoamZone 2D Origin` (`KismetMathLibrary.Conv_VectorToVector2D` _returnvalue))
  (set `self.TargetPoint` _returnvalue)
  (bind _zone (`self.Zone`)
    (:`then`
      _)
    (:`else`
      _))
  (set `self.RoamZone Radius` 20000.0))

(event `Attack Behavior`
  (`|ExecutionSequence`
    (:`then_0`
      (set `self.TargetPoint` (`self.BoatLocation`))
      (set `self.Attackframes` true))))

(event `self.Box.OnComponentBeginOverlap`
  (params (OverlappedComponent :type "PrimitiveComponent Object Reference") (OtherActor :type "Actor Object Reference") (OtherComp :type "PrimitiveComponent Object Reference") (OtherBodyIndex :type Integer) (bFromSweep :type Boolean) (SweepResult :type "HitResult Structure (by ref)"))
  (if (and (== OtherActor (`self.Boat`)) (`self.Attackframes`))
    (set `self.Attackframes` false)
    (set `self.BahaviorState` "NewEnumerator4")
    (`GameplayStatics.PlaySoundAtLocation` "/Game/Audio/SFX/Serpent/SerpentLandAttack.SerpentLandAttack" (`SceneComponent.K2_GetComponentLocation` (`self.SM_Sandserpent`)) (struct) 0.5 (`KismetMathLibrary.RandomFloatInRange` 0.8 1.2) 0.0 null null null null)
    (`KismetSystemLibrary.PrintString` "serpent attack" true true (struct :`G` 0.198949 :`B` 0.260417 :`A` 1.0) 2.0 "(::(::(")))

(event `Flee Bahavior`
  (bind _returnvalue (- (`SceneComponent.K2_GetComponentLocation` (`self.Sphere`)) (`self.BoatLocation`)))
  ;[1 1 1] Flee
  ;;[1 1 1] move away fromplayer toward middle of passive area
  (if (> (`KismetMathLibrary.VSize` _returnvalue) (`self.RoamZone Radius`))
    (set `self.TargetPoint` (`KismetMathLibrary.Conv_Vector2DToVector` (`self.RoamZone 2D Origin`))) ; To startpoint
    (else
      (set `self.TargetPoint` (* (`KismetMathLibrary.Normal` _returnvalue 1.0) (`self.FleeDistance`))) ; Away from player
    ))
  ;;;[1 1 1] ResetBehavior
  (if (`self.IsNearTargetLocation`)
    (`self.SetBehavior` "NewEnumerator1")))

(event `self.ReceiveTick`
  (params (DeltaSeconds :type "Float (single-precision)"))
  (bind (_targetpoint_x _targetpoint_y) (`KismetMathLibrary.BreakVector` (`self.TargetPoint`)))
  (bind _returnvalue (- (`self.TargetPoint`) (`SceneComponent.K2_GetComponentLocation` (`self.Sphere`))))
  (bind _returnvalue_2 (`KismetMathLibrary.VSize2D` (`KismetMathLibrary.Conv_VectorToVector2D` _returnvalue)))
  (set `self.BoatLocation` (`self.K2_GetActorLocation` (`self.Boat`)))
  ;[1 1 1] Base Move Towards Controlcube
  ;;[1 1 1] Rotation
  (bind (_dist _zrot _xrot) (`self.Get Distance And Rot from ControlSphere`))
  (set `self.XRot` _xrot)
  (set `self.ZRot` _zrot)
  (set `self.Distance to ControlSphere` _dist)
  (set `self.ForwardForce` (* (`KismetMathLibrary.Normal` (`self.Distance to ControlSphere`) 1.0) (`self.MoveSpeed`)))
  (`SceneComponent.K2_SetWorldRotation` (`self.SM_Sandserpent`) (`KismetMathLibrary.MakeRotator` (`self.XRot`) 0.0 (`self.ZRot`)) false false)
  ;;[1 1 1] MoveForce
  (if (> (`KismetMathLibrary.VSize` (`self.Distance to ControlSphere`)) (`self.TargetDistance From ControlSphere`))
    (`PrimitiveComponent.AddForce` (`self.SM_Sandserpent`) (`self.ForwardForce`) "None" true) ; Forward
    (else
      (`PrimitiveComponent.AddForce` (`self.SM_Sandserpent`) (* (`self.ForwardForce`) -0.5) "None" true) ; Slight Back
    ))
  (`|ExecutionSequence`
    (:`then_0`
      (switch `/Game/Blueprints/Serpent/SerpentBahaviorEnum` (`self.BahaviorState`)
        (:`NewEnumerator1`
          (`self.Passive Behavior`)
          (set `self.MoveSpeed` 4000.0))
        (:`NewEnumerator2`
          (`self.Chase Behavior`)
          (set `self.MoveSpeed` 8000.0))
        (:`NewEnumerator3`
          (`self.Attack Behavior`)
          (set `self.MoveSpeed` 8000.0))
        (:`NewEnumerator4`
          (`self.Flee Bahavior`)
          (set `self.MoveSpeed` 8000.0))))
    (:`then_1`
      ;[1 1 1] Sphere move towards target point
      (set `self.Distance to Target` _returnvalue_2)
      (if (> _returnvalue_2 (/ (`self.Is Near Target Range`) 10.0))
        (`PrimitiveComponent.AddForce` (`self.Sphere`) (`KismetMathLibrary.Conv_Vector2DToVector` (`KismetMathLibrary.Conv_VectorToVector2D` (* (`KismetMathLibrary.Normal` _returnvalue 1.0) (* (`self.MoveSpeed`) 0.5)))) "None" true)))
    (:`then_2`
      (if (`self.Debug?`)
        (`KismetSystemLibrary.DrawDebugPoint` (`KismetMathLibrary.MakeVector` _targetpoint_x _targetpoint_y 2500.0) 5.0 (struct :`R` 1.0 :`B` 0.067137 :`A` 1.0) 1.0)))))

(event `SetBehavior`
  (params (Behavior :type "/Game/Blueprints/Serpent/SerpentBahaviorEnum Enum" :default "NewEnumerator1"))
  (set `self.BahaviorState` Behavior))

(event `/Game/Blueprints/Interfaces/BPI_HitByCannon.Hit`
  (bind _serpenthit_cue (`self.SerpentHit_Cue`))
  (bind _hits_to_flee (`self.Hits to Flee`))
  (if (not (`AudioComponent.IsPlaying` _serpenthit_cue))
    (`AudioComponent.SetPitchMultiplier` _serpenthit_cue (`KismetMathLibrary.RandomFloatInRange` 0.8 1.2))
    (`AudioComponent.Play` (`self.SerpentHit_Cue`) 0.0))
  (`/Engine/EditorBlueprintResources/StandardMacros.DecrementInt` _hits_to_flee
    (:`  `
      (if (<= _hits_to_flee 0)
        (`self.SetBehavior` "NewEnumerator4")
        (set `self.Hits to Flee` 10)
        (`GameplayStatics.PlaySoundAtLocation` "/Game/Audio/SFX/Serpent/SerpentFlee.SerpentFlee" (`SceneComponent.K2_GetComponentLocation` (`self.SM_Sandserpent`)) (struct) 0.5 (`KismetMathLibrary.RandomFloatInRange` 0.8 1.2) 0.0 null null null null)))))

(fn `Get Distance And Rot from ControlSphere`
  (returns (dist :type "Vector Structure") (zrot :type "Float (double-precision)") (xrot :type "Float (double-precision)"))
  (bind _returnvalue (`SceneComponent.K2_GetComponentLocation` (`self.SM_Sandserpent`)))
  (bind _returnvalue_2 (`SceneComponent.K2_GetComponentLocation` (`self.Sphere`)))
  (bind (_returnvalue_roll _returnvalue_pitch _returnvalue_yaw) (`KismetMathLibrary.BreakRotator` (`KismetMathLibrary.FindLookAtRotation` _returnvalue_2 _returnvalue)))
  (return (- _returnvalue_2 _returnvalue) (+ _returnvalue_yaw 90.0) _returnvalue_pitch))

(fn `Get New Roam Point`
  (params (Radius :type "Float (double-precision)"))
  (returns (NewPoint :type "Vector2D Structure"))
  (bind (_returnvalue_x _returnvalue_y) (`KismetMathLibrary.BreakVector` (`KismetMathLibrary.RandomUnitVector`)))
  (return (+ (`self.RoamZone 2D Origin`) (`KismetMathLibrary.Conv_VectorToVector2D` (* (`KismetMathLibrary.MakeVector` _returnvalue_x _returnvalue_y) (`KismetMathLibrary.RandomFloatInRange` (/ Radius 3.0) Radius))))))

(fn `GetBoatFollowSide`
  (returns (LeftOf :type Boolean) (ChasePointLeft :type "Vector Structure") (ChasePointRight :type "Vector Structure"))
  (locals (TracePointLeft :type "Vector Structure") (TracePointRight :type "Vector Structure" :default (0.0 0.0 0.0)) (LengthLeft :type "Float (single-precision)" :default 0.0) (LengthRight :type "Float (single-precision)" :default 0.0))
  (bind (_tracepointright_x _tracepointright_y) (`KismetMathLibrary.BreakVector` (`local.TracePointRight`)))
  (bind _boat (`self.Boat`))
  (bind (_tracepointleft_x _tracepointleft_y) (`KismetMathLibrary.BreakVector` (`local.TracePointLeft`)))
  (bind _returnvalue (`self.K2_GetActorLocation` _boat))
  (bind _returnvalue_2 (* (`self.GetActorRightVector` _boat) (`self.Boat Chase SideDistance`)))
  (bind _returnvalue_3 (* (`self.GetActorForwardVector` _boat) 8000.0))
  (set `local.TracePointRight` (+ _returnvalue_3 _returnvalue_2 _returnvalue))
  (set `local.TracePointLeft` (+ _returnvalue_3 (* _returnvalue_2 -1) _returnvalue))
  (if (`self.Debug?`)
    ;[1 1 1] debug draws
    (`KismetSystemLibrary.DrawDebugPoint` (`KismetMathLibrary.MakeVector` _tracepointright_x _tracepointright_y 2500.0) 5.0 (struct :`R` 1.0 :`B` 0.962854 :`A` 1.0) 1.0)
    (`KismetSystemLibrary.DrawDebugPoint` (`KismetMathLibrary.MakeVector` _tracepointleft_x _tracepointleft_y 2500.0) 5.0 (struct :`R` 1.0 :`B` 0.962854 :`A` 1.0) 1.0))
  ;[1 1 1] distances to left and rightside of boat
  (set `local.LengthLeft` (`KismetMathLibrary.VSize` (- (`SceneComponent.K2_GetComponentLocation` (`self.Sphere`)) (`local.TracePointLeft`))))
  (set `local.LengthRight` (`KismetMathLibrary.VSize` (- (`SceneComponent.K2_GetComponentLocation` (`self.Sphere`)) (`local.TracePointRight`))))
  (if (> (`local.LengthLeft`) (`local.LengthRight`))
    (return false (`KismetMathLibrary.Conv_Vector2DToVector` (`KismetMathLibrary.Conv_VectorToVector2D` (`local.TracePointLeft`))) (`KismetMathLibrary.Conv_Vector2DToVector` (`KismetMathLibrary.Conv_VectorToVector2D` (`local.TracePointRight`))))
    (else
      (return true (`KismetMathLibrary.Conv_Vector2DToVector` (`KismetMathLibrary.Conv_VectorToVector2D` (`local.TracePointLeft`))) (`KismetMathLibrary.Conv_Vector2DToVector` (`KismetMathLibrary.Conv_VectorToVector2D` (`local.TracePointRight`)))))))

(fn `IsNearTargetLocation`
  (returns (ReturnValue :type Boolean))
  (return (< (`KismetMathLibrary.VSize2D` (`KismetMathLibrary.Conv_VectorToVector2D` (- (`self.TargetPoint`) (`SceneComponent.K2_GetComponentLocation` (`self.Sphere`))))) (`self.Is Near Target Range`))))

(fn `UserConstructionScript`)