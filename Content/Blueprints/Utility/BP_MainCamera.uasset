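; Shared two-player camera that takes over the first player controller's view and follows the midpoint between both characters.
; Each tick it moves the PlayersInput middle-point reference to that midpoint, rotates toward it and interpolates its position above it.
; Follow speed eases between three tiers based on horizontal distance, so the camera slows when near.
; The spring-arm attachment and RangeCheck hysteresis helpers are not called here.
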(event `self.ReceiveBeginPlay`
  ;[1 1 1] makes camera not follow player
  (`PlayerController.SetViewTargetWithBlend` (`GameplayStatics.GetPlayerController` 0) self 0.0 "VTBlend_Linear" 0.0 false)
  ;[1 1 1] manager ref
  (bind _returnvalue (`GameplayStatics.GetActorOfClass` "/Game/Blueprints/GameMode/TopDownGameMode.TopDownGameMode_C"))
  (bind _output_get (set `self.GameManager` _returnvalue))
  (set `self.Ref_MiddlePointReference` (`/Game/Blueprints/Players/BP_PlayersCombo.Middle Point Reference` (`/Game/Blueprints/GameMode/TopDownGameMode.Players Input` _output_get))))

(event `self.ReceiveTick`
  (params (DeltaSeconds :type "Float (single-precision)"))
  (bind _defaultsceneroot (`self.DefaultSceneRoot`))
  (bind (_returnvalue_x _returnvalue_y) (`KismetMathLibrary.BreakVector` (`SceneComponent.K2_GetComponentLocation` (`self.DefaultSceneRoot`))))
  (bind (_returnvalue_x_2 _returnvalue_y_2 _returnvalue_z) (`KismetMathLibrary.BreakVector` (`SceneComponent.K2_GetComponentLocation` (`self.DefaultSceneRoot`))))
  (bind (_returnvalue_x_3 _returnvalue_y_3 _returnvalue_z_2) (`KismetMathLibrary.BreakVector` (`SceneComponent.K2_GetComponentLocation` (`self.Ref_MiddlePointReference`))))
  (bind (_returnvalue_x_4 _returnvalue_y_4) (`KismetMathLibrary.BreakVector` (`SceneComponent.K2_GetComponentLocation` (`self.DefaultSceneRoot`))))
  (bind (_returnvalue_x_5 _returnvalue_y_5) (`KismetMathLibrary.BreakVector` (`SceneComponent.K2_GetComponentLocation` (`self.DefaultSceneRoot`))))
  (bind (_returnvalue_roll _returnvalue_pitch _returnvalue_yaw) (`KismetMathLibrary.BreakRotator` (`KismetMathLibrary.FindLookAtRotation` (`SceneComponent.K2_GetComponentLocation` _defaultsceneroot) (`SceneComponent.K2_GetComponentLocation` (`self.Ref_MiddlePointReference`)))))
  (bind _returnvalue (/ (+ (`self.K2_GetActorLocation` (`/Game/Blueprints/Players/BP_PlayersCombo.Player2Character` (`/Game/Blueprints/GameMode/TopDownGameMode.Players Input` (`self.GameManager`)))) (`self.K2_GetActorLocation` (`/Game/Blueprints/Players/BP_PlayersCombo.Player1Character` (`/Game/Blueprints/GameMode/TopDownGameMode.Players Input` (`self.GameManager`))))) 2))
  (`SceneComponent.K2_SetWorldLocation` (`self.Ref_MiddlePointReference`) _returnvalue false false)
  (`|ExecutionSequence`
    (:`then_0`
      (`SceneComponent.K2_SetWorldRotation` _defaultsceneroot (`KismetMathLibrary.MakeRotator` _returnvalue_roll _returnvalue_pitch _returnvalue_yaw) false false))
    (:`then_1`
      (if (< (`KismetMathLibrary.VSize` (- (`KismetMathLibrary.MakeVector` (.x _returnvalue) (.y _returnvalue)) (`KismetMathLibrary.MakeVector` _returnvalue_x_4 _returnvalue_y_4))) (+ (`self.VeryCloseRange`) 0.0))
        (set `self.FollowSpeed` (`KismetMathLibrary.FInterpTo` (`self.FollowSpeed`) 0.1 (`GameplayStatics.GetWorldDeltaSeconds`) 1.0))
        (elif (< (`KismetMathLibrary.VSize` (- (`KismetMathLibrary.MakeVector` (.x _returnvalue) (.y _returnvalue)) (`KismetMathLibrary.MakeVector` _returnvalue_x_5 _returnvalue_y_5))) (+ (`self.CloseRange`) (`self.CloseRangeThreshold`)))
          (set `self.FollowSpeed` (`KismetMathLibrary.FInterpTo` (`self.FollowSpeed`) 0.5 (`GameplayStatics.GetWorldDeltaSeconds`) 1.0))
          (elif (not (< (`KismetMathLibrary.VSize` (- (`KismetMathLibrary.MakeVector` (.x _returnvalue) (.y _returnvalue)) (`KismetMathLibrary.MakeVector` _returnvalue_x _returnvalue_y))) (+ (`self.CloseRange`) (`self.CloseRangeThreshold`))))
            (set `self.FollowSpeed` (`KismetMathLibrary.FInterpTo` (`self.FollowSpeed`) 1.25 (`GameplayStatics.GetWorldDeltaSeconds`) 1.0))))))
    (:`then_2`
      (if (<= (`self.FollowSpeed`) 0.1)
        _
        (else
          _))
      (`SceneComponent.K2_SetWorldLocation` (`self.DefaultSceneRoot`) (`KismetMathLibrary.MakeVector` (`KismetMathLibrary.FInterpTo` _returnvalue_x_2 _returnvalue_x_3 (`GameplayStatics.GetWorldDeltaSeconds`) (`self.FollowSpeed`)) (`KismetMathLibrary.FInterpTo` _returnvalue_y_2 _returnvalue_y_3 (`GameplayStatics.GetWorldDeltaSeconds`) (`self.FollowSpeed`)) (`KismetMathLibrary.FInterpTo` _returnvalue_z (+ _returnvalue_z_2 500.0) (`GameplayStatics.GetWorldDeltaSeconds`) (`self.FollowSpeed`))) false false))))

(fn `RangeCheck`
  (params (CurrentSpeed :type "Float (double-precision)"))
  (`|ExecutionSequence`
    (:`then_0`
      (if (< CurrentSpeed 0.5)
        (set `self.CloseRangeThreshold` (`self.Range Threshold`))
        (elif (> CurrentSpeed 0.5)
          (set `self.CloseRangeThreshold` (* (`self.Range Threshold`) -1.0))
          (else
            (set `self.CloseRangeThreshold` 0.0)))))
    (:`then_1`
      (set `self.LastSpeed` CurrentSpeed))))

(fn `SetSpringArmConnection`
  (params (NewSpringArm :type "SpringArmComponent Object Reference"))
  (`self.K2_AttachToComponent` NewSpringArm "None" "SnapToTarget" "SnapToTarget" "SnapToTarget")
  (set `self.Connected Spring Arm` NewSpringArm))

(fn `UserConstructionScript`)