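; Lighting manager that drives the pitch of a Directional Light at runtime, apparently intended as a moving sun.
; On BeginPlay it caches the Directional Light found in the level.
; Each Tick sets pitch to delta seconds minus current pitch, which flips its sign rather than steadily advancing it, keeping roll and yaw.
; A follow-up check resets pitch to 180 if it reaches -180 or lower.
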(event `self.ReceiveBeginPlay`
  (bind _returnvalue (`GameplayStatics.GetActorOfClass` "/Script/Engine.DirectionalLight"))
  (set `self.Ref_DirectionLight` _returnvalue))

(event `self.ReceiveTick`
  (params (DeltaSeconds :type "Float (single-precision)"))
  (bind _rootcomponent (`Actor.RootComponent` (`self.Ref_DirectionLight`)))
  (bind (_returnvalue_roll _returnvalue_pitch _returnvalue_yaw) (`KismetMathLibrary.BreakRotator` (`SceneComponent.K2_GetComponentRotation` _rootcomponent)))
  (`SceneComponent.K2_SetWorldRotation` _rootcomponent (`KismetMathLibrary.MakeRotator` _returnvalue_roll (- (* DeltaSeconds 1.0) _returnvalue_pitch) _returnvalue_yaw) false false)
  (if (<= _returnvalue_pitch -180.0)
    (`SceneComponent.K2_SetWorldRotation` _rootcomponent (`KismetMathLibrary.MakeRotator` _returnvalue_roll 180.0 _returnvalue_yaw) false false)))

(fn `UserConstructionScript`)