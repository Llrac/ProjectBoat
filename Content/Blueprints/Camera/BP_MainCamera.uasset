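; Main camera for a two-player boat game, taking over player 0's view and updating every tick once references are cached.
; Its position eases toward the player-count-weighted average of occupied BP_FocusHitbox views (default FocusViewer if none), plus a boat-aligned offset driven by speed and turning.
; It turns toward the players' midpoint plus a speed, turn and hitbox look-at offset, twice as fast while airborne.
; SetCamFollowSpeed and SetCamLocation are unused.
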(event `self.ReceiveBeginPlay`
  (`|ExecutionSequence`
    (:`then_0`
      (`KismetSystemLibrary.DelayUntilNextTick`)
      ;[1 1 1] Makes Camera NOT Follow Player
      (`PlayerController.SetViewTargetWithBlend` (`GameplayStatics.GetPlayerController` 0) self 0.0 "VTBlend_Linear" 0.0 false)
      (`|ExecutionSequence`
        (:`then_0`
          ;[1 1 1] Get References
          (bind _returnvalue (`GameplayStatics.GetActorOfClass` "/Game/Blueprints/GameMode/TopDownGameMode.TopDownGameMode_C"))
          (set `self.Ref_GameManager` _returnvalue))
        (:`then_1`
          (bind _returnvalue_2 (`GameplayStatics.GetActorOfClass` "/Game/Blueprints/Boat/BP_Boat.BP_Boat_C"))
          (set `self.Ref_Boat` _returnvalue_2))
        (:`then_2`
          (bind _outactors (`GameplayStatics.GetAllActorsOfClass` "/Game/Blueprints/Camera/BP_FocusHitbox.BP_FocusHitbox_C"))
          (set `self.FocusHitboxes` _outactors))
        (:`then_3`
          (set `self.HasRefs` true))))))

(event `self.ReceiveTick`
  (params (DeltaSeconds :type "Float (single-precision)"))
  (`|ExecutionSequence`
    (:`then_0`
      (`self.FocusViewer`
        (:`then`)
        (:`else`
          (bind _ref_boat (`self.Ref_Boat`)
            (:`then`
              (`/Game/Blueprints/Boat/BP_Boat.GetFocusView` _ref_boat))
            (:`else`)))))
    (:`then_1`
      (if (`self.HasRefs`)
        (`self.CalculateOffsets`)
        (`self.Set Middle Point`)
        (`self.Set Cam Focus Location`)
        (`self.SetCamRotation`)))))

(event `Set Default Focus Viewer`
  (params (`Focus Viewer` :type "/Game/Blueprints/Camera/SC_FocusViewer Object Reference"))
  (set `self.FocusViewer` `Focus Viewer`))

(fn `CalculateOffsets`
  (locals (SumOfCamOffset :type "Vector Structure") (NumOfCamOffset :type Integer))
  (bind _ref_boat (`self.Ref_Boat`)
    (:`then`
      (`|ExecutionSequence`
        (:`then_0`
          (set `local.NumOfCamOffset` 0)
          (for _array_element (`self.FocusHitboxes`)
            (if (and (`/Game/Blueprints/Camera/BP_FocusHitbox.UseCamOffset?` _array_element) (!= (`/Game/Blueprints/Camera/BP_FocusHitbox.NumOfPlayers` _array_element) 0))
              (`/Engine/EditorBlueprintResources/StandardMacros.IncrementInt` (`local.NumOfCamOffset`)
                (:`  `
                  (set `local.SumOfCamOffset` (+ (`/Game/Blueprints/Camera/BP_FocusHitbox.CameraLookAtOffset` _array_element) (`local.SumOfCamOffset`))))))))
        (:`then_1`
          (bind _bp_movementcomponent (`/Game/Blueprints/Boat/BP_Boat.BP_MovementComponent` _ref_boat))
          (bind _returnvalue (`KismetMathLibrary.FClamp` (`/Game/Blueprints/Boat/BP_MovementComponent.CurrentSpeed` _bp_movementcomponent) (`self.MinSpeedZoomOutDistance`) (`self.MaxSpeedZoomOutDistance`)))
          (bind _returnvalue_2 (`self.K2_GetActorRotation` _ref_boat))
          (set `self.CameraOffset` (`KismetMathLibrary.GreaterGreater_VectorRotator` (* (+ (* (`KismetMathLibrary.MakeVector` _returnvalue (`/Game/Blueprints/Boat/BP_MovementComponent.CurrentAngularSpeed` _bp_movementcomponent) _returnvalue) (`KismetMathLibrary.MakeVector` (`self.CamForwardFactor`) (`self.CamHorizontalFactor`) (`self.CamVerticalFactor`))) (`self.CamBaseOffset`)) (-1.0 -1.0 1.0)) _returnvalue_2))
          (bind _bp_movementcomponent_2 (`/Game/Blueprints/Boat/BP_Boat.BP_MovementComponent` _ref_boat))
          (bind _returnvalue_3 (* (`KismetMathLibrary.FClamp` (`/Game/Blueprints/Boat/BP_MovementComponent.CurrentSpeed` _bp_movementcomponent_2) (`self.MinSpeedLookUp`) (`self.MaxSpeedLookUp`)) (`self.SpeedLookUpFactor`)))
          (set `self.MiddlePointOffset` (`KismetMathLibrary.GreaterGreater_VectorRotator` (+ (* (`KismetMathLibrary.MakeVector` (`self.BaseForwardFactor`) (`self.BaseHorizontalFactor`) (`self.BaseVerticalFactor`)) (`self.LookAtOffset`)) (`KismetMathLibrary.MakeVector` 0.0 (* _returnvalue_3 (`/Game/Blueprints/Boat/BP_MovementComponent.CurrentAngularSpeed` _bp_movementcomponent_2) (`self.TurnSpeedFactor`)) _returnvalue_3) (`local.SumOfCamOffset`)) _returnvalue_2)))))
    (:`else`)))

(fn `Set Cam Focus Location`
  (locals (TargetLocation :type "Vector Structure") (SumOfPlayers :type Integer))
  (bind _sumofplayers (`local.SumOfPlayers`))
  ;[1 1 1] Calculate Target Location
  ;;[1 1 1] The sum of all FocusViewers locations
  (for _array_element (`self.FocusHitboxes`)
    (bind _numofplayers (`/Game/Blueprints/Camera/BP_FocusHitbox.NumOfPlayers` _array_element))
    (if (!= _numofplayers 0)
      (set `local.TargetLocation` (+ (`local.TargetLocation`) (* (`SceneComponent.K2_GetComponentLocation` (`/Game/Blueprints/Camera/BP_FocusHitbox.FocusView` _array_element)) _numofplayers)))
      (set `local.SumOfPlayers` (+ _numofplayers (`local.SumOfPlayers`)))))
  ;;[1 1 1] Divide by total to get middle point of all focuses
  (if (!= _sumofplayers 0)
    (set `local.TargetLocation` (/ (`local.TargetLocation`) _sumofplayers))
    (else
      (set `local.TargetLocation` (`SceneComponent.K2_GetComponentLocation` (`self.FocusViewer`)))
      (`KismetSystemLibrary.PrintString` "BP_MainCamera:SetCamFocus: Using Default Cam Location" true true (struct :`G` 0.66 :`B` 1.0 :`A` 1.0) 2.0 "focusviewer")))
  ;[1 1 1] Calculate camera Location
  (`SceneComponent.K2_AddWorldOffset` (`self.DefaultSceneRoot`) (* (- (+ (`local.TargetLocation`) (`self.CameraOffset`)) (`SceneComponent.K2_GetComponentLocation` (`self.DefaultSceneRoot`))) (`GameplayStatics.GetWorldDeltaSeconds`) (`self.CameraSpeed`)) false false))

(fn `Set Middle Point`
  (set `self.MiddlePointVector` (/ (+ (`self.K2_GetActorLocation` (`/Game/Blueprints/Players/BP_PlayersCombo.Player2Character` (`/Game/Blueprints/GameMode/TopDownGameMode.Players Input` (`self.Ref_GameManager`)))) (`self.K2_GetActorLocation` (`/Game/Blueprints/Players/BP_PlayersCombo.Player1Character` (`/Game/Blueprints/GameMode/TopDownGameMode.Players Input` (`self.Ref_GameManager`))))) 2))
  (`SceneComponent.K2_SetWorldLocation` (`self.MiddlePoint`) (`self.MiddlePointVector`) false false))

(fn `SetCamFollowSpeed`
  (bind (_returnvalue_x _returnvalue_y) (`KismetMathLibrary.BreakVector` (`SceneComponent.K2_GetComponentLocation` (`self.DefaultSceneRoot`))))
  (bind (_returnvalue_x_2 _returnvalue_y_2) (`KismetMathLibrary.BreakVector` (`SceneComponent.K2_GetComponentLocation` (`self.DefaultSceneRoot`))))
  (bind (_returnvalue_x_3 _returnvalue_y_3) (`KismetMathLibrary.BreakVector` (`SceneComponent.K2_GetComponentLocation` (`self.DefaultSceneRoot`))))
  (if (< (`KismetMathLibrary.VSize` (- (`KismetMathLibrary.MakeVector` (.x (`self.MiddlePointVector`)) (.y (`self.MiddlePointVector`))) (`KismetMathLibrary.MakeVector` _returnvalue_x_2 _returnvalue_y_2))) (`self.VeryCloseRange`))
    (set `self.FollowSpeed` (`KismetMathLibrary.FInterpTo` (`self.FollowSpeed`) 0.5 (`GameplayStatics.GetWorldDeltaSeconds`) 1.0))
    (elif (< (`KismetMathLibrary.VSize` (- (`KismetMathLibrary.MakeVector` (.x (`self.MiddlePointVector`)) (.y (`self.MiddlePointVector`))) (`KismetMathLibrary.MakeVector` _returnvalue_x_3 _returnvalue_y_3))) (`self.CloseRange`))
      (set `self.FollowSpeed` (`KismetMathLibrary.FInterpTo` (`self.FollowSpeed`) 1.0 (`GameplayStatics.GetWorldDeltaSeconds`) 1.0))
      (elif (not (< (`KismetMathLibrary.VSize` (- (`KismetMathLibrary.MakeVector` (.x (`self.MiddlePointVector`)) (.y (`self.MiddlePointVector`))) (`KismetMathLibrary.MakeVector` _returnvalue_x _returnvalue_y))) (`self.CloseRange`)))
        (set `self.FollowSpeed` (`KismetMathLibrary.FInterpTo` (`self.FollowSpeed`) 2.0 (`GameplayStatics.GetWorldDeltaSeconds`) 1.0))))))

(fn `SetCamLocation`
  (`SceneComponent.K2_AddWorldOffset` (`self.DefaultSceneRoot`) (* (- (`SceneComponent.K2_GetComponentLocation` (`self.DefaultSceneRoot`)) (`SceneComponent.K2_GetComponentLocation` (`self.MiddlePoint`))) (`GameplayStatics.GetWorldDeltaSeconds`) (/ (`/Game/Blueprints/Boat/BP_MovementComponent.CurrentSpeed` (`/Game/Blueprints/Boat/BP_Boat.BP_MovementComponent` (`self.Ref_Boat`))) 100.0)) false false))

(fn `SetCamRotation`
  ;[1 1 1] Rotate towards mid point
  (`SceneComponent.K2_SetWorldRotation` (`self.DefaultSceneRoot`) (`KismetMathLibrary.RInterpTo` (`SceneComponent.K2_GetComponentRotation` (`self.DefaultSceneRoot`)) (`KismetMathLibrary.FindLookAtRotation` (`SceneComponent.K2_GetComponentLocation` (`self.DefaultSceneRoot`)) (+ (`SceneComponent.K2_GetComponentLocation` (`self.MiddlePoint`)) (`self.MiddlePointOffset`))) (`GameplayStatics.GetWorldDeltaSeconds`) (select `bool` (`/Game/Blueprints/Boat/BP_Boat.Airborne?` (`self.Ref_Boat`)) :`false` (`self.CameraRotationSpeed`) :`true` (* (`self.CameraRotationSpeed`) 2.0) :!type "Float (double-precision)")) false false))

(fn `SetSpringArmConnection`
  (params (NewSpringArm :type "SpringArmComponent Object Reference"))
  (`self.K2_AttachToComponent` NewSpringArm "None" "SnapToTarget" "SnapToTarget" "SnapToTarget")
  (set `self.Connected Spring Arm` NewSpringArm))

(fn `UserConstructionScript`)