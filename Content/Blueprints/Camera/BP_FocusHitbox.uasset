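; BP_FocusHitbox is a station trigger volume that steers the main camera's focus as a third-person character moves around the boat.
; BeginPlay caches the game mode and boat, then derives a focus priority from StationType.
; On overlap begin or end, it scans the character capsule's overlapping hitboxes for rising priority, passing the boat's matching SC_FocusViewer to the camera.
; With no hitboxes overlapped, the camera's focus stays unchanged.
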(event `self.ReceiveBeginPlay`
  (`|ExecutionSequence`
    (:`then_0`
      (bind _returnvalue (`GameplayStatics.GetActorOfClass` "/Game/Blueprints/GameMode/TopDownGameMode.TopDownGameMode_C"))
      (set `self.Ref_GameManager` _returnvalue))
    (:`then_1`
      (bind _returnvalue_2 (`GameplayStatics.GetActorOfClass` "/Game/Blueprints/Boat/BP_Boat.BP_Boat_C"))
      (set `self.Ref_Boat` _returnvalue_2))
    (:`then_2`
      (switch `/Game/Blueprints/Enums/E_CameraStationFocus` (`self.StationType`)
        (:`NewEnumerator2`
          (set `self.FocusPriority` 4))
        (:`NewEnumerator3`
          (set `self.FocusPriority` 3))
        (:`NewEnumerator0`
          (set `self.FocusPriority` 2))
        (:`NewEnumerator1`
          (set `self.FocusPriority` 1))))))

(event `self.ReceiveActorBeginOverlap`
  (params (OtherActor :type "Actor Object Reference"))
  (`self.UpdateCameraFocus` true OtherActor)
  (`KismetSystemLibrary.PrintString` "I'm overlapping!"))

(event `self.ReceiveActorEndOverlap`
  (params (OtherActor :type "Actor Object Reference"))
  (`self.UpdateCameraFocus` false OtherActor)
  (`KismetSystemLibrary.PrintString` "I'm NOT overlapping!"))

(event `self.ReceiveTick`
  (params (DeltaSeconds :type "Float (single-precision)")))

(fn `GetHighestFocusHitbox`
  (params (Object :type "Object Object Reference")))

(fn `UpdateCameraFocus`
  (params (IsBeginOverlap :type Boolean :default true) (Object :type "Object Object Reference"))
  (if IsBeginOverlap
    _
    (else
      _))
  ;[1 1 1] Get Highest Focus Hitbox
  (bind _asbp_third_person_character (cast `/Game/Blueprints/Players/BP_ThirdPersonCharacter` Object))
  (set `self.CurrentHighestFocus` 0)
  (for _array_element (`PrimitiveComponent.GetOverlappingActors` (`Character.CapsuleComponent` _asbp_third_person_character) "BP_FocusHitbox_C")
    (bind _asbp_focus_hitbox (cast `/Game/Blueprints/Camera/BP_FocusHitbox` _array_element))
    (bind _focuspriority (`/Game/Blueprints/Camera/BP_FocusHitbox.FocusPriority` _asbp_focus_hitbox))
    (if (> _focuspriority (`self.CurrentHighestFocus`))
      (set `self.CurrentHighestFocus` _focuspriority)
      ;[1 1 1] Get Corresponding Focus Viewer
      (for _array_element_2 (`self.K2_GetComponentsByClass` (`self.Ref_Boat`) "/Game/Blueprints/Camera/SC_FocusViewer.SC_FocusViewer_C")
        (if (`|EnumEquality` (`/Game/Blueprints/Camera/BP_FocusHitbox.StationType` _asbp_focus_hitbox) (`/Game/Blueprints/Camera/SC_FocusViewer.StationType` _array_element_2))
          (`|ExecutionSequence`
            (:`then_0`
              ;[1 1 1] Set Camera's Focus Viewer
              (`KismetSystemLibrary.PrintString` (`KismetSystemLibrary.GetDisplayName` _array_element_2) true true (struct :`G` 0.66 :`B` 1.0 :`A` 1.0) 2.0 "FocusHitbox")
              (set `/Game/Blueprints/Camera/BP_MainCamera.CurrentHighestFocus` (`self.CurrentHighestFocus`) (`/Game/Blueprints/GameMode/TopDownGameMode.MainCamera` (`self.Ref_GameManager`)))
              (set `/Game/Blueprints/Camera/BP_MainCamera.FocusViewer` _array_element_2 (`/Game/Blueprints/GameMode/TopDownGameMode.MainCamera` (`self.Ref_GameManager`))))
            (:`then_1`
              (break))))))))

(fn `UserConstructionScript`)