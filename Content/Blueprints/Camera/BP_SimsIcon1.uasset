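; BP_SimsIcon1 is an icon actor whose SMSimsIcon component resizes with the horizontal distance between the boat and the main camera.
; On BeginPlay it finds the TopDownGameMode actor and stores it as GameManager, its source for both the boat and camera.
; Each Tick it offsets, divides and clamps that 2D distance to set the icon's world scale, with Z at half of X and Y.
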(event `self.ReceiveBeginPlay`
  (bind _returnvalue (`GameplayStatics.GetActorOfClass` "/Game/Blueprints/GameMode/TopDownGameMode.TopDownGameMode_C"))
  (set `self.GameManager` _returnvalue))

(event `self.ReceiveTick`
  (params (DeltaSeconds :type "Float (single-precision)"))
  (bind _gamemanager (`self.GameManager`))
  (bind _returnvalue (`KismetMathLibrary.FClamp` (/ (- (`KismetMathLibrary.Vector_Distance2D` (`self.K2_GetActorLocation` (`/Game/Blueprints/GameMode/TopDownGameMode.Boat` _gamemanager)) (`self.K2_GetActorLocation` (`/Game/Blueprints/GameMode/TopDownGameMode.MainCamera` _gamemanager))) 5500.0) 2000.0) 0.3 0.6))
  (`SceneComponent.SetWorldScale3D` (`self.SM_SimsIcon`) (`KismetMathLibrary.MakeVector` _returnvalue _returnvalue (/ _returnvalue 2.0))))

(fn `UserConstructionScript`)