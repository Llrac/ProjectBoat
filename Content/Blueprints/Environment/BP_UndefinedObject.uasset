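; BP_UndefinedObject is an environment placeholder actor that turns into its assigned Object class when a BP_Boat overlaps it.
; On BeginPlay it caches the BP_EnvironmentSpawner.
; On overlap it spawns the Object at its own transform, adjusting for collision but always spawning.
; It then replaces its own entry in the spawner's ObjectData with one for the spawned actor and destroys itself.
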(event `self.ReceiveBeginPlay`
  (bind _returnvalue (`GameplayStatics.GetActorOfClass` "/Game/Blueprints/Environment/BP_EnvironmentSpawner.BP_EnvironmentSpawner_C"))
  (set `self.NewVar` _returnvalue))

(event `self.ReceiveActorBeginOverlap`
  (params (OtherActor :type "Actor Object Reference"))
  (bind _returnvalue (`self.GetTransform`))
  (bind _object (`self.Object`))
  (bind _object_2 (`self.Object`))
  (bind _objectdata (`/Game/Blueprints/Environment/BP_EnvironmentSpawner.ObjectData` (`self.NewVar`)))
  (cast `/Game/Blueprints/Boat/BP_Boat` OtherActor)
  (if (`KismetSystemLibrary.IsValidClass` _object)
    (bind _returnvalue_2 (`|SpawnActorFromClass` _object (`self.GetTransform`) "AdjustIfPossibleButAlwaysSpawn" "OverrideRootScale" null null))
    (`KismetArrayLibrary.Array_RemoveItem` _objectdata (make `/Game/Blueprints/Structures/F_ObjectData` self _returnvalue _object_2 true))
    (`KismetArrayLibrary.Array_RemoveItem` _objectdata (make `/Game/Blueprints/Structures/F_ObjectData` self _returnvalue _object_2))
    (`KismetArrayLibrary.Array_AddUnique` (`/Game/Blueprints/Environment/BP_EnvironmentSpawner.ObjectData` (`self.NewVar`)) (make `/Game/Blueprints/Structures/F_ObjectData` _returnvalue_2 (`self.GetTransform` _returnvalue_2) (`self.Object`) true))
    (`self.K2_DestroyActor`)))

(fn `UserConstructionScript`)