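; Breakable crystal that loses HP per hit, shows remaining health on a prompt slider, and shatters at zero.
; Breaking enables physics on the destructible and triggers a short-lived radial Chaos field.
; At zero HP, randomly scaled shard pickups spawn only if HasSpawnedPickups is already true.
; A CustomLinecastCollider hit instead disables that collider, shatters immediately and sets HUD Money to a small random value.
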(event `self.ReceiveBeginPlay`
  (`parent.ReceiveBeginPlay`))

(event `self.ReceiveTick`
  (params (DeltaSeconds :type "Float (single-precision)")))

(event `/Game/Blueprints/Interfaces/BPI_HitByCannon.Hit`
  (params (HitDirection :type "Vector Structure"))
  (bind _as_image_prompt (`self.As Image Prompt`))
  (`/Engine/EditorBlueprintResources/StandardMacros.DecrementInt` (`self.Hp`)
    (:`  `
      (`/Game/Blueprints/Widgets/ImagePrompt.SetSlider` _as_image_prompt true (/ (`self.Hp`) (`self.MaxHp`)))
      (if (<= (`self.Hp`) 0)
        (`/Game/Blueprints/Widgets/ImagePrompt.SetSlider` _as_image_prompt false 0.0)
        (`self.BreakDestructible`)
        (if (`self.Has Spawned Pickups`)
          (`self.SpawnPickups`)
          (set `self.Has Spawned Pickups` true))))))

(event `self.CustomLinecastCollider.OnComponentHit`
  (params (HitComponent :type "PrimitiveComponent Object Reference") (OtherActor :type "Actor Object Reference") (OtherComp :type "PrimitiveComponent Object Reference") (NormalImpulse :type "Vector Structure") (Hit :type "HitResult Structure (by ref)"))
  (`PrimitiveComponent.SetCollisionEnabled` (`self.CustomLinecastCollider`) "NoCollision")
  (`self.BreakDestructible`)
  (bind _returnvalue (`GameplayStatics.GetActorOfClass` "/Game/Blueprints/GameMode/TopDownGameMode.TopDownGameMode_C"))
  ;[1 1 1] cashmoney to hud
  (set `/Game/Blueprints/Widgets/WBP_HUD.Money` (`KismetMathLibrary.RandomIntegerInRange` 0 5) (`/Game/Blueprints/GameMode/TopDownGameMode.Main_HUD` _returnvalue)))

(fn `BreakDestructible`
  (`PrimitiveComponent.SetSimulatePhysics` (`self.destructable`) true)
  (bind _returnvalue (`|SpawnActorFromClass` "/Engine/EditorResources/FieldNodes/FS_MasterField.FS_MasterField_C" (`KismetMathLibrary.MakeTransform` (`self.K2_GetActorLocation`) (`self.K2_GetActorRotation`) (0.7 0.7 0.7)) "Undefined" "OverrideRootScale" null null))
  (bind _output_get (set `self.Master Field` _returnvalue))
  (set `/Engine/EditorResources/FieldNodes/FS_MasterField.ActivationType` "NewEnumerator4" _output_get)
  (set `/Engine/EditorResources/FieldNodes/FS_MasterField.FieldLifespan` 0.01 _output_get)
  (set `/Engine/EditorResources/FieldNodes/FS_MasterField.Radial Magnitude` 150.0 _output_get)
  (`/Engine/EditorResources/FieldNodes/FS_MasterField.CE_Trigger` _output_get))

(fn `SpawnPickups`
  (bind (_returnvalue_location _returnvalue_rotation _returnvalue_scale) (`KismetMathLibrary.BreakTransform` (`self.GetTransform`)))
  (for _ (range (+ (`KismetMathLibrary.RandomIntegerInRange` 0 2) 1))
    (`|SpawnActorFromClass` "/Game/Blueprints/Props/BP_PickupableCrystalShard.BP_PickupableCrystalShard_C" (`KismetMathLibrary.MakeTransform` _returnvalue_location _returnvalue_rotation (* _returnvalue_scale (`KismetMathLibrary.RandomFloatInRange` 0.8 2.0))) "Undefined" "OverrideRootScale" null null)))

(fn `UserConstructionScript`
  (`parent.UserConstructionScript`))