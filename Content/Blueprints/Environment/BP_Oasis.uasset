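; BP_Oasis is an environment actor that serves as a navigation point on the compass HUD.
; One tick after BeginPlay, it finds the first top-level WBP_Compass_HUD widget and adds itself to that widget's NavPoints.
; When a BP_Boat overlaps it, it looks up the widget again and removes itself from NavPoints.
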(event `self.ReceiveBeginPlay`
  (`KismetSystemLibrary.DelayUntilNextTick`)
  (bind _foundwidgets (`WidgetBlueprintLibrary.GetAllWidgetsOfClass` "/Game/Blueprints/Widgets/WBP_Compass_HUD.WBP_Compass_HUD_C"))
  (`KismetArrayLibrary.Array_Add` (`/Game/Blueprints/Widgets/WBP_Compass_HUD.NavPoints` (`|GetArrayItem` _foundwidgets)) self))

(event `self.ReceiveActorBeginOverlap`
  (params (OtherActor :type "Actor Object Reference"))
  (cast `/Game/Blueprints/Boat/BP_Boat` OtherActor)
  (bind _foundwidgets (`WidgetBlueprintLibrary.GetAllWidgetsOfClass` "/Game/Blueprints/Widgets/WBP_Compass_HUD.WBP_Compass_HUD_C"))
  (`KismetArrayLibrary.Array_RemoveItem` (`/Game/Blueprints/Widgets/WBP_Compass_HUD.NavPoints` (`|GetArrayItem` _foundwidgets)) self))

(fn `UserConstructionScript`)