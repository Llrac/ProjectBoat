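; BP_Volcano is an environment actor that launches boats upward while they are inside its trigger capsule.
; Capsule overlaps cache the BP_Boat and toggle a Trigger flag on entry and exit.
; While the flag is set, Tick applies a scaled UpForce through the boat's BPMovementComponent every frame, printing a warning if the boat reference is invalid.
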(event `self.ReceiveTick`
  (params (DeltaSeconds :type "Float (single-precision)"))
  (if (`self.Trigger?`)
    (bind _as_bp_boat (`self.As BP Boat`)
      (:`then`
        (`/Game/Blueprints/Boat/BP_MovementComponent.AddUpForce` (`/Game/Blueprints/Boat/BP_Boat.BP_MovementComponent` _as_bp_boat) (* (`self.Up Force`) 100000000.0)))
      (:`else`
        (`KismetSystemLibrary.PrintString` "Volcano is triggering without boat reference")))))

(event `self.Capsule.OnComponentBeginOverlap`
  (params (OverlappedComponent :type "PrimitiveComponent Object Reference") (OtherActor :type "Actor Object Reference") (OtherComp :type "PrimitiveComponent Object Reference") (OtherBodyIndex :type Integer) (bFromSweep :type Boolean) (SweepResult :type "HitResult Structure (by ref)"))
  (bind _asbp_boat (cast `/Game/Blueprints/Boat/BP_Boat` OtherActor))
  (set `self.As BP Boat` _asbp_boat)
  (set `self.Trigger?` true))

(event `self.Capsule.OnComponentEndOverlap`
  (params (OverlappedComponent :type "PrimitiveComponent Object Reference") (OtherActor :type "Actor Object Reference") (OtherComp :type "PrimitiveComponent Object Reference") (OtherBodyIndex :type Integer))
  (cast `/Game/Blueprints/Boat/BP_Boat` OtherActor)
  (set `self.Trigger?` false))

(fn `UserConstructionScript`)